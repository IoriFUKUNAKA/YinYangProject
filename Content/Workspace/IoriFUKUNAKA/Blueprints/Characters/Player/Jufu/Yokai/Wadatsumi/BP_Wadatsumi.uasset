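; Wadatsumi Yokai Jufu actor: a player thrust attack that deals Sui-element damage to the actor's Owner.
; On init it turns the instigating player toward a nearby enemy and binds to the player's Jufu animation notifies.
; Notify begin runs a timeline pulling the player toward the Owner with squared easing and sweep.
; Notify end applies attack-scaled damage, and animation completion destroys the actor, both through ROS-prefixed calls.
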(event Custom|E_OnJufuAnimCompleated
  (Default|ROSDestroyActor (Variables|Default|GetInstigatorPlayer) self))

(event Custom|E_OnAnimNotifyEnd
  (params (NotifyName :type Name))
  (bind _returnvalue (Components|GetOwner))
  (bind _instigatorplayer (Variables|Default|GetInstigatorPlayer))
  (bind _returnvalue_2 (Transformation|GetActorLocation _returnvalue))
  (bind _returnvalue_3 (Transformation|GetActorLocation _instigatorplayer))
  (bind (_x _y) (Math|Vector|BreakVector _returnvalue_2))
  (bind (_x_2 _y_2) (Math|Vector|BreakVector _returnvalue_3))
  (bind _returnvalue_4 (Math|Vector|MakeVector _x _y 0.0))
  (bind _returnvalue_5 (Math|Vector|MakeVector _x_2 _y_2 0.0))
  (bind _returnvalue_6 (Math|Rotator|FindLookatRotation _returnvalue_5 _returnvalue_4))
  (switch name NotifyName
    (:Thrust
      (Utilities|FlowControl|Sequence
        (:then_0
          (bind _rate (Timeline|Trust Stop)
            (:Update
              (Transformation|SetActorTransform (Variables|Default|GetInstigatorPlayer) (Math|Transform|MakeTransform (Math|Vector|MakeVector (.x (Math|Vector|Lerp(Vector) _returnvalue_5 _returnvalue_4 (Math|Float|Square _rate))) (.y (Math|Vector|Lerp(Vector) _returnvalue_5 _returnvalue_4 (Math|Float|Square _rate))) (Variables|/Script/Engine.CapsuleComponent|GetCapsuleHalfHeight (Variables|/Script/Engine.Character|GetCapsuleComponent _instigatorplayer))) _returnvalue_6 "1,1,1") true)
              (Default|ROSSetActorTransform (Variables|Default|GetInstigatorPlayer) (Math|Transform|MakeTransform (Math|Vector|MakeVector (.x (Math|Vector|Lerp(Vector) _returnvalue_5 _returnvalue_4 (Math|Float|Square _rate))) (.y (Math|Vector|Lerp(Vector) _returnvalue_5 _returnvalue_4 (Math|Float|Square _rate))) (Variables|/Script/Engine.CapsuleComponent|GetCapsuleHalfHeight (Variables|/Script/Engine.Character|GetCapsuleComponent _instigatorplayer))) _returnvalue_6 "1,1,1") true false))))
        (:then_1
          (bind _instigatorplayer_2 (Variables|Default|GetInstigatorPlayer)
            (:then
              (bind _playerstate (Variables|/Script/Engine.Pawn|GetPlayerState _instigatorplayer_2)
                (:then
                  (bind _attack (Class|BPIControlPlayerState|IGetCurrentPlayerStatus(Message) _playerstate))
                  (Default|ROSApplyDamage _instigatorplayer_2 (Components|GetOwner) (* _attack (Variables|Config|GetAttackMag)) (Pawn|GetController _instigatorplayer_2) self "/Game/Workspace/IoriFUKUNAKA/Blueprints/Characters/Player/DamageType/D_GiveElementDamage_Sui.D_GiveElementDamage_Sui_C"))
                (:else)))
            (:else)))))))

(event Custom|E_OnAnimNotifyBegin
  (params (NotifyName :type Name))
  (bind _returnvalue (Components|GetOwner))
  (bind _instigatorplayer (Variables|Default|GetInstigatorPlayer))
  (bind _returnvalue_2 (Transformation|GetActorLocation _returnvalue))
  (bind _returnvalue_3 (Transformation|GetActorLocation _instigatorplayer))
  (bind (_x _y) (Math|Vector|BreakVector _returnvalue_2))
  (bind (_x_2 _y_2) (Math|Vector|BreakVector _returnvalue_3))
  (bind _returnvalue_4 (Math|Vector|MakeVector _x _y 0.0))
  (bind _returnvalue_5 (Math|Vector|MakeVector _x_2 _y_2 0.0))
  (bind _returnvalue_6 (Math|Rotator|FindLookatRotation _returnvalue_5 _returnvalue_4))
  (switch name NotifyName
    (:Thrust
      (bind _rate (Timeline|Trust PlayFromStart)
        (:Update
          (Transformation|SetActorTransform (Variables|Default|GetInstigatorPlayer) (Math|Transform|MakeTransform (Math|Vector|MakeVector (.x (Math|Vector|Lerp(Vector) _returnvalue_5 _returnvalue_4 (Math|Float|Square _rate))) (.y (Math|Vector|Lerp(Vector) _returnvalue_5 _returnvalue_4 (Math|Float|Square _rate))) (Variables|/Script/Engine.CapsuleComponent|GetCapsuleHalfHeight (Variables|/Script/Engine.Character|GetCapsuleComponent _instigatorplayer))) _returnvalue_6 "1,1,1") true)
          (Default|ROSSetActorTransform (Variables|Default|GetInstigatorPlayer) (Math|Transform|MakeTransform (Math|Vector|MakeVector (.x (Math|Vector|Lerp(Vector) _returnvalue_5 _returnvalue_4 (Math|Float|Square _rate))) (.y (Math|Vector|Lerp(Vector) _returnvalue_5 _returnvalue_4 (Math|Float|Square _rate))) (Variables|/Script/Engine.CapsuleComponent|GetCapsuleHalfHeight (Variables|/Script/Engine.Character|GetCapsuleComponent _instigatorplayer))) _returnvalue_6 "1,1,1") true false))))))

(event Custom|E_BindOnJufuAnimNotifyEvent
  (bind _instigatorplayer (Variables|Default|GetInstigatorPlayer)
    (:then
      (EventDispatchers|BindEventtoOnJufuAnimNotifyBegin _instigatorplayer (EventDispatchers|CreateEvent :!event Custom|E_OnAnimNotifyBegin))
      (EventDispatchers|BindEventtoOnJufuAnimNotifyEnd _instigatorplayer (EventDispatchers|CreateEvent :!event Custom|E_OnAnimNotifyEnd))
      (EventDispatchers|BindEventtoOnJufuAnimCompleated _instigatorplayer (EventDispatchers|CreateEvent :!event Custom|E_OnJufuAnimCompleated)))
    (:else)))

(event Custom|MC_InitializeWadatsumi
  (bind _instigator (Variables|Default|GetInstigator)
    (:then
      (bind _asbp_yin_yang_player (Utilities|Casting|CastToBP_YinYangPlayer _instigator))
      (bind _output_get (Variables|Default|SetInstigatorPlayer _asbp_yin_yang_player))
      (bind _rotation (Default|FRotationtoNearEnemy _output_get 5e+03))
      (Transformation|SetActorRotation _output_get _rotation)
      (CallFunction|EBindonJufuAnimNotifyEvent))
    (:else)))

(fn ConstructionScript
  (|CallParentFunction))

(fn FonInitialize
  (|CallParentFunction)
  (CallFunction|MCInitializeWadatsumi))