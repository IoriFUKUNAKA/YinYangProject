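; Main GameMode (named as an old version) that tracks connected player controllers through login and logout.
; On login it assigns each controller's array index as player ID, mirrored to PlayerState, and registers it with BP_GameManager, looked up lazily.
; Both events have the manager spawn visual characters and rebuild status and matchmaking arrays from all controllers and pawns, copying them to every controller.
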(event Custom|E_SetAllPlayerStatusInfoMation
  ;[1 1 1] ステータス情報を作成
  (for _array_element (Variables|Ref|GetPlayerControllersRef)
    (bind __playerdata (CallFunction|FGetAllPlayerInfo))
    (Variables|/Game/Workspace/IoriFUKUNAKA/Blueprints/Characters/Player/BP_PlayerController.BP_PlayerController_C|SetPlayersData _array_element __playerdata)))

(event Custom|E_SetAllMatchingDataInfo
  ;[1 1 1] マッチング情報を作成
  (for _array_element (Variables|Ref|GetPlayerControllersRef)
    (bind _matchingdata (CallFunction|FGetAllMatchingData))
    (Variables|/Game/Workspace/IoriFUKUNAKA/Blueprints/Characters/Player/BP_PlayerController.BP_PlayerController_C|SetMatchData _array_element _matchingdata)))

(event Custom|MC_SetId
  (params (PlayerID :type Integer) (ターゲット :type BP%20Player%20Controller%20Object%20Reference))
  ;[1 1 1] ログイン時の処理
  (bind _output_get (Variables|/Game/Workspace/IoriFUKUNAKA/Blueprints/Characters/Player/BP_PlayerController.BP_PlayerController_C|SetPlayerID ターゲット PlayerID))
  (bind _asps_my_player_state (Utilities|Casting|CastToPS_MyPlayerState (Variables|/Script/Engine.Controller|GetPlayerState ターゲット)))
  (Variables|/Game/Workspace/Yamashita/Blueprint/PlayerState/PS_MyPlayerState.PS_MyPlayerState_C|SetMyPlayerID _asps_my_player_state _output_get))

(event EventOnLogout
  (params (ExitingController :type Controller%20Object%20Reference))
  (bind _asbp_player_controller (Utilities|Casting|CastToBP_PlayerController ExitingController))
  (Utilities|Array|RemoveItem (Variables|Ref|GetPlayerControllersRef) _asbp_player_controller)
  (CallFunction|ESetAllPlayerStatusInfoMation)
  (CallFunction|ESetAllMatchingDataInfo)
  (bind _gamemanagerref (Variables|Ref|GetGameManagerRef)
    (:then
      (Default|ESpawnVisualCharacter _gamemanagerref))
    (:else)))

(event EventPostLogin
  (params (NewPlayer :type Player%20Controller%20Object%20Reference))
  ;[1 1 1] ログイン時の処理
  (bind _asbp_player_controller (Utilities|Casting|CastToBP_PlayerController NewPlayer)
    (:then
      (bind _returnvalue (Utilities|Array|AddUnique (Variables|Ref|GetPlayerControllersRef) _asbp_player_controller))
      (Networking|SwitchHasAuthority
        (:Authority
          (CallFunction|MCSetId _returnvalue _asbp_player_controller)
          (bind _gamemanagerref (Variables|Ref|GetGameManagerRef)
            (:then
              (Default|EPlayerLogin _gamemanagerref _asbp_player_controller :!label _label)
              (Default|ESpawnVisualCharacter _gamemanagerref)
              (CallFunction|ESetAllPlayerStatusInfoMation)
              (CallFunction|ESetAllMatchingDataInfo)
              (Variables|/Game/Workspace/IoriFUKUNAKA/Blueprints/Characters/Player/BP_PlayerController.BP_PlayerController_C|SetGM%20Main _asbp_player_controller self))
            (:else
              (bind _returnvalue_2 (Actor|GetActorOfClass "/Game/Workspace/IoriFUKUNAKA/Blueprints/System/Main/BP_GameManager.BP_GameManager_C"))
              (bind _output_get (Variables|Ref|SetGameManagerRef _returnvalue_2))
              (Utilities|IsValid _output_get
                (:Is%20Valid
                  (goto _label))
                (:Is%20Not%20Valid
                  (Development|PrintString "BP_GameManagerが見つかりません。" true true "(R=1.000000,G=0.000000,B=0.000000,A=1.000000)"))))))))
    (:CastFailed
      (Development|PrintString "Error:PlayerControllerのキャストに失敗" true true "(R=1.000000,G=0.000000,B=0.000000,A=1.000000)"))))

(fn ConstructionScript)

(fn FGetPlayerControllerRef
  (return (Variables|Ref|GetPlayerControllersRef)))

(fn FGetAllPlayerInfo
  (for _array_element (Variables|Ref|GetPlayerControllersRef)
    ;[1 1 1] Playerのステータスを設定
    (Utilities|IsValid (Pawn|GetControlledPawn _array_element)
      (:Is%20Valid
        (bind _asbp_player (Utilities|Casting|CastToBP_Player (Pawn|GetControlledPawn _array_element)))
        (Utilities|Array|Add (LocalVariables|GetPlayerData) (Utilities|Struct|MakeST_PlayerData (PlayerState|GetPlayerName (Variables|/Script/Engine.Controller|GetPlayerState _array_element)) (Variables|/Game/Workspace/IoriFUKUNAKA/Blueprints/Characters/Player/BP_Player.BP_Player_C|GetCurrentHP _asbp_player) (Variables|/Game/Workspace/IoriFUKUNAKA/Blueprints/Characters/Player/BP_Player.BP_Player_C|GetMaxHP _asbp_player) (Variables|/Game/Workspace/IoriFUKUNAKA/Blueprints/Characters/Player/BP_Player.BP_Player_C|GetCurrentEnergy _asbp_player) (Default|FGetValidEffects (Variables|/Game/Workspace/IoriFUKUNAKA/Blueprints/Characters/Player/BP_Player.BP_Player_C|GetBPC_StatusManager _asbp_player)))))))
  (return (LocalVariables|GetPlayerData)))

(fn FGetAllMatchingData
  (for _array_element (Variables|Ref|GetPlayerControllersRef)
    (Utilities|Array|Add (LocalVariables|GetPlayerMatchingData) (Utilities|Struct|MakeST_PlayerMatchiData (PlayerState|GetPlayerName (Variables|/Script/Engine.Controller|GetPlayerState _array_element)) (Variables|/Game/Workspace/IoriFUKUNAKA/Blueprints/Characters/Player/BP_PlayerController.BP_PlayerController_C|GetisReady _array_element) (Variables|/Game/Workspace/IoriFUKUNAKA/Blueprints/Characters/Player/BP_PlayerController.BP_PlayerController_C|GetTempSkills _array_element))))
  (return (LocalVariables|GetPlayerMatchingData)))