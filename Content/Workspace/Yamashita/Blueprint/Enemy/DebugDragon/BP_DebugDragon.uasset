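; BP_DebugDragon is an enemy Blueprint that implements the Kirin boss's attack interface using dragon montages, apparently as a debug stand-in.
; Behavior Tree interface calls play montages through multicast; rush attacks also spawn BP_RushCollision in one HealthState, notified when the rush finishes.
; A collision override picks a head-socket sphere or body box overlap from the AttackState gameplay tag.
; Getters expose gimmick settings and hate-stage thresholds.
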(event Collision|EventActorBeginOverlap
  (params (OtherActor :type Actor%20Object%20Reference)))

(event EventTick
  (params (DeltaSeconds :type Float%20%28single-precision%29))
  (|CallParentFunction DeltaSeconds))

(event Custom|MC_SpawnRushCollision
  (params (StartLoc :type Vector) (TargetLoc :type Vector))
  ;[1 0 0.9549] From BT
  ;;[1 1 1] 突進攻撃（スキル強化後）
  (Game|SpawnActorfromClass "/Game/Workspace/Yamashita/Blueprint/Enemy/Kirin/Object/BP_RushCollision.BP_RushCollision_C" (Math|Conversions|ToTransform(Vector) StartLoc) "Undefined" 0 self StartLoc TargetLoc 0))

(event Custom|MC_RushFinish_Kirin
  (params (ターゲット :type Object%20Object%20Reference))
  ;[1 0 0.9549] From BT
  ;;[1 1 1] 突進終了
  (bind _outactors (Actor|GetAllActorsOfClass "/Game/Workspace/Yamashita/Blueprint/Enemy/Kirin/Object/BP_RushCollision.BP_RushCollision_C"))
  (for _array_element _outactors
    (Class|BPIEnemy|IRushFinishKirin(Message) _array_element)))

(event Custom|MC_SetIsWalkWait
  (params (isWalkWait :type Boolean))
  ;[1 0 0.9549] From BT
  ;;[1 1 1] 歩く待機か
  (Class|BPIEnemy|ISetIsWalkWait(Message) (Components|SkeletalMesh|GetAnimInstance (Variables|Character|GetMesh)) isWalkWait))

(event EventINormalAttackKirin
  ;[1 0 0.9549] From BT
  ;;[1 1 1] 通常攻撃　通知
  (CallFunction|MCPlayMontage "/Game/Workspace/Yamashita/Animation/DebugDragon/Montage/AM_AttackMouthAnim.AM_AttackMouthAnim" 1.0))

(event EventIIndiscriminateAttackKirin
  ;[1 0 0.9549] From BT
  ;;[1 1 1] 落雷攻撃　通知
  (CallFunction|MCPlayMontage "/Game/Workspace/Yamashita/Animation/DebugDragon/Montage/AM_AttackWingClawAnim.AM_AttackWingClawAnim" 1.0))

(event EventIRangeAttackKirin
  ;[1 0 0.9549] From BT
  ;;[1 1 1] スパーク攻撃
  (CallFunction|MCPlayMontage "/Game/Workspace/Yamashita/Animation/DebugDragon/Montage/AM_GetHitAnim.AM_GetHitAnim" 1.0))

(event EventIRushAttackKirin
  (params (startLoc :type Vector :default "0, 0, 0") (targetLoc :type Vector :default "0, 0, 0"))
  ;[1 0 0.9549] From BT
  ;;[1 1 1] 突進攻撃（スキル強化後）
  (CallFunction|MCPlayMontage "/Game/Workspace/Yamashita/Animation/DebugDragon/Montage/AM_RunAnim.AM_RunAnim" 1.0)
  (if (Utilities|Enum|Equal(Enum) (Variables|Default|GetHealthState) "NewEnumerator1")
    (CallFunction|MCSpawnRushCollision startLoc targetLoc)))

(event EventIRushFinishKirin
  ;[1 0 0.9549] From BT
  ;;[1 1 1] 突進終了
  (CallFunction|MCRushFinishKirin))

(event EventISetIsWalkWait
  (params (isWalkWait :type Boolean))
  ;[1 0 0.9549] From BT
  ;;[1 1 1] 歩く待機か
  (CallFunction|MCSetIsWalkWait isWalkWait))

(event EventIGimickAttackKirin
  ;[1 0 0.9549] From BT
  ;;[1 1 1] ギミック攻撃
  (CallFunction|MCPlayMontage "/Game/Workspace/Yamashita/Animation/DebugDragon/Montage/AM_DefendAnim.AM_DefendAnim" 1.0))

(fn ConstructionScript
  (|CallParentFunction))

(fn FOverrideCollision
  (|CallParentFunction)
  (|SwitchGameplayTag (Variables|Default|GetAttackState)
    (:Enemy.Attack.Kirin.NormalAttack
      (CallFunction|FSphereOverlap (Transformation|GetSocketLocation (Variables|Character|GetMesh) "UpperHead2") 2e+02))
    (:Enemy.Attack.Kirin.RushAttack
      (CallFunction|FBoxOverlap (Transformation|GetActorLocation) "200.000000,200.000000,150.000000"))))

(fn IGetGimickAppearNumKirin
  (return (Variables|プランナー編集可|GetGimickNum)))

(fn IGetGimickRangeKirin
  (return (Variables|プランナー編集可|GetAttackRange_GimickAttack)))

(fn IGetTimeforGimickActivateKirin
  (return (Variables|プランナー編集可|GetTimeForGimickActivate)))

(fn IGetHateStageBorder
  (params (Stage :type E_EnemyStageState%20Enum :default "NewEnumerator0"))
  (for (_array_element _array_index) (Variables|プランナー編集可|GetHateStage)
    (if (Utilities|Enum|Equal(Enum) (.stage (Utilities|Struct|BreakST_HateStage _array_element)) Stage)
      (return (.hate (Utilities|Struct|BreakST_HateStage _array_element)) (== _array_index (Utilities|Array|LastIndex (Variables|プランナー編集可|GetHateStage))))))
  (return 0.0 false))