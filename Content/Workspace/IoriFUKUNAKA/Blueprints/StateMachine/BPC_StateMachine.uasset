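; BPC_StateMachine is a generic state machine component that stores state components and runs one current state at a time.
; Added states receive a reference back to the machine, and the update event forwards world delta seconds to the current state's tick.
; Transitions by name or reference call end on the old state and begin on the new.
; Getters expose the states, and removing the running state is refused with a warning.
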(event Custom|E_UpdateStateMachine
  ;[1 1 1] 更新処理
  (Default|OnStateTick (Variables|StateMachine|GetCurrentState) (Utilities|Time|GetWorldDeltaSeconds)) ; 現在のステートのTickイベント呼び出し
)

(event Custom|E_AddState
  (params (StateComponent :type BPC%20State%20Base%20Object%20Reference))
  (bind _statename (Variables|/Game/Workspace/IoriFUKUNAKA/Blueprints/StateMachine/BPC_StateBase.BPC_StateBase_C|GetStateName StateComponent))
  ;[1 1 1] ステートを追加する
  (bind _array_element (Utilities|Array|ForEachLoopwithBreak (Variables|StateMachine|GetStateComponent) :!label _label)
    (:LoopBody
      (if (and (Utilities|Enum|Equal(Enum) (Variables|/Game/Workspace/IoriFUKUNAKA/Blueprints/StateMachine/BPC_StateBase.BPC_StateBase_C|GetStateName _array_element) _statename) (Utilities|Enum|Equal(Enum) _statename ""))
        (Development|PrintString "State Machine Warning!! : State can not be Added" true true "(R=1.000000,G=0.000000,B=0.000000,A=1.000000)")
        (goto _label Break)))
    (:Completed
      (bind _returnvalue (Utilities|Array|Add (Variables|StateMachine|GetStateComponent) StateComponent))
      (Variables|/Game/Workspace/IoriFUKUNAKA/Blueprints/StateMachine/BPC_StateBase.BPC_StateBase_C|SetParentStateMachine (Utilities|Array|Get(acopy) (Variables|StateMachine|GetStateComponent) _returnvalue) self) ; ステートマシンコンポーネントの\n情報を参照できるように保存しておく。
    )))

(event Custom|E_SwitchState
  (params (StateClass :type BPC%20State%20Base%20Object%20Reference))
  (bind _statecomponent (Variables|StateMachine|GetStateComponent))
  ;[1 1 1] ステートを切り替える
  (if (Utilities|Array|ContainsItem _statecomponent StateClass) ; 配列にステートがあればステート変更を行う。\nなかった場合には警告を表示する。
    (Default|OnStateEnd (Variables|StateMachine|GetCurrentState))
    (bind _output_get (Variables|StateMachine|SetCurrentState (Utilities|Array|Get(acopy) _statecomponent (Utilities|Array|FindItem _statecomponent StateClass))))
    (Default|OnStateBegin _output_get)
    (else
      (Development|PrintString "State Machine Warning!! : Unknown state" true true "(R=1.000000,G=0.000000,B=0.000000,A=1.000000)"))))

(event Custom|E_LaunchState
  (params (StateComponent :type BPC%20State%20Base%20Object%20Reference))
  ;[1 1 1] ステートの起動
  (bind _output_get (Variables|StateMachine|SetCurrentState StateComponent))
  (Default|OnStateBegin _output_get))

(event Custom|E_RemoveState
  (params (StateComponent :type BPC%20State%20Base%20Object%20Reference))
  ;[1 1 1] ステートの削除
  (if (== StateComponent (Variables|StateMachine|GetCurrentState))
    (Development|PrintString "State Machine Warning!! : State can note be deleted running" true true "(R=1.000000,G=0.000000,B=0.000000,A=1.000000)")
    (else
      (Utilities|Array|RemoveItem (Variables|StateMachine|GetStateComponent) StateComponent))))

(event Custom|E_TransitionState
  (params (NewStateName :type String))
  ;[1 1 1] ステート名からステートを切り替える
  (bind _array_element (Utilities|Array|ForEachLoopwithBreak (Variables|StateMachine|GetStateComponent) :!label _label)
    (:LoopBody
      (if (Utilities|Enum|Equal(Enum) (Variables|/Game/Workspace/IoriFUKUNAKA/Blueprints/StateMachine/BPC_StateBase.BPC_StateBase_C|GetStateName _array_element) NewStateName)
        (CallFunction|ESwitchState _array_element)
        (goto _label Break)))))

(fn FGetCurrentState
  (return (Variables|StateMachine|GetCurrentState)))

(fn FGetCurrentStateName
  (bind _currentstate (Variables|StateMachine|GetCurrentState)
    (:then
      (return (Variables|/Game/Workspace/IoriFUKUNAKA/Blueprints/StateMachine/BPC_StateBase.BPC_StateBase_C|GetStateName _currentstate)))
    (:else
      (return ""))))

(fn FGetAllState
  (return (Variables|StateMachine|GetStateComponent)))