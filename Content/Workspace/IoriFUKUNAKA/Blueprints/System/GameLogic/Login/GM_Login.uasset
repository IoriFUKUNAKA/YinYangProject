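; Login game mode that drives which login screen is shown, switching between Menu and Server List states and opening Menu on BeginPlay.
; E_ChangeState runs M_TransitionState, which tells player controller 0 to remove the current screen, then on success sends the show message for the new one via interface calls.
; Same-state and Valid targets print errors; Valid serves as the invalid initial value, though its check runs after the current screen's removal.
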(event Custom|E_ChangeState
  (params (NextState :type En_LoginState%20Enum :default "NewEnumerator0"))
  (bind _returnvalue (Game|GetPlayerController 0))
  (Utilities|MTransitionState NextState
    (:NewState
      (switch Utilities|FlowControl|Switch|SwitchonEn_LoginState NextState
        (:NewEnumerator0
          (Class|BPIControlWidget|IShowLoginMenu(Message) _returnvalue))
        (:NewEnumerator1
          (Class|BPIControlWidget|IShowServerList(Message) _returnvalue))))))

(event EventBeginPlay
  (Variables|Default|SetCurrentLoginState "NewEnumerator2")
  (CallFunction|EChangeState "NewEnumerator0"))

(fn ConstructionScript)