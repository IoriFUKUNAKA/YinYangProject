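; Seiryu player special: a server-authoritative area attack that deals Moku-element damage and heals players.
; An enemy entering SpecialArea takes damage scaled from the instigator's Attack, and the actor destroys itself.
; BeginPlay also binds OnEndPlay and immediately destroys the actor.
; Destruction triggers the overridden additional effect, healing every valid player pawn by the cached Attack times a multiplier with slight random variance.
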(event OnComponentBeginOverlap(SpecialArea)
  (params (OverlappedComponent :type Primitive%20Component%20Object%20Reference) (OtherActor :type Actor%20Object%20Reference) (OtherComp :type Primitive%20Component%20Object%20Reference) (OtherBodyIndex :type Integer) (bFromSweep :type Boolean) (SweepResult :type Hit%20Result%20Structure%20%28by%20ref%29))
  (bind _returnvalue (Game|GetInstigator))
  (bind _returnvalue_2 (Pawn|GetController _returnvalue))
  (Networking|SwitchHasAuthority
    (:Authority
      (if (Actor|ActorHasTag OtherActor "Enemy")
        (Utilities|IsValid _returnvalue
          (:Is%20Valid
            (bind _playerstate (Variables|/Script/Engine.Controller|GetPlayerState _returnvalue_2)
              (:then
                (bind _attack (Class|BPIControlPlayerState|IGetCurrentPlayerStatus(Message) _playerstate))
                (bind _output_get (Variables|Default|SetInstigatorAttack _attack))
                (Game|Damage|ApplyDamage OtherActor (* _output_get (Variables|Default|GetSpecialAttackMag)) _returnvalue_2 self "/Game/Workspace/IoriFUKUNAKA/Blueprints/Characters/Player/DamageType/D_GiveElementDamage_Moku.D_GiveElementDamage_Moku_C")
                (Actor|DestroyActor))
              (:else))))))))

(event Custom|E_OnEndPlay
  (params (Actor :type Actor%20Object%20Reference) (EndPlayReason :type EEndPlayReason%20Enum :default "Destroyed"))
  (switch Utilities|FlowControl|Switch|SwitchonEEndPlayReason EndPlayReason
    (:Destroyed
      (CallFunction|FAdditionalEffect))))

(event EventBeginPlay
  (Networking|SwitchHasAuthority
    (:Authority
      (Game|BindEventtoOnEndPlay (EventDispatchers|CreateEvent :!event Custom|E_OnEndPlay))
      (Actor|DestroyActor))))

(fn ConstructionScript
  (|CallParentFunction))

(fn FAdditionalEffect
  (|CallParentFunction)
  (for _array_element (Variables|/Script/Engine.GameStateBase|GetPlayerArray (Game|GetGameState))
    (bind _pawnprivate (Variables|/Script/Engine.PlayerState|GetPawnPrivate _array_element)
      (:then
        (Class|BPIControlPlayer|IHealPlayer(Message) _pawnprivate (Math|Float|Truncate (* (Variables|Default|GetInstigatorAttack) (Variables|Default|GetHealMag) (Math|Random|RandomFloatinRange 0.9 1.1))) false))
      (:else))))