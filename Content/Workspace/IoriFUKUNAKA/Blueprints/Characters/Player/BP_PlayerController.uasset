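; Networked player controller that forwards movement, attack, avoid and skill input to the pawn through interfaces, with separate gamepad and mouse camera handling.
; It drives each game phase's UI: login/server list, skill-select matching, battle HUD and results.
; RoS events gather server-side state via GMMain, while RoC events update client widgets, audio, damage pops and the enemy-appear sequence.
; Matching previews are reordered so the player's own character takes the first slot.
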(event EventBeginPlay
  (|CallParentFunction))

(event Input|ActionEvents|InputActionUseSkill_A
  (params (Key :type Key%20Structure))
  ;[1 1 1] スキル
  (:Pressed
    (CallFunction|FUseSkill)))

(event Input|ActionEvents|InputActionNomalAttack
  (params (Key :type Key%20Structure))
  ;[1 1 1] アクション
  (:Pressed
    (Class|BPIControllertoPlayer|INormalAttack(Message) (Pawn|GetControlledPawn))))

(event Input|ActionEvents|InputActionSpecialAttack
  (params (Key :type Key%20Structure))
  ;[1 1 1] アクション
  (:Pressed
    (Class|BPIControllertoPlayer|ISpecialAttack(Message) (Pawn|GetControlledPawn))))

(event Input|ActionEvents|InputActionAvoid
  (params (Key :type Key%20Structure))
  ;[1 1 1] アクション
  (:Pressed
    (Class|BPIControllertoPlayer|IAvoid(Message) (Pawn|GetControlledPawn))))

(event Input|ActionEvents|InputActionUseSKill_B
  (params (Key :type Key%20Structure))
  ;[1 1 1] スキル
  (:Pressed
    (CallFunction|FUseSkill 1)))

(event Input|ActionEvents|InputActionUseSkill_X
  (params (Key :type Key%20Structure))
  ;[1 1 1] スキル
  (:Pressed
    (CallFunction|FUseSkill 2)))

(event Input|ActionEvents|InputActionUseSkill_Y
  (params (Key :type Key%20Structure))
  ;[1 1 1] スキル
  (:Pressed
    (CallFunction|FUseSkill 3)))

(event Input|AxisEvents|InputAxisMoveForward
  (params (AxisValue :type Float%20%28single-precision%29))
  ;[1 1 1] 移動処理
  (Class|BPIControllertoPlayer|IMoveForward(Message) (Pawn|GetControlledPawn) AxisValue))

(event Input|AxisEvents|InputAxisMoveRight
  (params (AxisValue :type Float%20%28single-precision%29))
  ;[1 1 1] 移動処理
  (Class|BPIControllertoPlayer|IMoveRight(Message) (Pawn|GetControlledPawn) AxisValue))

(event Input|AxisEvents|InputAxisTurn
  (params (AxisValue :type Float%20%28single-precision%29))
  ;[1 1 1] 旋回処理
  ;;[1 1 1] マウス
  (bind _returnvalue (Class|AppUtilBPLibrary|IsGamePadConnected))
  (if (not _returnvalue)
    (Class|PlayerController|AddYawInput AxisValue)))

(event Input|AxisEvents|InputAxisTurnRate
  (params (AxisValue :type Float%20%28single-precision%29))
  ;[1 1 1] 旋回処理
  ;;[1 1 1] ゲームパッド
  (bind _returnvalue (Class|AppUtilBPLibrary|IsGamePadConnected))
  (if _returnvalue
    (Class|PlayerController|AddYawInput (* AxisValue (Variables|Rotate|GetBaseTurnRate) (Utilities|Time|GetWorldDeltaSeconds)))))

(event Input|AxisEvents|InputAxisLookUpRate
  (params (AxisValue :type Float%20%28single-precision%29))
  ;[1 1 1] 旋回処理
  ;;[1 1 1] ゲームパッド
  (bind _returnvalue (Class|AppUtilBPLibrary|IsGamePadConnected))
  (if _returnvalue
    (Class|PlayerController|AddPitchInput (* AxisValue (Variables|Rotate|GetBaseLookUpRate) (Utilities|Time|GetWorldDeltaSeconds)))))

(event Input|AxisEvents|InputAxisLookUp
  (params (AxisValue :type Float%20%28single-precision%29))
  ;[1 1 1] 旋回処理
  ;;[1 1 1] マウス
  (bind _returnvalue (Class|AppUtilBPLibrary|IsGamePadConnected))
  (if (not _returnvalue)
    (Class|PlayerController|AddPitchInput AxisValue)))

(event Custom|E_LoginInitialize
  ;[1 1 1] 初期化処理
  (Variables|/Script/Engine.PlayerController|SetbShowMouseCursor self true))

(event EventIRemoveLoginMenu
  ;[1 1 1] LoginMenuを非表示にする
  (Widget|RemovefromParent (Variables|Login|GetLoginMenu)))

(event EventIShowServerList
  ;[1 1 1] ServerListを表示する
  (Utilities|IsValid (Variables|Login|GetServerList)
    (:Is%20Valid
      _)
    (:Is%20Not%20Valid
      (bind _returnvalue (UserInterface|CreateWidget "/Game/Workspace/IoriFUKUNAKA/Blueprints/HeadUpDisplays/LoginHUD/WBP_ServerList.WBP_ServerList_C" self))
      (Variables|Login|SetServerList _returnvalue)))
  (Input|SetInputModeUIOnly self (Variables|Login|GetServerList) "DoNotLock")
  (UserInterface|Viewport|AddtoViewport (Variables|Login|GetServerList) 0))

(event EventIRemoveServerList
  ;[1 1 1] ServerListを非表示にする
  (Widget|RemovefromParent (Variables|Login|GetServerList)))

(event EventIShowLoginMenu
  ;[1 1 1] LoginMenuを表示する
  (Utilities|IsValid (Variables|Login|GetLoginMenu)
    (:Is%20Valid
      _)
    (:Is%20Not%20Valid
      (bind _returnvalue (UserInterface|CreateWidget "/Game/Workspace/IoriFUKUNAKA/Blueprints/HeadUpDisplays/LoginHUD/WBP_LoginMenu.WBP_LoginMenu_C" self))
      (Variables|Login|SetLoginMenu _returnvalue)))
  (Input|SetInputModeUIOnly self (Variables|Login|GetLoginMenu) "DoNotLock")
  (UserInterface|Viewport|AddtoViewport (Variables|Login|GetLoginMenu) 0))

(event Custom|E_MainUpdate
  (CallFunction|ROSUpdateBattleScoreUI)
  (CallFunction|ROCUpdateUI))

(event Custom|E_MainInitialize
  (params (Controllers :type Array%20of%20BP%20Player%20Controller%20Object%20References))
  ;[1 1 1] 初期化処理
  (CallFunction|ROCInitializeMainUI)
  (Variables|Main|SetSelectSkills (Variables|Select|GetTempSkills))
  (Input|EnableInput self)
  (CallFunction|ROCPlayBGM "/Game/Workspace/IoriFUKUNAKA/Sound/SC_BattleBGM.SC_BattleBGM")
  (CallFunction|RoCPlayEnemyAppearSequence Controllers))

(event Custom|ROC_UpdateUI
  (bind _skillcoolstatusarray (Variables|Main|GetSkillCoolStatusArray))
  (bind _currentchantdata (Variables|Main|GetCurrentChantData))
  ;[1 1 1] UI更新処理
  (bind _mainui (Variables|Main|GetMainUI)
    (:then
      (Default|EUpdatePlayerStatus _mainui (Variables|Main|GetPlayersData))
      ;;[1 1 1] スキルクールタイム残時間
      (Class|BPIControllertoMainWidget|ISetCoolingElapsedTime(Message) _mainui (Utilities|Array|Get(acopy) _skillcoolstatusarray) (Utilities|Array|Get(acopy) _skillcoolstatusarray 1) (Utilities|Array|Get(acopy) _skillcoolstatusarray 2) (Utilities|Array|Get(acopy) _skillcoolstatusarray 3))
      ;;[1 1 1] 詠唱残り時間
      (Class|BPIControllertoMainWidget|ISetCastingElapsedTime(Message) _mainui (.holderindex _currentchantdata) (.ischanting? _currentchantdata) (.elapsedtime _currentchantdata) (.maxchanttime _currentchantdata))
      ;;[1 1 1] 敵情報
      (bind (_fightingenemystate _hp _maxhp _enable) (Class|BPIControllertoPlayer|IGetFightingEnemyInfo(Message) (Pawn|GetControlledPawn)))
      (Class|BPIControllertoMainWidget|ISetFightingEnemyInfo(Message) (Variables|Main|GetMainUI) _fightingenemystate _hp _maxhp _enable (Variables|Main|GetEnemyStatusEffect))
      ;;[1 1 1] 必殺技ゲージ用パラメータ
      (bind (_currentspecial _maxspecial) (Class|BPIControllertoPlayer|IGetSpecial(Message) (Pawn|GetControlledPawn)))
      (Class|BPIControllertoMainWidget|ISetSpecial(Message) (Variables|Main|GetMainUI) _currentspecial _maxspecial))
    (:else)))

(event Custom|ROC_InitializeMainUI
  ;[1 1 1] 初期化処理
  (bind _returnvalue (UserInterface|CreateWidget "/Game/Workspace/Yamashita/Blueprint/UI/W_MainGameUI.W_MainGameUI_C" self (Variables|Select|GetTempSkills)))
  (bind _output_get (Variables|Main|SetMainUI _returnvalue))
  (UserInterface|Viewport|AddtoViewport _output_get 0)
  (Input|SetInputModeGameOnly (Game|GetPlayerController 0))
  (Variables|Default|SetbShowMouseCursor self false))

(event Custom|ROC_DamagePop
  (params (WorldLocation :type Vector) (DamageValue :type Integer) (Specified%20Color :type Linear%20Color%20Structure))
  (bind (_screenlocation _returnvalue) (Class|PlayerController|ProjectWorldLocationtoScreen WorldLocation true))
  (bind _returnvalue_2 (Pawn|GetControlledPawn))
  (bind _returnvalue_3 (Math|Float|MakeLiteralFloat 1e+03))
  (bind _returnvalue_4 (Math|Float|MakeLiteralFloat 5e+03))
  (bind _returnvalue_5 (Transformation|GetActorLocation _returnvalue_2))
  (bind _returnvalue_6 (- _returnvalue_4 _returnvalue_3))
  (bind _returnvalue_7 (Math|Vector|Distance2D(Vector) WorldLocation _returnvalue_5))
  (bind _returnvalue_8 (- _returnvalue_7 _returnvalue_3))
  (bind _returnvalue_9 (/ _returnvalue_8 _returnvalue_6))
  (bind _returnvalue_10 (Math|Float|Clamp(Float) _returnvalue_9))
  (bind _returnvalue_11 (Math|Float|Lerp 1.0 0.1 _returnvalue_10))
  ;[1 1 1] ダメージ表示
  (if _returnvalue
    (bind _returnvalue_12 (UserInterface|CreateWidget "/Game/Workspace/IoriFUKUNAKA/Blueprints/HeadUpDisplays/WBP_DamagePop.WBP_DamagePop_C" self _screenlocation (Math|Vector2D|MakeVector2D _returnvalue_11 _returnvalue_11) DamageValue))
    (Appearance|SetColorandOpacity _returnvalue_12 Specified%20Color :!class /Script/UMG.UserWidget)
    (UserInterface|Viewport|AddtoViewport _returnvalue_12 0)))

(event Custom|ROS_UpdateBattleScoreUI
  (bind _returnvalue (Pawn|GetControlledPawn))
  ;[1 1 1] UIに設定する値を取得する
  (Networking|SwitchHasAuthority
    (:Authority
      (bind _gm_main (Variables|Default|GetGM%20Main)
        (:then
          (Default|ESetAllPlayerStatusInfoMation _gm_main)
          (bind (_skilla _skillb _skillx _skilly) (Class|BPIControllertoPlayer|IGetCoolingElapsedTime(Message) _returnvalue))
          (Variables|Main|SetSkillCoolStatusArray (Utilities|Array|MakeArray _skilla _skillb _skillx _skilly))
          (bind (_holderindex _iscasting _elapsedtime _maxcastingtime) (Class|BPIControllertoPlayer|IGetCastingElapsedTime(Message) _returnvalue))
          (Variables|Main|SetCurrentChantData (Utilities|Struct|MakeST_ChantData _holderindex _iscasting _elapsedtime _maxcastingtime))
          (bind _statuseffect (Class|BPIControllertoPlayer|IGetFightingEnemyInfo(Message) _returnvalue))
          (Variables|Main|SetEnemyStatusEffect _statuseffect))
        (:else)))))

(event Custom|ROC_StartCutInAnimation
  (params (SkillHolderIndex :type Integer))
  ;[1 1 1] スキルカットイン
  (Default|ECutin (Variables|Main|GetMainUI) SkillHolderIndex))

(event Custom|RoC_PlayEnemyAppearSequence
  (params (Controllers :type Array%20of%20BP%20Player%20Controller%20Object%20References))
  ;[1 1 1] シーケンサー再生
  (bind (_outactor _returnvalue) (Sequencer|Player|CreateLevelSequencePlayer "/Game/Workspace/Yamashita/Cinematics/Sequence/LS_EnemyAppear.LS_EnemyAppear" (Utilities|Struct|MakeMovieSceneSequencePlaybackSettings false "(Value=0)" 1.0 0.0 false false true false false true)))
  (for (_array_element _array_index) Controllers
    (switch int _array_index
      (:0
        (Utilities|IsValid _array_element
          (:Is%20Valid
            (Class|LevelSequenceActor|SetBinding _outactor (|GetSequenceBinding) (Utilities|Array|MakeArray (Pawn|GetControlledPawn _array_element)) false))))
      (:1
        (Utilities|IsValid _array_element
          (:Is%20Valid
            (Class|LevelSequenceActor|SetBinding _outactor (|GetSequenceBinding) (Utilities|Array|MakeArray (Pawn|GetControlledPawn _array_element)) false))))))
  (Sequencer|Player|Play _returnvalue :!class /Script/MovieScene.MovieSceneSequencePlayer))

(event EventIDamagePop
  (params (WorldPos :type Vector :default "0, 0, 0") (DamageValue :type Integer) (InitColor :type Linear%20Color%20Structure))
  ;[1 1 1] ダメージ表示
  (CallFunction|ROCDamagePop WorldPos DamageValue InitColor))

(event EventIStartCutinAnimation
  (params (UseSkillNo :type Integer))
  ;[1 1 1] スキルカットイン
  (CallFunction|ROCStartCutinAnimation UseSkillNo))

(event Custom|ROC_LogOut
  (bind _asgi_yin_yang_project (Utilities|Casting|CastToGI_YinYangProject (Game|GetGameInstance)))
  (Default|EDestroySession _asgi_yin_yang_project self))

(event Custom|E_SelectInitialize
  (bind _returnvalue (Game|GetGameInstance))
  (bind _asgi_yin_yang_project (Utilities|Casting|CastToGI_YinYangProject _returnvalue))
  (bind _useskilldatatable (Default|FGetUseSkillDataTable _asgi_yin_yang_project))
  ;[1 1 1] 初期化
  (Input|DisableInput self)
  (bind _returnvalue_2 (Utilities|GetDataTableRow _useskilldatatable "AttackBuff")
    (:then
      (bind _returnvalue_3 (Utilities|GetDataTableRow _useskilldatatable "Heal")
        (:then
          (bind _returnvalue_4 (Utilities|GetDataTableRow _useskilldatatable "Provocation")
            (:then
              (bind _returnvalue_5 (Utilities|GetDataTableRow _useskilldatatable "SpeedBuff")
                (:then
                  (CallFunction|RoSSetTempSkills (Utilities|Array|MakeArray _returnvalue_2 _returnvalue_3 _returnvalue_4 _returnvalue_5))
                  (CallFunction|RoCSelectInitialize))))))))))

(event Custom|RoC_UpdateSelectUI
  (params (CountDownTimer :type Float%20%28single-precision%29) (isAllPlayerReady? :type Boolean))
  ;[1 1 1] マッチング画面を更新する
  (bind _matchingui (Variables|Select|GetMatchingUI)
    (:then
      (Default|EUpdateSelectUI _matchingui (Variables|Select|GetMatchData) CountDownTimer isAllPlayerReady?))
    (:else)))

(event Custom|RoC_ClearVisualPlayer
  ;[1 1 1] マッチング画面用のアクタ
  (bind _outactors (Actor|GetAllActorsOfClass "/Game/Workspace/Yamashita/Blueprint/Player/VisualCharacter/BP_PlayerBaseForVisual.BP_PlayerBaseForVisual_C"))
  (for _array_element _outactors
    (Utilities|IsValid _array_element
      (:Is%20Valid
        (if (not (Variables|/Game/Workspace/Yamashita/Blueprint/Player/VisualCharacter/BP_PlayerBaseForVisual.BP_PlayerBaseForVisual_C|GetisSequence _array_element))
          (Actor|DestroyActor _array_element))))))

(event Custom|E_SelectUpdate
  (params (CountDownTimer :type Float%20%28single-precision%29) (isAllPlayerReady? :type Boolean))
  ;[1 1 1] マッチング画面を更新する
  (CallFunction|RoCUpdateSelectUI CountDownTimer isAllPlayerReady?))

(event Custom|RoC_SelectInitialize
  ;[1 1 1] セレクト画面を表示
  (Utilities|IsValid (Variables|Select|GetMatchingUI)
    (:Is%20Valid
      _)
    (:Is%20Not%20Valid
      (bind _returnvalue (UserInterface|CreateWidget "/Game/Workspace/IoriFUKUNAKA/Blueprints/HeadUpDisplays/SelectHUD/WBP_Matching.WBP_Matching_C" self))
      (Variables|Select|SetMatchingUI _returnvalue)))
  (Input|SetInputModeGameandUI self (Variables|Select|GetMatchingUI) "DoNotLock" true)
  (Variables|/Script/Engine.PlayerController|SetbShowMouseCursor self true)
  (UserInterface|Viewport|AddtoViewport (Variables|Select|GetMatchingUI) 0))

(event Custom|RoS_SetIsReady
  (params (isReady :type Boolean))
  ;[1 1 1] 準備OK？
  (Variables|Select|SetisReady isReady)
  (CallFunction|EUpdateSelectUI))

(event Custom|E_UpdateSelectUI
  ;[1 1 1] マッチング情報を再更新
  (Networking|SwitchHasAuthority
    (:Authority
      (bind _gm_main (Variables|Default|GetGM%20Main)
        (:then
          (Default|ESetAllMatchingDataInfo _gm_main))
        (:else)))))

(event Custom|RoS_SetTempSkills
  (params (TempSkills :type Array%20of%20ST%20Skill%20Data%20Structures))
  ;[1 1 1] 選択中のスキル配列を更新
  (Variables|Select|SetTempSkills TempSkills)
  (CallFunction|EUpdateSelectUI))

(event Custom|RoC_RemoveSelectHUD
  (bind _matchingui (Variables|Select|GetMatchingUI))
  ;[1 1 1] マッチング画面を非表示にする
  (Utilities|IsValid _matchingui
    (:Is%20Valid
      (Widget|RemovefromParent _matchingui))))

(event Custom|RoC_SpawnVisual
  (params (Controllers :type Array%20of%20Player%20Controller%20Object%20References) (VisualActors :type Array%20of%20Actor%20Class%20References) (targetpoints :type Array%20of%20Target%20Point%20Object%20References))
  ;[1 1 1] マッチング画面用のアクタ
  (CallFunction|RoCClearVisualPlayer)
  (bind _visualactors (CallFunction|FSortVisualPlayers Controllers VisualActors))
  (for (_array_element _array_index) _visualactors
    (Game|SpawnActorfromClass _array_element (Transformation|GetActorTransform (Utilities|Array|Get(acopy) targetpoints _array_index)) "Undefined" self 0)))

(event Custom|E_ResultInitialize
  (params (gameClear :type Boolean) (ClearTime :type Float%20%28single-precision%29))
  ;[1 1 1] 初期化処理
  (CallFunction|RoCCreateResultWidget gameClear ClearTime))

(event Custom|RoC_CreateResultWidget
  (params (gameclear :type Boolean) (ClearTime :type Float%20%28single-precision%29))
  (bind _self self)
  ;[1 1 1] 初期化処理
  (if gameclear
    (bind _returnvalue (UserInterface|CreateWidget "/Game/Workspace/Yamashita/Blueprint/UI/Result/WBP_GameClear.WBP_GameClear_C" _self ClearTime))
    (UserInterface|Viewport|AddtoViewport _returnvalue 0)
    (else
      (bind _returnvalue_2 (UserInterface|CreateWidget "/Game/Workspace/Yamashita/Blueprint/UI/Result/WBP_GameOver.WBP_GameOver_C" _self))
      (UserInterface|Viewport|AddtoViewport _returnvalue_2 0)))
  (Input|SetInputModeGameOnly (Game|GetPlayerController 0))
  (Variables|Default|SetbShowMouseCursor self false))

(event Custom|ROC_PlaySE
  (params (Sound :type Sound%20Base%20Object%20Reference) (Location :type Vector) (AttenuationSettings :type Sound%20Attenuation%20Object%20Reference))
  (Audio|PlaySoundatLocation Sound Location "0, 0, 0" (Default|FGetSEVolume (.AsGI%20Yin%20Yang%20Project (Utilities|Casting|CastToGI_YinYangProject (Game|GetGameInstance)))) 1.0 0.0 AttenuationSettings 0 0))

(event Custom|ROC_PlayBGM
  (params (Sound :type Sound%20Base%20Object%20Reference))
  (Audio|PlaySound2D Sound (Default|FGetBGMVolume (.AsGI%20Yin%20Yang%20Project (Utilities|Casting|CastToGI_YinYangProject (Game|GetGameInstance)))) 1.0 0.0 0 0))

(fn ConstructionScript)

(fn FUseSkill
  (params (UseSkillNo :type Integer))
  (Class|BPIControllertoPlayer|ISkill(Message) (Pawn|GetControlledPawn) UseSkillNo))

(fn FSortVisualPlayers
  (params (Controllers :type Array%20of%20Player%20Controller%20Object%20References) (SpawnActors :type Array%20of%20Actor%20Class%20References))
  (for (_ _array_index) Controllers
    (Utilities|Array|Add (LocalVariables|GetActors) (Utilities|Array|Get(acopy) SpawnActors _array_index)))
  (LocalVariables|SetIndex0Actor (Utilities|Array|Get(acopy) (LocalVariables|GetActors)))
  (for (_array_element _array_index_2) Controllers
    (bind _asbp_player_controller (Utilities|Casting|CastToBP_PlayerController _array_element))
    (if (== (Variables|BP_PlayerController_C|GetPlayerID _asbp_player_controller) (Variables|Status|GetPlayerID))
      (Utilities|Array|SetArrayElem (LocalVariables|GetActors) 0 (Utilities|Array|Get(acopy) (LocalVariables|GetActors) _array_index_2) true)
      (Utilities|Array|SetArrayElem (LocalVariables|GetActors) _array_index_2 (LocalVariables|GetIndex0Actor) true)))
  (return (LocalVariables|GetActors)))