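; BP_RushAfterImage is a short-lived afterimage actor for Kirin's rush, showing a frozen copy of the enemy's pose.
; On spawn it gives each poseable mesh material slot a dynamic instance of MI_Kirin_Rush, stored in DynamicMats.
; It copies the pose from its owning BP_Kirin's skeletal mesh, then destroys itself after a brief delay.
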(event Custom|E_Trail
  (for _array_element (Rendering|Material|GetMaterials (Variables|Default|GetPoseableMesh))
    (bind _returnvalue (Rendering|Material|CreateDynamicMaterialInstance "/Game/Workspace/Yamashita/Material/Enemy/Kirin/MI_Kirin_Rush.MI_Kirin_Rush" "None" "None" :!class /Script/Engine.KismetMaterialLibrary))
    (bind _returnvalue_2 (Utilities|Array|Add (Variables|Default|GetDynamicMats) _returnvalue))
    (Rendering|Material|SetMaterial (Variables|Default|GetPoseableMesh) _returnvalue_2 _returnvalue)
    (bind _asbp_kirin (Utilities|Casting|CastToBP_Kirin (Components|GetOwner)))
    (Class|PoseableMeshComponent|CopyPosefromSkeletalComponent (Variables|Default|GetPoseableMesh) (Variables|/Script/Engine.Character|GetMesh _asbp_kirin))))

(event EventBeginPlay
  (CallFunction|ETrail)
  (Utilities|FlowControl|Delay 0.6)
  (Actor|DestroyActor))

(fn ConstructionScript)