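; BP_Thunder is a delayed lightning strike for the Kirin enemy, with a decal and a Niagara effect.
; On spawn it pauses the Niagara through a server-to-multicast event pair and starts a short timer.
; The strike event removes the decal, unpauses the effect and calls the owning enemy's box overlap check at its location.
; The actor destroys itself when the Niagara system finishes.
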(event Custom|E_PlayEffect
  (Components|DestroyComponent (Variables|Default|GetDecal))
  (CallFunction|RoSSetNiagaraEnable false)
  (bind _enemyref (Variables|Default|GetEnemyRef)
    (:then
      (Default|FBoxOverlap _enemyref (Transformation|GetActorLocation) "300.000000,300.000000,500.000000" false false 10))
    (:else)))

(event Custom|E_Destroy
  (params (PSystem :type Niagara%20Component%20Object%20Reference))
  (Actor|DestroyActor))

(event Custom|RoS_SetNiagaraEnable
  (params (bInRenderingEnabled :type Boolean))
  (CallFunction|MCSetNiagaraEnable bInRenderingEnabled))

(event Custom|MC_SetNiagaraEnable
  (params (bInRenderingEnabled :type Boolean))
  (Class|NiagaraComponent|SetPaused (Variables|Default|GetNiagara) bInRenderingEnabled))

(event EventBeginPlay
  (|CallParentFunction)
  (CallFunction|RoSSetNiagaraEnable true)
  (Utilities|Time|SetTimerbyEvent (EventDispatchers|CreateEvent :!event Custom|E_PlayEffect) 3.0)
  (EventDispatchers|BindEventtoOnSystemFinished (Variables|Default|GetNiagara) (EventDispatchers|CreateEvent :!event Custom|E_Destroy)))

(fn ConstructionScript
  (|CallParentFunction))