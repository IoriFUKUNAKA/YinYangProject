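; Girl variant of the YinYang player character, which tints its emissive material to match the player's element.
; Its override of F_InitilizeEachPlayer runs the parent logic, then reads the element from a valid PlayerState through an interface message.
; It creates a dynamic instance of MI_Girl_Emissive on mesh slot 1 and sets EmissiveColor from a color lookup indexed by that element.
; The event graph and construction script add no logic of their own.
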(event EventBeginPlay
  (|CallParentFunction) ; このノードは無効になっているため呼び出せません。\n機能をビルドするにはピンをドラッグしてください。
)

(event Collision|EventActorBeginOverlap
  (params (OtherActor :type Actor%20Object%20Reference)))

(event EventTick
  (params (DeltaSeconds :type Float%20%28single-precision%29)))

(fn ConstructionScript
  (|CallParentFunction))

(fn FInitilizeEachPlayer
  (|CallParentFunction)
  (bind _playerstate (Variables|Default|GetPlayerState)
    (:then
      (bind _element (Class|BPIControlPlayerStateData|IGetElement(Message) _playerstate))
      (bind _returnvalue (Rendering|Material|CreateDynamicMaterialInstance (Variables|Character|GetMesh) 1 "/Game/Workspace/IoriFUKUNAKA/Materials/LightingTest/YinYangCharacters/MI_Girl_Emissive.MI_Girl_Emissive" "None" :!class /Script/Engine.PrimitiveComponent))
      (bind _output_get (LocalVariables|SetEmissiveMI _returnvalue))
      (Rendering|Material|SetVectorParameterValue _output_get "EmissiveColor" (Utilities|Array|Get(acopy) (LocalVariables|GetElementEmissiveColor) (Math|Conversions|ToInteger(Byte) _element)) :!class /Script/Engine.MaterialInstanceDynamic)
      (Rendering|Material|SetMaterial (Variables|Character|GetMesh) 1 (LocalVariables|GetEmissiveMI)))
    (:else)))