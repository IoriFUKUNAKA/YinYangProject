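; BP_DOg is the Dog variant of the player's Chinese zodiac Jufu, a child Blueprint that extends its parent's initialization.
; On initialize, it casts a valid Instigator to BP_YinYangPlayer and turns that player toward a nearby enemy.
; It then binds to the player's Jufu anim notify begin and end events; the visible handlers switch on notify name but contain no actions.
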(event Custom|E_OnAnimNotifyBegin
  (params (NotifyName :type Name))
  (switch name NotifyName))

(event Custom|E_OnAnimNotifyEnd
  (params (NotifyName :type Name))
  (switch name NotifyName))

(fn ConstructionScript
  (|CallParentFunction))

(fn FonInitialize
  (|CallParentFunction)
  (bind _instigator (Variables|Default|GetInstigator)
    (:then
      (bind _asbp_yin_yang_player (Utilities|Casting|CastToBP_YinYangPlayer _instigator))
      (bind _rotation (Default|FRotationtoNearEnemy _asbp_yin_yang_player 5e+03))
      (Default|ROSSetActorRotation _asbp_yin_yang_player _rotation false)
      (EventDispatchers|BindEventtoOnJufuAnimNotifyBegin _asbp_yin_yang_player (EventDispatchers|CreateEvent :!event Custom|E_OnAnimNotifyBegin))
      (EventDispatchers|BindEventtoOnJufuAnimNotifyEnd _asbp_yin_yang_player (EventDispatchers|CreateEvent :!event Custom|E_OnAnimNotifyEnd)))
    (:else)))