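; BP_Suzaku is a player special attack actor, a Suzaku effect that strikes an enemy and buffs the party.
; On the server, the first valid enemy overlap triggers an explosion via the instigator, deals Attack-scaled Ka-element damage, then destroys the actor.
; It also self-destroys when its particle effect finishes.
; Any destruction, hit or not, applies a timed status buff twice to every player pawn with a BPC_BuffManager.
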(event OnComponentBeginOverlap(SpecialArea)
  (params (OverlappedComponent :type Primitive%20Component%20Object%20Reference) (OtherActor :type Actor%20Object%20Reference) (OtherComp :type Primitive%20Component%20Object%20Reference) (OtherBodyIndex :type Integer) (bFromSweep :type Boolean) (SweepResult :type Hit%20Result%20Structure%20%28by%20ref%29))
  (bind _returnvalue (Game|GetInstigator))
  (bind _returnvalue_2 (Transformation|GetActorLocation OtherActor))
  (bind _returnvalue_3 (Pawn|GetController _returnvalue))
  (Networking|SwitchHasAuthority
    (:Authority
      (if (Actor|ActorHasTag OtherActor "Enemy")
        (Utilities|IsValid _returnvalue
          (:Is%20Valid
            (Class|BPIControlEmitter|ISpawnSystematLocation(Message) _returnvalue "/Game/Workspace/Azuma/Effect/01fenix/NS_fenix_exprosion.NS_fenix_exprosion" (Math|Vector|MakeVector (.x _returnvalue_2) (.y _returnvalue_2) 0.0) "0, 0, 0" "1.000000,1.000000,1.000000" false)
            (bind _playerstate (Variables|/Script/Engine.Controller|GetPlayerState _returnvalue_3)
              (:then
                (bind _attack (Class|BPIControlPlayerState|IGetCurrentPlayerStatus(Message) _playerstate))
                (Game|Damage|ApplyDamage OtherActor (* _attack (Variables|Default|GetSpecialAttackMag)) _returnvalue_3 self "/Game/Workspace/IoriFUKUNAKA/Blueprints/Characters/Player/DamageType/D_GiveElementDamage_Ka.D_GiveElementDamage_Ka_C")
                (Actor|DestroyActor))
              (:else))))))))

(event Custom|E_OnSuzakuEffectFinished
  (params (PSystem :type Niagara%20Component%20Object%20Reference))
  (Actor|DestroyActor))

(event Custom|E_OnEndPlay
  (params (Actor :type Actor%20Object%20Reference) (EndPlayReason :type EEndPlayReason%20Enum :default "Destroyed"))
  (switch Utilities|FlowControl|Switch|SwitchonEEndPlayReason EndPlayReason
    (:Destroyed
      (CallFunction|FAdditionalEffect))))

(event EventBeginPlay
  (Networking|SwitchHasAuthority
    (:Authority
      (EventDispatchers|BindEventtoOnSystemFinished (Variables|Default|GetNS_Suzaku) (delegate Custom|E_OnSuzakuEffectFinished))
      (Game|BindEventtoOnEndPlay (EventDispatchers|CreateEvent :!event Custom|E_OnEndPlay)))))

(fn ConstructionScript
  (|CallParentFunction))

(fn FAdditionalEffect
  (for _array_element (Variables|/Script/Engine.GameStateBase|GetPlayerArray (Game|GetGameState))
    (bind _pawnprivate (Variables|/Script/Engine.PlayerState|GetPawnPrivate _array_element)
      (:then
        (Utilities|IsValid (Actor|GetComponentbyClass _pawnprivate "/Game/Workspace/IoriFUKUNAKA/Blueprints/Characters/BPC_BuffManager.BPC_BuffManager_C")
          (:Is%20Valid
            (for _index (range 0 1)
              (Default|ROCAddBuffEffect (Actor|GetComponentbyClass _pawnprivate "/Game/Workspace/IoriFUKUNAKA/Blueprints/Characters/BPC_BuffManager.BPC_BuffManager_C") "NewEnumerator0" 0.5 1e+01)))))
      (:else))))