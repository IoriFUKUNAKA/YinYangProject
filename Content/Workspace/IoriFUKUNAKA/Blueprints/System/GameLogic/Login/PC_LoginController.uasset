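; Player controller for the login screen, which plays the title BGM on BeginPlay and manages the login menu and server list widgets.
; Interface events create each widget once, then show it with UI-only input or remove it.
; Tick toggles the mouse cursor based on gamepad connection.
; Sound events handle BGM playback, stop and fade-out, plus 2D SE, scaling playback volume by GI_YinYangProject's settings.
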(event EventIShowLoginMenu
  ;[1 1 1] LoginMenuを表示する
  (Utilities|IsValid (Variables|Default|GetLoginMenu)
    (:Is%20Valid
      _)
    (:Is%20Not%20Valid
      (bind _returnvalue (UserInterface|CreateWidget "/Game/Workspace/IoriFUKUNAKA/Blueprints/HeadUpDisplays/LoginHUD/WBP_LoginMenu.WBP_LoginMenu_C" self))
      (Variables|Default|SetLoginMenu _returnvalue)))
  (Input|SetInputModeUIOnly self (Variables|Default|GetLoginMenu) "DoNotLock")
  (UserInterface|Viewport|AddtoViewport (Variables|Default|GetLoginMenu) 0)
  (Default|EInitializeLoginMenu (Variables|Default|GetLoginMenu)))

(event EventIRemoveLoginMenu
  ;[1 1 1] LoginMenuを非表示にする
  (Widget|RemovefromParent (Variables|Default|GetLoginMenu)))

(event EventIShowServerList
  ;[1 1 1] ServerListを表示する
  (Utilities|IsValid (Variables|Default|GetServerList)
    (:Is%20Valid
      _)
    (:Is%20Not%20Valid
      (bind _returnvalue (UserInterface|CreateWidget "/Game/Workspace/IoriFUKUNAKA/Blueprints/HeadUpDisplays/LoginHUD/WBP_ServerList.WBP_ServerList_C" self))
      (Variables|Default|SetServerList _returnvalue)))
  (Input|SetInputModeUIOnly self (Variables|Default|GetServerList) "DoNotLock")
  (UserInterface|Viewport|AddtoViewport (Variables|Default|GetServerList) 0))

(event EventIRemoveServerList
  ;[1 1 1] ServerListを非表示にする
  (Widget|RemovefromParent (Variables|Default|GetServerList)))

(event EventBeginPlay
  ;[1 1 1] BGM再生開始
  (CallFunction|EPlayBGM "/Game/Workspace/IoriFUKUNAKA/Sounds/SC_TitleBGM.SC_TitleBGM" 1.0))

(event EventTick
  (params (DeltaSeconds :type Float%20%28single-precision%29))
  ;[1 1 1] ゲームパッド接続によってカーソルの表示、非表示を切り替える
  (bind _returnvalue (Class|AppUtilBPLibrary|IsGamePadConnected))
  (if (Math|Boolean|NotEqual(Boolean) (not _returnvalue) (Variables|Default|GetbShowMouseCursor))
    (Variables|Default|SetbShowMouseCursor (not _returnvalue))))

(event Custom|E_StopBGM
  (Audio|Components|Audio|Stop (Variables|Default|GetBGMPlayer)))

(event Custom|E_FadeOutBGM
  (params (FadeOutDuration :type Float%20%28single-precision%29))
  (Audio|Components|Audio|FadeOut (Variables|Default|GetBGMPlayer) FadeOutDuration 0.0 "Linear" :!class /Script/Engine.AudioComponent))

(event Custom|E_PlaySE
  (params (Sound :type Sound%20Base%20Object%20Reference) (VolumeMultiplier :type Float%20%28single-precision%29))
  (Audio|PlaySound2D Sound (* VolumeMultiplier (Default|FGetSEVolume (.AsGI%20Yin%20Yang%20Project (Utilities|Casting|CastToGI_YinYangProject (Game|GetGameInstance))))) 1.0 0.0 0 0))

(event Custom|E_PlayBGM
  (params (Sound :type Sound%20Base%20Object%20Reference) (Volume :type Float%20%28single-precision%29))
  (Audio|Components|Audio|SetSound (Variables|Default|GetBGMPlayer) Sound)
  (Audio|Components|Audio|SetVolumeMultiplier (Variables|Default|GetBGMPlayer) (* Volume (Default|FGetBGMVolume (.AsGI%20Yin%20Yang%20Project (Utilities|Casting|CastToGI_YinYangProject (Game|GetGameInstance))))) :!class /Script/Engine.AudioComponent)
  (Audio|Components|Audio|Play (Variables|Default|GetBGMPlayer) 0.0))

(event EventIPlaySE
  (params (Sound :type Sound%20Base%20Object%20Reference) (Volume%20Multipier :type Float%20%28single-precision%29))
  (CallFunction|EPlaySE Sound Volume%20Multipier))

(fn ConstructionScript)