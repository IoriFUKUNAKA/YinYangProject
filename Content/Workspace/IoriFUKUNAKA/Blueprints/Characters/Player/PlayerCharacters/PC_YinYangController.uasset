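; Player controller for the networked YinYang game, running each player's presentation through the Matching, Ready, Main and Result phases.
; Phase events forward to ROC_ events that handle cameras, widgets, BGM/SE and input.
; Matching spawns visual characters from controller IDs, Ready binds player pawns into the enemy-appear sequence, and Result plays a clear sequence at Qilin or shows game over.
; It also shows element-colored, distance-scaled damage pop-ups and toggles the cursor by gamepad connection.
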(event Custom|ROC_OpenLevel
  (params (LevelName :type Name))
  ;[1 1 1] クライアントごとでレベルを遷移
  (Game|OpenLevel(byName) LevelName))

(event EventTick
  (params (DeltaSeconds :type Float%20%28single-precision%29))
  ;[1 1 1] ゲームパッド接続によってカーソルの表示、非表示を切り替える
  (bind _mygs (Variables|Ref|GetmyGS)
    (:then
      (if (and (Utilities|Enum|NotEqual(Enum) (Default|FGetinGameState _mygs) "NewEnumerator3") (Utilities|Enum|NotEqual(Enum) (Default|FGetinGameState _mygs) "NewEnumerator1"))
        (bind _returnvalue (Class|AppUtilBPLibrary|IsGamePadConnected))
        (if (Math|Boolean|NotEqual(Boolean) (not _returnvalue) (Variables|Default|GetbShowMouseCursor))
          (Variables|Default|SetbShowMouseCursor (not _returnvalue)))
        (else
          (Variables|Default|SetbShowMouseCursor false))))
    (:else)))

(event EventBeginPlay
  (bind _playerstate (Variables|GetPlayerState))
  ;[1 1 1] 初期化処理
  (Utilities|MWaitUntilwithTimeOut (Utilities|IsValid _playerstate) 5.0
    (:Success
      (bind _asps_yin_yang_player_state (Utilities|Casting|CastToPS_YinYangPlayerState _playerstate))
      (Variables|Ref|SetmyPS _asps_yin_yang_player_state)
      (bind _asgs_main (Utilities|Casting|CastToGS_Main (Game|GetGameState)))
      (Variables|Ref|SetmyGS _asgs_main))))

(event Custom|ROC_ShowMatchingUI
  ;[1 1 1] マッチング画面を表示
  (Utilities|IsValid (Variables|Matching|GetMatchingUI)
    (:Is%20Valid
      _)
    (:Is%20Not%20Valid
      (bind _returnvalue (UserInterface|CreateWidget "/Game/Workspace/IoriFUKUNAKA/Blueprints/HeadUpDisplays/SelectHUD/WBP_Matching.WBP_Matching_C" self))
      (Variables|Matching|SetMatchingUI _returnvalue)))
  (UserInterface|Viewport|AddtoViewport (Variables|Matching|GetMatchingUI) 0))

(event Custom|E_MatchingInitialize
  ;[1 1 1] 初期化処理
  (CallFunction|ROCBlendMatchingCamera)
  (CallFunction|ROCShowMatchingUI)
  (CallFunction|ROCPlayBGM "/Game/Workspace/IoriFUKUNAKA/Sounds/SC_MatchingBGM.SC_MatchingBGM" 1.0))

(event Custom|ROC_ClearVisualPlayer
  ;[1 1 1] 既存のマッチング画面用のキャラクターを削除
  (bind _outactors (Actor|GetAllActorsOfClass "/Game/Workspace/Yamashita/Blueprint/Player/VisualCharacter/BP_PlayerBaseForVisual.BP_PlayerBaseForVisual_C"))
  (for _array_element _outactors
    (Utilities|IsValid _array_element
      (:Is%20Valid
        (Actor|DestroyActor _array_element)))))

(event Custom|ROC_CreateVisualPlayer
  (params (InGameControllerIDs :type Array%20of%20Integers))
  (bind _visualplayerclass (Variables|Config|GetVisualPlayerClass))
  (bind _myps (Variables|Ref|GetmyPS))
  (bind _controller_id (Default|FGetControllerID _myps))
  ;[1 1 1] マッチング画面用のキャラクターを生成
  (Utilities|MWaitUntilwithTimeOut (Utilities|IsValid _myps) 5.0
    (:Success
      (for _array_element InGameControllerIDs
        (bind _spawnpointtransform (CallFunction|FGetSpawnPointsTransform))
        (if (Utilities|Array|IsValidIndex _visualplayerclass _controller_id)
          (Game|SpawnActorfromClass (Utilities|Array|Get(acopy) _visualplayerclass _array_element) (Math|Transform|MakeTransform (.location (Utilities|Array|Get(acopy) _spawnpointtransform (Math|Integer|SelectInt 0 1 (== _array_element _controller_id)))) (.rotation (Utilities|Array|Get(acopy) _spawnpointtransform (Math|Integer|SelectInt 0 1 (== _array_element _controller_id))))) "Undefined" 0 0))))))

(event Custom|E_MatchingUpdate
  ;[1 1 1] 更新処理
  (CallFunction|ROCUpdateMatchingUI))

(event Custom|ROC_BlendMatchingCamera
  ;[1 1 1] マッチング画面を表示
  (Utilities|FlowControl|Delay 0.0)
  (bind _outactors (Actor|GetAllActorswithTag "MatchingCamera"))
  (Game|Player|SetViewTargetwithBlend (Utilities|Array|Get(acopy) _outactors) 0.0 "VTBlend_Linear" 0.0 false))

(event Custom|ROC_UpdateMatchingUI
  ;[1 1 1] 更新処理
  (bind _matchingui (Variables|Matching|GetMatchingUI)
    (:then
      (Default|EUpdateMathingUI _matchingui))
    (:else)))

(event Custom|E_CreateVisualPlayer
  ;[1 1 1] マッチング画面用のキャラクターを生成
  (CallFunction|ROCClearVisualPlayer)
  (bind _ingamecontrollerids (CallFunction|FMakeinGamePlayerIDArray))
  (CallFunction|ROCCreateVisualPlayer _ingamecontrollerids))

(event Custom|E_MatchingFinalize
  ;[1 1 1] 終了処理
  (CallFunction|ROCRemoveMatchingUI)
  (CallFunction|ROCFadeOutBGM 1.0))

(event Custom|ROC_RemoveMatchingUI
  ;[1 1 1] 終了処理
  (bind _matchingui (Variables|Matching|GetMatchingUI)
    (:then
      (Widget|RemovefromParent _matchingui))
    (:else)))

(event Custom|E_ReadyInitialize
  ;[1 1 1] 初期化処理
  (CallFunction|ROCChangeCanInput false)
  (CallFunction|ROCPlayEnemyAppearSequence))

(event Custom|ROC_PlayEnemyAppearSequence
  ;[1 1 1] シーケンサー再生
  (bind (_outactor _returnvalue) (Sequencer|Player|CreateLevelSequencePlayer "/Game/Workspace/Yamashita/Cinematics/Sequence/LS_EnemyAppear.LS_EnemyAppear" (Utilities|Struct|MakeMovieSceneSequencePlaybackSettings false "(Value=0)" 1.0 0.0 false false false false false true false true)))
  (Variables|Ready|SetLevelSequenceActor_EnemyAppear _outactor)
  (bind _output_get (Variables|Ready|SetSequencePlayerEnemyAppear _returnvalue))
  (EventDispatchers|BindEventtoOnFinished _output_get (EventDispatchers|CreateEvent :!event Custom|E_SequenceEnd))
  (for _array_element (Variables|/Script/Engine.GameStateBase|GetPlayerArray (Game|GetGameState))
    (bind _asps_yin_yang_player_state (Utilities|Casting|CastToPS_YinYangPlayerState _array_element))
    (bind _asbp_yin_yang_player (Utilities|Casting|CastToBP_YinYangPlayer (Variables|/Script/Engine.PlayerState|GetPawnPrivate _array_element)))
    (switch int (Default|FGetControllerID _asps_yin_yang_player_state)
      (:0
        (Class|LevelSequenceActor|SetBinding (Variables|Ready|GetLevelSequenceActor_EnemyAppear) (|GetSequenceBinding) (Utilities|Array|MakeArray _asbp_yin_yang_player) false))
      (:1
        (Class|LevelSequenceActor|SetBinding (Variables|Ready|GetLevelSequenceActor_EnemyAppear) (|GetSequenceBinding) (Utilities|Array|MakeArray _asbp_yin_yang_player) false))))
  (bind _sequenceplayerenemyappear (Variables|Ready|GetSequencePlayerEnemyAppear)
    (:then
      (Sequencer|Player|Play _sequenceplayerenemyappear :!class /Script/MovieScene.MovieSceneSequencePlayer))
    (:else)))

(event Custom|E_ReadyFinalize
  ;[1 1 1] 終了処理
  (CallFunction|ROCChangeCanInput true))

(event Custom|E_SequenceEnd
  ;[1 1 1] シーケンサー終了時
  (Pawn|SetControlRotation self (Math|Rotator|MakeRotator 0.0 0.0 1.8e+02))
  (bind _sequenceplayerenemyappear (Variables|Ready|GetSequencePlayerEnemyAppear)
    (:then
      (Game|Player|SetViewTargetwithBlend (Components|GetOwner (Class|LevelSequencePlayer|GetActiveCameraComponent _sequenceplayerenemyappear)) 0.0 "VTBlend_Linear" 0.0 false)
      (Utilities|FlowControl|Delay 0.0)
      (Game|Player|SetViewTargetwithBlend (Pawn|GetControlledPawn) 0.7 "VTBlend_Linear" 0.0 false)
      (Utilities|FlowControl|Delay 0.7)
      (bind _sequenceplayerenemyappear_2 (Variables|Ready|GetSequencePlayerEnemyAppear)
        (:then
          (Sequencer|Player|Stop _sequenceplayerenemyappear_2 :!class /Script/MovieScene.MovieSceneSequencePlayer)
          (bind _myps (Variables|Ref|GetmyPS)
            (:then
              (Default|ROSSetIsEndSequence _myps true))
            (:else)))
        (:else)))
    (:else)))

(event Custom|E_MainInitialize
  (CallFunction|RoCSetInputModeGameOnly)
  (CallFunction|ROCShowMainUI)
  (CallFunction|ROCPlayBGM "/Game/Workspace/IoriFUKUNAKA/Sounds/SC_BattleBGM.SC_BattleBGM" 1.0))

(event Custom|ROC_ShowMainUI
  (bind _returnvalue (UserInterface|CreateWidget "/Game/Workspace/Yamashita/Blueprint/UI/MainGame/W_MainGameUI.W_MainGameUI_C" self))
  (bind _output_get (Variables|Main|SetMainUI _returnvalue))
  (UserInterface|Viewport|AddtoViewport _output_get 0))

(event Custom|RoC_SetInputModeGameOnly
  (Input|SetInputModeGameOnly self)
  (Variables|Default|SetbShowMouseCursor self false))

(event Custom|ROC_DamagePop
  (params (WorldPos :type Vector) (Damage :type Integer) (Element :type En_Elements%20Enum :default "NewEnumerator6"))
  (bind _returnvalue (Pawn|GetControlledPawn))
  (bind _returnvalue_2 (Math|Float|MakeLiteralFloat 5e+02))
  (bind _returnvalue_3 (Math|Float|MakeLiteralFloat 2e+03))
  (bind _returnvalue_4 (Transformation|GetActorLocation _returnvalue))
  (bind _returnvalue_5 (- _returnvalue_3 _returnvalue_2))
  (bind _returnvalue_6 (Math|Vector|Distance2D(Vector) WorldPos _returnvalue_4))
  (bind _returnvalue_7 (- _returnvalue_6 _returnvalue_2))
  (bind _returnvalue_8 (/ _returnvalue_7 _returnvalue_5))
  (bind _returnvalue_9 (Math|Float|Clamp(Float) _returnvalue_8))
  (bind _returnvalue_10 (Math|Float|Lerp 1.0 0.3 _returnvalue_9))
  (bind _returnvalue_11 (UserInterface|CreateWidget "/Game/Workspace/IoriFUKUNAKA/Blueprints/HeadUpDisplays/WBP_DamagePop.WBP_DamagePop_C" self (+ WorldPos "0.000000, 0,80.000000") (Math|Vector2D|MakeVector2D _returnvalue_10 _returnvalue_10) Damage))
  (Appearance|SetColorandOpacity _returnvalue_11 (Utilities|Select :Index Element :NewEnumerator6 "(R=0.791298,G=0.560251,B=0.134774,A=1.000000)" :NewEnumerator0 "(R=0.039546,G=0.456411,B=0.258183,A=1.000000)" :NewEnumerator1 "(R=0.806952,G=0.040915,B=0.022174,A=1.000000)" :NewEnumerator2 "" :NewEnumerator3 "(R=0.527115,G=0.564712,B=0.584079,A=1.000000)" :NewEnumerator4 "(R=0.072272,G=0.149960,B=0.450786,A=1.000000)") :!class /Script/UMG.UserWidget)
  (UserInterface|Viewport|AddtoViewport _returnvalue_11 0))

(event Custom|ROC_RemoveMainUI
  (bind _mainui (Variables|Main|GetMainUI)
    (:then
      (Widget|RemovefromParent _mainui))
    (:else)))

(event EventIDamagePopUI
  (params (WorldPos :type Vector :default "0, 0, 0") (Damage :type Integer) (Element :type En_Elements%20Enum :default "NewEnumerator6"))
  (CallFunction|ROCDamagePop WorldPos Damage Element))

(event Custom|E_ResultInitialize
  (Utilities|FlowControl|Sequence
    (:then_0
      (CallFunction|ROCRemoveMainUI))
    (:then_1
      (bind _mygs (Variables|Ref|GetmyGS)
        (:then
          (if (.isGameClear? (Default|FGetResultStatus _mygs))
            (CallFunction|ROCSetClearTime (.ClearTime (Default|FGetResultStatus _mygs)))
            (CallFunction|ROCPlayGameClearSequencer (Math|Transform|MakeTransform (Math|Vector|MakeVector (.X (Math|Vector|BreakVector (.location (Transformation|GetActorTransform (Default|FGetQilinRef _mygs))))) (.Y (Math|Vector|BreakVector (.location (Transformation|GetActorTransform (Default|FGetQilinRef _mygs))))) 0.0) (.rotation (Transformation|GetActorTransform (Default|FGetQilinRef _mygs)))))
            (else
              (CallFunction|ROCShowGameOverUI)
              (CallFunction|ROCSetInputModeResultUIOnly)
              (CallFunction|ROCStopBGM)
              (CallFunction|ROCPlayBGM "/Game/Workspace/IoriFUKUNAKA/Sounds/SC_GameOverME.SC_GameOverME" 1.0))))
        (:else)))))

(event Custom|ROC_ShowGameOverUI
  (bind _returnvalue (UserInterface|CreateWidget "/Game/Workspace/Yamashita/Blueprint/UI/Result/WBP_GameOver.WBP_GameOver_C" self))
  (bind _output_get (Variables|Result|SetResultUI _returnvalue))
  (UserInterface|Viewport|AddtoViewport _output_get 0))

(event Custom|ROC_SetInputModeResultUIOnly
  (bind _resultui (Variables|Result|GetResultUI)
    (:then
      (Input|SetInputModeUIOnly self _resultui "DoNotLock")
      (Variables|Default|SetbShowMouseCursor self true))
    (:else)))

(event Custom|ROC_PlayGameClearSequencer
  (params (Transform%20Origin :type Transform))
  (bind (_outactor _returnvalue) (Sequencer|Player|CreateLevelSequencePlayer "/Game/Workspace/Takagishi/Cinematics/Sequence/LS_GameClear.LS_GameClear" (Utilities|Struct|MakeMovieSceneSequencePlaybackSettings true "(Value=0)" 1.0 0.0 false false false false false false false true)))
  (bind _output_get (Variables|リザルト|SetGameClearSequencer _outactor))
  (Variables|/Script/LevelSequence.LevelSequenceActor|SetbOverrideInstanceData _output_get true)
  (bind _asdefault_level_sequence_instance_data (Utilities|Casting|CastToDefaultLevelSequenceInstanceData (Variables|/Script/LevelSequence.LevelSequenceActor|GetDefaultInstanceData _output_get)))
  (Variables|/Script/LevelSequence.DefaultLevelSequenceInstanceData|SetTransformOrigin _asdefault_level_sequence_instance_data Transform%20Origin)
  (bind _output_get_2 (Variables|リザルト|SetGameClearPlayer _returnvalue))
  (EventDispatchers|BindEventtoOnFinished _output_get_2 (EventDispatchers|CreateEvent :!event Custom|E_ShowGameClearUI)))

(event Custom|E_ShowGameClearUI
  (bind _returnvalue (UserInterface|CreateWidget "/Game/Workspace/Yamashita/Blueprint/UI/Result/WBP_GameClear.WBP_GameClear_C" self (Variables|Result|GetClearTime)))
  (bind _output_get (Variables|Result|SetResultUI _returnvalue))
  (UserInterface|Viewport|AddtoViewport _output_get 0))

(event Custom|ROC_SetClearTime
  (params (ClearTime :type Float%20%28single-precision%29))
  (Variables|Result|SetClearTime ClearTime))

(event Custom|ROC_StopBGM
  ;[1 1 1] BGM
  (Audio|Components|Audio|Stop (Variables|Default|GetBGMPlayer)))

(event Custom|ROC_FadeOutBGM
  (params (FadeOutDuration :type Float%20%28single-precision%29))
  ;[1 1 1] BGM
  (Audio|Components|Audio|FadeOut (Variables|Default|GetBGMPlayer) FadeOutDuration 0.0 "Linear" :!class /Script/Engine.AudioComponent))

(event Custom|ROC_ChangeCanInput
  (params (Enable? :type Boolean))
  (bind _returnvalue (Pawn|GetControlledPawn))
  (bind _self self)
  ;[1 1 1] 入力受付切り替え
  (if Enable?
    (Input|EnableInput _returnvalue _self)
    (else
      (Input|DisableInput _returnvalue _self))))

(event Custom|ROC_PlaySE
  (params (Sound :type Sound%20Base%20Object%20Reference) (VolumeMultiplier :type Float%20%28single-precision%29))
  ;[1 1 1] UIの効果音再生
  (Audio|PlaySound2D Sound (* VolumeMultiplier (Default|FGetSEVolume (.AsGI%20Yin%20Yang%20Project (Utilities|Casting|CastToGI_YinYangProject (Game|GetGameInstance))))) 1.0 0.0 0 0))

(event Custom|ROC_FadeInBGM
  (params (Sound :type Sound%20Base%20Object%20Reference) (VolumeMultiplier :type Float%20%28single-precision%29) (FadeInDuration :type Float%20%28single-precision%29))
  ;[1 1 1] BGM
  (Audio|Components|Audio|SetSound (Variables|Default|GetBGMPlayer) Sound)
  (Audio|Components|Audio|SetVolumeMultiplier (Variables|Default|GetBGMPlayer) 0.0 :!class /Script/Engine.AudioComponent)
  (Audio|Components|Audio|Play (Variables|Default|GetBGMPlayer) 0.0)
  (Audio|Components|Audio|FadeIn (Variables|Default|GetBGMPlayer) FadeInDuration (* VolumeMultiplier (Default|FGetBGMVolume (.AsGI%20Yin%20Yang%20Project (Utilities|Casting|CastToGI_YinYangProject (Game|GetGameInstance))))) 0.0 "Linear" :!class /Script/Engine.AudioComponent))

(event Custom|ROC_PlayBGM
  (params (Sound :type Sound%20Base%20Object%20Reference) (Volume :type Float%20%28single-precision%29))
  ;[1 1 1] BGM
  (Audio|Components|Audio|SetSound (Variables|Default|GetBGMPlayer) Sound)
  (Audio|Components|Audio|SetVolumeMultiplier (Variables|Default|GetBGMPlayer) (* Volume (Default|FGetBGMVolume (.AsGI%20Yin%20Yang%20Project (Utilities|Casting|CastToGI_YinYangProject (Game|GetGameInstance))))) :!class /Script/Engine.AudioComponent)
  (Audio|Components|Audio|Play (Variables|Default|GetBGMPlayer) 0.0))

(event EventISpawnSoundatLocation
  (params (Sound :type Sound%20Base%20Object%20Reference) (Location :type Vector :default "0, 0, 0") (Rotation :type Rotator :default "0, 0, 0") (Volume%20Multiplier :type Float%20%28single-precision%29) (Pitch%20Multiplier :type Float%20%28single-precision%29) (StartTime :type Float%20%28single-precision%29) (AttenuationSetting :type Sound%20Attenuation%20Object%20Reference) (ConcurrencySetting :type Sound%20Concurrency%20Object%20Reference))
  ;[1 1 1] UIの効果音再生
  (CallFunction|ROCPlaySE Sound Volume%20Multiplier))

(fn ConstructionScript)

(fn FGetSpawnPointsTransform
  (bind _outactors (Actor|GetAllActorswithTag "SpawnPoint"))
  (for (_array_element _array_index) _outactors
    (Utilities|Array|SetArrayElem (LocalVariables|GetTempTrsList) _array_index (Transformation|GetActorTransform _array_element) true))
  (return (LocalVariables|GetTempTrsList)))

(fn FGetPlayerState
  (return (Variables|Ref|GetmyPS)))

(fn FMakeinGamePlayerIDArray
  (bind _asgm_main (Utilities|Casting|CastToGM_Main (Game|GetGameMode)))
  (for _array_element (Default|FGetPlayerControllersRef _asgm_main)
    (bind _playerstate (Variables|/Script/Engine.Controller|GetPlayerState _array_element)
      (:then
        (bind _asps_yin_yang_player_state (Utilities|Casting|CastToPS_YinYangPlayerState _playerstate))
        (Utilities|Array|Add (LocalVariables|GetInGameControllerID) (Default|FGetControllerID _asps_yin_yang_player_state)))
      (:else)))
  (return (LocalVariables|GetInGameControllerID)))