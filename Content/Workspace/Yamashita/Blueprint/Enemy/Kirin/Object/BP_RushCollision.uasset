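; Rush attack hitbox for the Kirin enemy, covering the path swept from the rush's start point to the enemy's current position.
; Each tick it recenters on the midpoint, takes its yaw from the start-to-target direction and stretches the box's Y extent to half the travelled distance.
; Any overlapping actor receives the hit attack interface message.
; The rush-finish message freezes the box, which stays for a few seconds before destroying itself.
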(event OnComponentBeginOverlap(Box)
  (params (OverlappedComponent :type Primitive%20Component%20Object%20Reference) (OtherActor :type Actor%20Object%20Reference) (OtherComp :type Primitive%20Component%20Object%20Reference) (OtherBodyIndex :type Integer) (bFromSweep :type Boolean) (SweepResult :type Hit%20Result%20Structure%20%28by%20ref%29))
  (Class|BPIHitBoxtoCharacter|IHitAttack(Message) OtherActor))

(event EventBeginPlay)

(event Collision|EventActorBeginOverlap
  (params (OtherActor :type Actor%20Object%20Reference)))

(event EventTick
  (params (DeltaSeconds :type Float%20%28single-precision%29))
  (if (not (Variables|Default|GetisFinishRush))
    (Transformation|SetActorLocation (CallFunction|FCalcLocation) false false)
    (Transformation|SetActorRotation (CallFunction|FCalcRotation))
    (Components|Box|SetBoxExtent (Variables|Default|GetBox) (CallFunction|FCalcBoxElement 2e+02) true)))

(event EventIRushFinishKirin
  ;[1 1 1] 突進終了通知
  (Variables|Default|SetisFinishRush true)
  (Utilities|FlowControl|Delay 5.0)
  (Actor|DestroyActor))

(fn ConstructionScript
  (|CallParentFunction))

(fn FCalcRotation
  (bind _returnvalue (Transformation|GetActorRotation))
  (return (Math|Rotator|MakeRotator (.roll _returnvalue) (.pitch _returnvalue) (.yaw (Math|Rotator|MakeRotfromZ (- (Variables|Default|GetEnemy'sTarget) (Variables|Default|GetstartLoc)))))))

(fn FCalcLocation
  (return (* (+ (Variables|Default|GetstartLoc) (Transformation|GetActorLocation (Variables|Default|GetEnemyRef))) 0.5)))

(fn FCalcBoxElement
  (params (Large :type Float%20%28single-precision%29))
  (return (Math|Vector|MakeVector Large (* (Math|Vector|Distance(Vector) (Variables|Default|GetstartLoc) (Transformation|GetActorLocation (Variables|Default|GetEnemyRef))) 0.5) Large)))