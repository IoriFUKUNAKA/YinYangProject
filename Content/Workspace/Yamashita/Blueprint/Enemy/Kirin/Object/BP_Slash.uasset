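; BP_Slash is a moving slash object, filed under the Kirin enemy's objects.
; Each Tick it offsets its location by MoveDirection times Speed, scaled by world delta seconds, with no sweep.
; BeginPlay and ActorBeginOverlap are disabled stubs, so the graph holds no hit or lifetime logic, and nothing here sets the direction or speed.
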(event EventBeginPlay
  (|CallParentFunction) ; このノードは無効になっているため呼び出せません。\n機能をビルドするにはピンをドラッグしてください。
)

(event Collision|EventActorBeginOverlap
  (params (OtherActor :type Actor%20Object%20Reference)))

(event EventTick
  (params (DeltaSeconds :type Float%20%28single-precision%29))
  (Transformation|SetActorLocation (+ (Transformation|GetActorLocation) (* (* (Variables|Default|GetMoveDirection) (Variables|Default|GetSpeed)) (Utilities|Time|GetWorldDeltaSeconds))) false false))

(fn ConstructionScript
  (|CallParentFunction))