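; Base skill actor for the player, with empty initialize, update and destroy functions, apparently meant as overrides for specific skills.
; E_Initialize runs on authority, setting a lifespan, binding end-play, calling FInitialize and caching the owning BP_Player.
; Tick destroys non-stay skills when that owner enters a specific player state.
; FOnDestroy fires only when end-play reason is Destroyed; FOnUpdate is never called here.
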(event Custom|E_EndPlay
  (params (Actor :type Actor%20Object%20Reference) (EndPlayReason :type EEndPlayReason%20Enum :default "Destroyed"))
  (switch Utilities|FlowControl|Switch|SwitchonEEndPlayReason EndPlayReason
    (:Destroyed
      (CallFunction|FonDestroy))))

(event Custom|E_Initialize
  (Networking|SwitchHasAuthority
    (:Authority
      (Actor|SetLifeSpan (Variables|ステータス|GetLifeTime))
      (Game|AssignOnEndPlay (EventDispatchers|CreateEvent :!event Custom|E_EndPlay))
      (CallFunction|FInitialize)
      (bind _asbp_player (Utilities|Casting|CastToBP_Player (Components|GetOwner)))
      (Variables|Default|Setm_Owner _asbp_player))))

(event EventTick
  (params (DeltaSeconds :type Float%20%28single-precision%29))
  (if (not (Variables|ステータス|GetisStaySkill?))
    (bind _m_owner (Variables|Default|Getm_Owner)
      (:then
        (if (Utilities|Enum|Equal(Enum) (Default|FGetCurrentPlayerState _m_owner) "NewEnumerator6")
          (Actor|DestroyActor)))
      (:else))))

(fn ConstructionScript)

(fn FInitialize)

(fn FonDestroy)

(fn FonUpdate)