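; Weather actor that periodically spawns thunder strikes at random points, apparently for the Kirin enemy encounter.
; A looping 3-second timer checks the owner's tag message and skips spawning during Kirin's gimmick attack.
; Otherwise a RoS event spawns BP_Thunder with the same owner.
; The random-point helper ignores its Origin input, so strikes land only in the positive X/Y square from world origin, at zero height.
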(event Custom|E_SpawnThunder
  (bind _state (Class|BPIEnemy|IGetTag(Message) (Components|GetOwner)))
  (if (not (GameplayTags|MatchesTag _state "(TagName=\"Enemy.Attack.Kirin.GimickAttack\")" true))
    (CallFunction|RoSSpawnThunder)))

(event Custom|RoS_SpawnThunder
  ;[1 1 1] 生成
  (Game|SpawnActorfromClass "/Game/Workspace/Yamashita/Blueprint/Enemy/Kirin/Object/BP_Thunder.BP_Thunder_C" (Math|Conversions|ToTransform(Vector) (CallFunction|FGetRandomPoint "0, 0, 0" 1.3e+03)) "Undefined" (Components|GetOwner) 0.0 0))

(event EventBeginPlay
  (|CallParentFunction)
  (Utilities|Time|SetTimerbyEvent (delegate Custom|E_SpawnThunder) 3.0 true))

(fn ConstructionScript
  (|CallParentFunction))

(fn FGetRandomPoint
  (params (origin :type Vector) (radius :type Float%20%28single-precision%29))
  (bind _returnvalue (Math|Float|Absolute(Float) 0.0))
  (bind _returnvalue_2 (* -1 _returnvalue))
  (return (+ "0, 0, 0" (Math|Vector|MakeVector (Math|Random|RandomFloatinRange _returnvalue_2 radius) (Math|Random|RandomFloatinRange _returnvalue_2 radius) 0.0))))