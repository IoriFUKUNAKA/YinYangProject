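; Player character Blueprint for the YinYang game that configures combo attacks and the special-move cinematic for the player's element.
; On initialization it reads the element from PS_YinYangPlayerState and looks up the matching row in DT_ElementPlayerData.
; The row's three combo animations are stored through a multicast-named event.
; Its special Level Sequence goes to a client-named event that creates and caches a HUD-hiding sequence player without playing it.
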(event Custom|E_InitializePlayer
  (Utilities|FlowControl|Sequence
    (:then_0
      ;[1 1 1] 属性ごとのアニメーションの設定
      (bind _asps_yin_yang_player_state (Utilities|Casting|CastToPS_YinYangPlayerState (Variables|GetPlayerState)))
      (bind _output_get (Variables|Ref|SetmyPS _asps_yin_yang_player_state))
      (bind _returnvalue (Utilities|GetDataTableRow "/Game/Workspace/IoriFUKUNAKA/DataTable/DT_ElementPlayerData.DT_ElementPlayerData" (Utilities|Name|EnumtoName (Variables|/Game/Workspace/IoriFUKUNAKA/Blueprints/Characters/Player/PS_YinYangPlayerState.PS_YinYangPlayerState_C|GetElement _output_get)))
        (:then
          (CallFunction|MCSetComboAttackAnimations (Utilities|Array|MakeArray (.ComboAttack01 (Utilities|Struct|BreakST_PlayerElementData _returnvalue)) (.ComboAttack02 (Utilities|Struct|BreakST_PlayerElementData _returnvalue)) (.ComboAttack03 (Utilities|Struct|BreakST_PlayerElementData _returnvalue))))
          (CallFunction|ROCCreateSpecialSeaquencer (.SpecialLevelSequence (Utilities|Struct|BreakST_PlayerElementData _returnvalue))))))))

(event Custom|ROC_CreateSpecialSeaquencer
  (params (LevelSequence :type Level%20Sequence%20Object%20Reference))
  ;[1 1 1] 必殺技シーケンサーの生成
  (bind (_outactor _returnvalue) (Sequencer|Player|CreateLevelSequencePlayer LevelSequence (Utilities|Struct|MakeMovieSceneSequencePlaybackSettings false "(Value=0)" 1.0 0.0 false false false false false true)))
  (Variables|SpecialAttack|SetSpecialLevelSequenceActor _outactor)
  (Variables|SpecialAttack|SetLevelSequencePlayer _returnvalue))

(event Custom|MC_SetComboAttackAnimations
  (params (ComboAttackAnimations :type Array%20of%20Anim%20Montage%20Object%20References))
  ;[1 1 1] 属性ごとの攻撃アニメーションを設定
  (Variables|NormalAttack|SetComboAttackAnimations ComboAttackAnimations))

(fn ConstructionScript)