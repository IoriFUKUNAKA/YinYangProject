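; Base Blueprint for objects owned by an enemy, giving them a reference back to that enemy.
; On BeginPlay it casts its owner to BP_EnemyBase and stores it in EnemyRef, doing nothing if the cast fails.
; The interface getters for enemy stats, attacks, hate, targeting, game state and thunderbolt settings are empty stubs returning default values.
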(event EventBeginPlay
  (bind _asbp_enemy_base (Utilities|Casting|CastToBP_EnemyBase (Components|GetOwner)))
  (Variables|Default|SetEnemyRef _asbp_enemy_base))

(fn ConstructionScript)

(fn IGetAlivePlayerNum
  (return 0))

(fn IGetAttackHit?
  (return false))

(fn IGetAttackRange
  (return 0.0))

(fn IGetAttackStatus
  (params (tag :type Gameplay%20Tag%20Structure))
  (return (Utilities|Struct|MakeST_EnemyAttack "(TagName=\"\")" 0.0 0.0) false))

(fn IGetAttackTag
  (return ""))

(fn IGetCurrentGameState
  (return "NewEnumerator0"))

(fn IGetCurrentJuryoku
  (return 0.0))

(fn IGetDefaultMoveSpeed
  (return 0.0))

(fn IGetEnemyHealthState
  (return "NewEnumerator0"))

(fn IGetEnemyLarge
  (return 0.0))

(fn IGetEnemyTarget
  (return 0))

(fn IGetHateStageBorder
  (params (Stage :type En_EnemyStageState%20Enum :default "NewEnumerator7"))
  (return 0.0 false))

(fn IGetHighestHateCharacterLoc
  (return "0, 0, 0"))

(fn IGetHP
  (return 0))

(fn IGetIsBeforeAttackHit
  (return false))

(fn IGetIsMoveLocked
  (return false))

(fn IGetNorticeRange
  (return 0.0))

(fn IGetPlayersHateValue
  (return 0))

(fn IGetRadiusOfThunderBolt
  (return 0.0))

(fn IGetSightCharacters
  (return 0))

(fn IGetTag
  (return ""))

(fn IGetTimeforFallThunderBolt
  (return 0.0))

(fn IGetValidBuffEffectsEnemy
  (params (type :type En_BuffType%20Enum :default "NewEnumerator0"))
  (return 0))