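; BP_Ground is a stage ground object that generates enemy jump points on two concentric rings when play begins.
; It fills inside and outside 2D point arrays from cosine and sine scaled by each radius, centered on the origin, then stores both on GS_Main.
; The outside ring is offset half a step to stagger the points, and its angle step derives from the inside point count, not its own.
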(event EventBeginPlay
  (bind _insidecirclepointnum (Variables|Default|GetInSideCirclePointNum))
  (bind _returnvalue (Math|Conversions|ToFloat(Integer) _insidecirclepointnum))
  (bind _returnvalue_2 (/ 3.6e+02 _returnvalue))
  (bind _returnvalue_3 (Math|Float|MakeLiteralFloat _returnvalue_2))
  (bind _asgs_main (Utilities|Casting|CastToGS_Main (Game|GetGameState)))
  (Utilities|FlowControl|Sequence
    (:then_0
      (for _index (range 0 (- (Variables|Default|GetInSideCirclePointNum) 1))
        (Utilities|Array|SetArrayElem (Variables|Default|GetInSideEnemyJumpPoints) _index (* (Math|Vector2D|MakeVector2D (Math|Trig|Cos(Degrees) (* _index _returnvalue_3)) (Math|Trig|Sin(Degrees) (* _index _returnvalue_3))) (Variables|Default|GetInSideCircleRadius)) true))
      (Variables|/Game/Workspace/IoriFUKUNAKA/Blueprints/System/GameLogic/Main/GS_Main.GS_Main_C|SetInSideEnemyJumpPoints _asgs_main (Variables|Default|GetInSideEnemyJumpPoints)))
    (:then_1
      (for _index_2 (range 0 (- (Variables|Default|GetOutSideCirclePointNum) 1))
        (Utilities|Array|SetArrayElem (Variables|Default|GetOutSideEnemyJumpPoints) _index_2 (* (Math|Vector2D|MakeVector2D (Math|Trig|Cos(Degrees) (+ (* _index_2 _returnvalue_3) (* _returnvalue_3 0.5))) (Math|Trig|Sin(Degrees) (+ (* _index_2 _returnvalue_3) (* _returnvalue_3 0.5)))) (Variables|Default|GetOutSideCircleRadius)) true))
      (Variables|/Game/Workspace/IoriFUKUNAKA/Blueprints/System/GameLogic/Main/GS_Main.GS_Main_C|SetOutSideEnemyJumpPoints _asgs_main (Variables|Default|GetOutSideEnemyJumpPoints)))))

(fn ConstructionScript)