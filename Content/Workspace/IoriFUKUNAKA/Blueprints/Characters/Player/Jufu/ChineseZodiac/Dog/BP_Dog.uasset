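; Dog zodiac Jufu skill actor that turns the player toward a nearby enemy and performs an afterimage dash attack.
; Player animation notifies spawn the afterimage, drive the Through dash and apply Attack-scaled damage, then animation completion destroys the actor.
; The dash is a power-eased timeline with pawn collision set to overlap, gated by a circular-boundary check around the world origin.
; Its end spawns a slash effect and sphere-gathers enemies near the start point.
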(event Custom|E_OnAnimNotifyBegin
  (params (NotifyName :type Name))
  (bind _returnvalue (Components|GetOwner))
  (bind _returnvalue_2 (Transformation|GetActorLocation _returnvalue))
  (bind (_x _y) (Math|Vector|BreakVector _returnvalue_2))
  (switch name NotifyName
    (:Phantom
      (bind _instigatorplayer (Variables|プロパティ|GetInstigatorPlayer)
        (:then
          (Game|SpawnActorfromClass "/Game/Workspace/IoriFUKUNAKA/Blueprints/Characters/Player/Jufu/ChineseZodiac/Dog/BP_DogAfterImage.BP_DogAfterImage_C" (Math|Transform|MakeTransform (.location (Transformation|GetActorTransform _instigatorplayer)) (Math|Rotator|MakeRotator 0.0 0.0 (.Yaw (Math|Rotator|BreakRotator (.rotation (Transformation|GetActorTransform _instigatorplayer))))) "1,1,1") "Undefined" _instigatorplayer (Variables|Default|GetLife%20Time) (Variables|プロパティ|GetAfter%20Image%20HP) 0)
          (Default|ROSSwitchTrailEffect _instigatorplayer true))
        (:else)))
    (:Through
      (Utilities|FlowControl|Sequence
        (:then_0
          (bind _instigatorplayer_2 (Variables|プロパティ|GetInstigatorPlayer)
            (:then
              (Transformation|SetActorTransform _instigatorplayer_2 (Math|Transform|MakeTransform (Math|Vector|MakeVector _x _y (Variables|/Script/Engine.CapsuleComponent|GetCapsuleHalfHeight (Variables|/Script/Engine.Character|GetCapsuleComponent _instigatorplayer_2))) (Math|Rotator|MakeRotator 0.0 0.0 (.yaw (Math|Rotator|FindLookatRotation (Transformation|GetActorLocation _instigatorplayer_2) _returnvalue_2))) "1,1,1") true)
              (Default|ROSSetActorTransform _instigatorplayer_2 (Math|Transform|MakeTransform (Math|Vector|MakeVector _x _y (Variables|/Script/Engine.CapsuleComponent|GetCapsuleHalfHeight (Variables|/Script/Engine.Character|GetCapsuleComponent _instigatorplayer_2))) (Math|Rotator|MakeRotator 0.0 0.0 (.yaw (Math|Rotator|FindLookatRotation (Transformation|GetActorLocation _instigatorplayer_2) _returnvalue_2))) "1,1,1") true false))
            (:else)))
        (:then_1
          (bind _instigatorplayer_3 (Variables|プロパティ|GetInstigatorPlayer)
            (:then
              (Collision|SetCollisionResponsetoChannel (Variables|/Script/Engine.Character|GetCapsuleComponent _instigatorplayer_3) "ECC_Pawn" "ECR_Overlap")
              (Variables|Default|SetStartPosition (Math|Vector|MakeVector (.X (Math|Vector|BreakVector (.location (Transformation|GetActorTransform _instigatorplayer_3)))) (.Y (Math|Vector|BreakVector (.location (Transformation|GetActorTransform _instigatorplayer_3)))) (Variables|/Script/Engine.CapsuleComponent|GetCapsuleHalfHeight (Variables|/Script/Engine.Character|GetCapsuleComponent _instigatorplayer_3))))
              (Variables|Default|SetEndPosition (+ (Variables|Default|GetStartPosition) (* (Math|Vector|GetForwardVector (Math|Rotator|MakeRotator 0.0 0.0 (.Yaw (Math|Rotator|BreakRotator (.rotation (Transformation|GetActorTransform _instigatorplayer_3)))))) (Variables|プロパティ|GetThroughDistance))))
              (bind _intersectionpoint (CallFunction|FCalcIntersectionPoint (Variables|Default|GetStartPosition) (Variables|Default|GetEndPosition) 2e+03))
              (bind _output_get (Variables|Default|SetThroughBack? (> (Class|KismetMathLibrary|VSize2DSquared _intersectionpoint) (Class|KismetMathLibrary|VSizeXYSquared (Variables|Default|GetEndPosition)))))
              (if _output_get
                (Components|Timeline|PlayfromStart (Variables|Default|GetThrough))
                (else
                  (Default|ROSSwitchTrailEffect (Variables|プロパティ|GetInstigatorPlayer) false))))
            (:else)))))
    (:Damage
      (bind _instigatorplayer_4 (Variables|プロパティ|GetInstigatorPlayer)
        (:then
          (bind _attack (Class|BPIControlPlayerState|IGetCurrentPlayerStatus(Message) (Variables|/Script/Engine.Pawn|GetPlayerState _instigatorplayer_4)))
          (for _array_element (Variables|Default|GetHitEnemys)
            (Default|ROSApplyDamage _instigatorplayer_4 (Components|GetOwner) (* _attack 1.5) (Pawn|GetController _instigatorplayer_4) self)))
        (:else)))))

(event Custom|E_BindOnJufuAnimNotifyEvent
  (bind _instigatorplayer (Variables|プロパティ|GetInstigatorPlayer)
    (:then
      (EventDispatchers|BindEventtoOnJufuAnimNotifyBegin _instigatorplayer (EventDispatchers|CreateEvent :!event Custom|E_OnAnimNotifyBegin))
      (EventDispatchers|BindEventtoOnJufuAnimNotifyEnd _instigatorplayer (EventDispatchers|CreateEvent :!event Custom|E_OnAnimNotifyEnd))
      (EventDispatchers|BindEventtoOnJufuAnimCompleated _instigatorplayer (EventDispatchers|CreateEvent :!event Custom|E_OnJufuAnimCompleated)))
    (:else)))

(event Custom|MC_InitializeDog
  (bind _instigator (Variables|Default|GetInstigator)
    (:then
      (bind _asbp_yin_yang_player (Utilities|Casting|CastToBP_YinYangPlayer _instigator))
      (bind _output_get (Variables|プロパティ|SetInstigatorPlayer _asbp_yin_yang_player))
      (bind _rotation (Default|FRotationtoNearEnemy _output_get 5e+03))
      (Transformation|SetActorRotation _output_get _rotation)
      (CallFunction|EBindonJufuAnimNotifyEvent))
    (:else)))

(event Custom|E_OnAnimNotifyEnd
  (params (NotifyName :type Name))
  (switch name NotifyName
    (:Through
      (Audio|Components|Audio|Stop (Variables|Default|GetThrough))
      (bind _instigatorplayer (Variables|プロパティ|GetInstigatorPlayer)
        (:then
          (Collision|SetCollisionResponsetoChannel (Variables|/Script/Engine.Character|GetCapsuleComponent _instigatorplayer) "ECC_Pawn" "ECR_Block")
          (Default|ROSSwitchTrailEffect _instigatorplayer false)
          (Class|BPIControlEmitter|ISpawnSystematLocation(Message) (Variables|Default|GetInstigator) "/Game/Workspace/Nishii/NS/NS_E_SwordFlash_001_00.NS_E_SwordFlash_001_00" (Math|Vector|MakeVector (.X (Math|Vector|BreakVector (+ (Variables|Default|GetStartPosition) (* (Math|Vector|GetForwardVector (.rotation (Transformation|GetActorTransform _instigatorplayer))) 1.5e+02)))) (.Y (Math|Vector|BreakVector (+ (Variables|Default|GetStartPosition) (* (Math|Vector|GetForwardVector (.rotation (Transformation|GetActorTransform _instigatorplayer))) 1.5e+02)))) 2.5e+02) (.rotation (Transformation|GetActorTransform _instigatorplayer)) "1.000000,1.000000,1.000000")
          (bind _outactors (Collision|SphereOverlapActors (Math|Vector|MakeVector (.X (Math|Vector|BreakVector (+ (Variables|Default|GetStartPosition) (* (Math|Vector|GetForwardVector (.rotation (Transformation|GetActorTransform _instigatorplayer))) 1.5e+02)))) (.Y (Math|Vector|BreakVector (+ (Variables|Default|GetStartPosition) (* (Math|Vector|GetForwardVector (.rotation (Transformation|GetActorTransform _instigatorplayer))) 1.5e+02)))) 2.5e+02) 2.5e+02 (Utilities|Array|MakeArray "ObjectTypeQuery3") "/Game/Workspace/Yamashita/Blueprint/Base/BP_EnemyBase.BP_EnemyBase_C"))
          (Variables|Default|SetHitEnemys _outactors))
        (:else)))))

(event Custom|E_OnJufuAnimCompleated
  (Default|ROSDestroyActor (Variables|プロパティ|GetInstigatorPlayer) self))

(fn ConstructionScript
  (|CallParentFunction))

(fn FonInitialize
  (|CallParentFunction)
  (CallFunction|MCInitializeDog))

(fn FCalcIntersectionPoint
  (params (StartPosition :type Vector) (EndPosition :type Vector) (Radius :type Float%20%28single-precision%29))
  (bind _returnvalue (Math|Float|Square Radius))
  (bind _output_get (LocalVariables|Set_StartPosition (Math|Conversions|ToVector2D(Vector) StartPosition)))
  (bind _output_get_2 (LocalVariables|Set_EndPosition (Math|Conversions|ToVector2D(Vector) EndPosition)))
  (LocalVariables|SetvecPE (- _output_get_2 _output_get))
  (if (<= (Class|KismetMathLibrary|VSize2DSquared _output_get) _returnvalue)
    (return (+ (LocalVariables|Get_StartPosition) (* (LocalVariables|GetvecPE) (/ (- (- _returnvalue (Class|KismetMathLibrary|VSize2DSquared (LocalVariables|Get_StartPosition))) (Class|KismetMathLibrary|VSize2DSquared (LocalVariables|GetvecPE))) (* 2.0 (Math|Vector2D|DotProduct(2D) (LocalVariables|Get_StartPosition) (LocalVariables|GetvecPE)))))))
    (else
      (return (LocalVariables|Get_StartPosition)))))