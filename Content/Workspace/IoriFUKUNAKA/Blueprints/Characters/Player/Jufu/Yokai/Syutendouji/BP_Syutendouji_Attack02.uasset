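; Attack02 hit actor for the Syutendouji yokai, dealing player Attack times a multiplier as damage through its owning BP_Syutendouji.
; An enemy overlapping AttackArea takes Syutendoji-type damage, then the actor destroys itself.
; Once bound to the owner's OnLastAttack, it instead hits everything in EnemyList with Byakko special-attack damage plus a debuff, then destroys itself.
; EnemyList is not filled in this graph, and the movable-area call is disconnected.
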(event OnComponentBeginOverlap(AttackArea)
  (params (OverlappedComponent :type Primitive%20Component%20Object%20Reference) (OtherActor :type Actor%20Object%20Reference) (OtherComp :type Primitive%20Component%20Object%20Reference) (OtherBodyIndex :type Integer) (bFromSweep :type Boolean) (SweepResult :type Hit%20Result%20Structure%20%28by%20ref%29))
  (bind _returnvalue (Components|GetOwner))
  (if (Actor|ActorHasTag OtherActor "Enemy")
    (bind _playerstate (Variables|/Script/Engine.Pawn|GetPlayerState (Game|GetInstigator))
      (:then
        (bind _attack (Class|BPIControlPlayerState|IGetCurrentPlayerStatus(Message) _playerstate))
        (bind _asbp_syutendouji (Utilities|Casting|CastToBP_Syutendouji _returnvalue))
        (Default|ROSApplyDamage _asbp_syutendouji OtherActor (* _attack (Variables|Default|GetAttack%20Magnification)) (Game|GetInstigatorController) _returnvalue "/Game/Workspace/IoriFUKUNAKA/Blueprints/Characters/Player/DamageType/Jufu/D_Syutendoji.D_Syutendoji_C")
        (Actor|DestroyActor))
      (:else))))

(event Custom|E_LastAttack
  (bind _returnvalue (Components|GetOwner))
  (bind _playerstate (Variables|/Script/Engine.Pawn|GetPlayerState (Game|GetInstigator))
    (:then
      (bind _attack (Class|BPIControlPlayerState|IGetCurrentPlayerStatus(Message) _playerstate))
      (bind _asbp_syutendouji (Utilities|Casting|CastToBP_Syutendouji _returnvalue))
      (for _array_element (Variables|Default|GetEnemyList)
        (Default|ROSApplyDamage _asbp_syutendouji _array_element (* _attack (Variables|Default|GetAttack%20Magnification)) (Game|GetInstigatorController) _returnvalue "/Game/Workspace/IoriFUKUNAKA/Blueprints/Characters/Player/DamageType/SpecialAttack/D_SpecialAttack_Byakko.D_SpecialAttack_Byakko_C")
        (Default|ROSDebuff _asbp_syutendouji _array_element))
      (Actor|DestroyActor))
    (:else)))

(event Custom|E_BindOnLastAttack
  (bind _asbp_syutendouji (Utilities|Casting|CastToBP_Syutendouji (Components|GetOwner)))
  (EventDispatchers|BindEventtoOnLastAttack _asbp_syutendouji (delegate Custom|E_LastAttack)))

(fn ConstructionScript)