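; BP_FireFox is a yokai actor that launches a volley of nine BP_Kitsunebi projectiles from its Instigator at its Owner.
; On initialize, it spawns them in a ring perpendicular to the horizontal Instigator-to-Owner direction, centered at an offset from the Instigator.
; Each gets a forward, outward-splayed injection direction and the Owner as target.
; On update, it prunes invalid projectiles and destroys itself once none remain.
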(fn ConstructionScript
  (|CallParentFunction))

(fn FonInitialize
  (|CallParentFunction)
  (bind _instigator (Variables|Default|GetInstigator)
    (:then
      (Private|FInstantiateKitsunebi 9))
    (:else)))

(fn FInstantiateKitsunebi
  (params (InstantiateNum :type Integer))
  (bind _returnvalue (Components|GetOwner))
  (bind _kitsunebicenteroffset (Variables|Config|GetKitsunebiCenterOffset))
  (bind _kitsunebiradius (Variables|Config|GetKitsunebiRadius))
  (bind (_x _y _z) (Math|Vector|BreakVector _kitsunebicenteroffset))
  (bind _returnvalue_2 (Transformation|GetActorLocation _returnvalue))
  (bind (_x_2 _y_2) (Math|Vector|BreakVector _returnvalue_2))
  (LocalVariables|SetKitsunebiInterval%28Degree%29 (Math|Float|SelectFloat (/ 3.6e+02 (Math|Conversions|ToFloat(Integer) InstantiateNum)) 0.0 (> InstantiateNum 0)))
  (bind _instigator (Variables|Default|GetInstigator)
    (:then
      (LocalVariables|SetCenterPos (+ (Transformation|GetActorLocation _instigator) (* (.X (Math|Rotator|BreakRotIntoAxes (Math|Rotator|FindLookatRotation (Math|Vector|MakeVector (.X (Math|Vector|BreakVector (Transformation|GetActorLocation _instigator))) (.Y (Math|Vector|BreakVector (Transformation|GetActorLocation _instigator))) 0.0) (Math|Vector|MakeVector _x_2 _y_2 0.0)))) _x) (* (.Y (Math|Rotator|BreakRotIntoAxes (Math|Rotator|FindLookatRotation (Math|Vector|MakeVector (.X (Math|Vector|BreakVector (Transformation|GetActorLocation _instigator))) (.Y (Math|Vector|BreakVector (Transformation|GetActorLocation _instigator))) 0.0) (Math|Vector|MakeVector _x_2 _y_2 0.0)))) _y) (* (.Z (Math|Rotator|BreakRotIntoAxes (Math|Rotator|FindLookatRotation (Math|Vector|MakeVector (.X (Math|Vector|BreakVector (Transformation|GetActorLocation _instigator))) (.Y (Math|Vector|BreakVector (Transformation|GetActorLocation _instigator))) 0.0) (Math|Vector|MakeVector _x_2 _y_2 0.0)))) _z)))
      (for _index (range 0 (- InstantiateNum 1))
        (LocalVariables|SetLoopIndex _index)
        (bind _output_get (LocalVariables|SetSpawnPos (+ (+ (Transformation|GetActorLocation _instigator) (* (.X (Math|Rotator|BreakRotIntoAxes (Math|Rotator|FindLookatRotation (Math|Vector|MakeVector (.X (Math|Vector|BreakVector (Transformation|GetActorLocation _instigator))) (.Y (Math|Vector|BreakVector (Transformation|GetActorLocation _instigator))) 0.0) (Math|Vector|MakeVector _x_2 _y_2 0.0)))) _x) (* (.Y (Math|Rotator|BreakRotIntoAxes (Math|Rotator|FindLookatRotation (Math|Vector|MakeVector (.X (Math|Vector|BreakVector (Transformation|GetActorLocation _instigator))) (.Y (Math|Vector|BreakVector (Transformation|GetActorLocation _instigator))) 0.0) (Math|Vector|MakeVector _x_2 _y_2 0.0)))) _y) (* (.Z (Math|Rotator|BreakRotIntoAxes (Math|Rotator|FindLookatRotation (Math|Vector|MakeVector (.X (Math|Vector|BreakVector (Transformation|GetActorLocation _instigator))) (.Y (Math|Vector|BreakVector (Transformation|GetActorLocation _instigator))) 0.0) (Math|Vector|MakeVector _x_2 _y_2 0.0)))) _z)) (* (.Y (Math|Rotator|BreakRotIntoAxes (Math|Rotator|FindLookatRotation (Math|Vector|MakeVector (.X (Math|Vector|BreakVector (Transformation|GetActorLocation _instigator))) (.Y (Math|Vector|BreakVector (Transformation|GetActorLocation _instigator))) 0.0) (Math|Vector|MakeVector _x_2 _y_2 0.0)))) (* (Math|Trig|Cos(Degrees) (+ (* (LocalVariables|GetLoopIndex) (LocalVariables|GetKitsunebiInterval%28Degree%29)) 9e+01)) _kitsunebiradius)) (* (.Z (Math|Rotator|BreakRotIntoAxes (Math|Rotator|FindLookatRotation (Math|Vector|MakeVector (.X (Math|Vector|BreakVector (Transformation|GetActorLocation _instigator))) (.Y (Math|Vector|BreakVector (Transformation|GetActorLocation _instigator))) 0.0) (Math|Vector|MakeVector _x_2 _y_2 0.0)))) (* _kitsunebiradius (Math|Trig|Sin(Degrees) (+ (* (LocalVariables|GetLoopIndex) (LocalVariables|GetKitsunebiInterval%28Degree%29)) 9e+01)))))))
        (bind _returnvalue_3 (Game|SpawnActorfromClass "/Game/Workspace/IoriFUKUNAKA/Blueprints/Characters/Player/Jufu/Yokai/FireFox/BP_Kitsunebi.BP_Kitsunebi_C" (Math|Transform|MakeTransform _output_get (Math|Rotator|FindLookatRotation (Math|Vector|MakeVector (.X (Math|Vector|BreakVector (Transformation|GetActorLocation _instigator))) (.Y (Math|Vector|BreakVector (Transformation|GetActorLocation _instigator))) 0.0) (Math|Vector|MakeVector _x_2 _y_2 0.0)) "1,1,1") "Undefined" 0 (Math|Vector|Normalize (+ (.X (Math|Rotator|BreakRotIntoAxes (Math|Rotator|FindLookatRotation (Math|Vector|MakeVector (.X (Math|Vector|BreakVector (Transformation|GetActorLocation _instigator))) (.Y (Math|Vector|BreakVector (Transformation|GetActorLocation _instigator))) 0.0) (Math|Vector|MakeVector _x_2 _y_2 0.0)))) (* (Math|Vector|Normalize (- (LocalVariables|GetSpawnPos) (LocalVariables|GetCenterPos))) 0.5))) (Components|GetOwner) (Game|GetInstigator)))
        (Utilities|Array|Add (Variables|Ref|GetKitsunebiArray) _returnvalue_3)
        (Default|EInitializeKitsunebi _returnvalue_3))
      (return))
    (:else)))

(fn FonUpdate
  (|CallParentFunction)
  (bind (_arrayindex _arrayelement) (Utilities|Array|ReverseforEachLoop (Variables|Ref|GetKitsunebiArray))
    (:LoopBody
      (Utilities|IsValid _arrayelement
        (:Is%20Not%20Valid
          (Utilities|Array|RemoveIndex (Variables|Ref|GetKitsunebiArray) _arrayindex))))
    (:Completed
      (if (<= (Utilities|Array|Length (Variables|Ref|GetKitsunebiArray)) 0)
        (Actor|DestroyActor)))))