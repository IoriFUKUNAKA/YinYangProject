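; BP_Tengu is the Tengu yokai Jufu actor, which makes the instigating player throw a shuriken.
; On initialization it snaps the player toward a nearby enemy and binds to the player's Jufu animation events.
; The Rotate notify drives a timeline that eases the player toward this actor's owner, while Active spawns BP_Shuriken at an offset through the player.
; Animation completion destroys the actor through the player's ROS call.
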(event Custom|E_OnJufuAnimCompleated
  (Default|ROSDestroyActor (Variables|Default|GetInstigatorPlayer) self))

(event Custom|E_OnAnimNotifyEnd
  (params (NotifyName :type Name))
  (bind _returnvalue (Components|GetOwner))
  (bind _instigatorplayer (Variables|Default|GetInstigatorPlayer))
  (bind _returnvalue_2 (Transformation|GetActorLocation _returnvalue))
  (bind _returnvalue_3 (Transformation|GetActorLocation _instigatorplayer))
  (bind (_x _y) (Math|Vector|BreakVector _returnvalue_2))
  (bind (_x_2 _y_2) (Math|Vector|BreakVector _returnvalue_3))
  (switch name NotifyName
    (:Rotate
      (bind _rotaterate (Timeline|Rotate Stop)
        (:Update
          (Transformation|SetActorRotation (Variables|Default|GetInstigatorPlayer) (Math|Rotator|Lerp(Rotator) (Transformation|GetActorRotation _instigatorplayer) (Math|Rotator|FindLookatRotation (Math|Vector|MakeVector _x_2 _y_2 0.0) (Math|Vector|MakeVector _x _y 0.0)) (Math|Float|Square _rotaterate) true))
          (Default|ROSSetActorRotation (Variables|Default|GetInstigatorPlayer) (Math|Rotator|Lerp(Rotator) (Transformation|GetActorRotation _instigatorplayer) (Math|Rotator|FindLookatRotation (Math|Vector|MakeVector _x_2 _y_2 0.0) (Math|Vector|MakeVector _x _y 0.0)) (Math|Float|Square _rotaterate) true) false))))))

(event Custom|E_OnAnimNotifyBegin
  (params (NotifyName :type Name))
  (bind _returnvalue (Components|GetOwner))
  (bind _instigatorplayer (Variables|Default|GetInstigatorPlayer))
  (bind _instigatorplayer_2 (Variables|Default|GetInstigatorPlayer))
  (bind _offset (Variables|Default|GetOffset))
  (bind _instigatorplayer_3 (Variables|Default|GetInstigatorPlayer))
  (bind _returnvalue_2 (Transformation|GetActorTransform _instigatorplayer_3))
  (bind _returnvalue_3 (Transformation|GetActorLocation _returnvalue))
  (bind (_x _y _z) (Math|Vector|BreakVector _offset))
  (bind _returnvalue_4 (Transformation|GetActorLocation _instigatorplayer_2))
  (bind (_x_2 _y_2) (Math|Vector|BreakVector _returnvalue_3))
  (bind (_x_3 _y_3) (Math|Vector|BreakVector _returnvalue_4))
  (bind (_x_4 _y_4 _z_2) (Math|Rotator|BreakRotIntoAxes (.rotation _returnvalue_2)))
  (switch name NotifyName
    (:Rotate
      (bind _rotaterate (Timeline|Rotate PlayFromStart)
        (:Update
          (Transformation|SetActorRotation (Variables|Default|GetInstigatorPlayer) (Math|Rotator|Lerp(Rotator) (Transformation|GetActorRotation _instigatorplayer_2) (Math|Rotator|FindLookatRotation (Math|Vector|MakeVector _x_3 _y_3 0.0) (Math|Vector|MakeVector _x_2 _y_2 0.0)) (Math|Float|Square _rotaterate) true))
          (Default|ROSSetActorRotation (Variables|Default|GetInstigatorPlayer) (Math|Rotator|Lerp(Rotator) (Transformation|GetActorRotation _instigatorplayer_2) (Math|Rotator|FindLookatRotation (Math|Vector|MakeVector _x_3 _y_3 0.0) (Math|Vector|MakeVector _x_2 _y_2 0.0)) (Math|Float|Square _rotaterate) true) false))))
    (:Active
      (Default|ROSSpawnActorfromClass _instigatorplayer "/Game/Workspace/IoriFUKUNAKA/Blueprints/Characters/Player/Jufu/Yokai/Tengu/BP_Shuriken.BP_Shuriken_C" (Math|Transform|MakeTransform (+ (.location _returnvalue_2) (* _x_4 _x) (* _y_4 _y) (* _z_2 _z)) (.rotation _returnvalue_2) "1,1,1") 0 _instigatorplayer))))

(event Custom|E_BindOnJufuAnimNotifyEvent
  (bind _instigatorplayer (Variables|Default|GetInstigatorPlayer)
    (:then
      (EventDispatchers|BindEventtoOnJufuAnimNotifyBegin _instigatorplayer (EventDispatchers|CreateEvent :!event Custom|E_OnAnimNotifyBegin))
      (EventDispatchers|BindEventtoOnJufuAnimNotifyEnd _instigatorplayer (EventDispatchers|CreateEvent :!event Custom|E_OnAnimNotifyEnd))
      (EventDispatchers|BindEventtoOnJufuAnimCompleated _instigatorplayer (EventDispatchers|CreateEvent :!event Custom|E_OnJufuAnimCompleated)))
    (:else)))

(event Custom|MC_InitializeWadatsumi
  (bind _instigator (Variables|Default|GetInstigator)
    (:then
      (bind _asbp_yin_yang_player (Utilities|Casting|CastToBP_YinYangPlayer _instigator))
      (bind _output_get (Variables|Default|SetInstigatorPlayer _asbp_yin_yang_player))
      (bind _rotation (Default|FRotationtoNearEnemy _output_get 5e+03 true))
      (Transformation|SetActorRotation _output_get _rotation)
      (CallFunction|EBindonJufuAnimNotifyEvent))
    (:else)))

(fn ConstructionScript
  (|CallParentFunction))

(fn FonInitialize
  (|CallParentFunction)
  (CallFunction|MCInitializeWadatsumi))