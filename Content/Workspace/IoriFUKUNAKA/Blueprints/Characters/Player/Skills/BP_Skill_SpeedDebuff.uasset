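; BP_Skill_SpeedDebuff is a player skill that applies a timed status effect, by its name a speed debuff, to a nearby enemy.
; On initialization it asks the owner's game manager for a near enemy within a fixed check distance.
; If one is found, it adds a new status data object to that enemy's status manager, plays a status-down sound there and destroys itself.
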(fn ConstructionScript
  (|CallParentFunction))

(fn FInitialize
  (|CallParentFunction)
  (bind _m_owner (Variables|Default|Getm_Owner)
    (:then
      (bind _m_gamemanager (Variables|/Game/Workspace/IoriFUKUNAKA/Blueprints/Characters/Player/BP_Player.BP_Player_C|Getm_GameManager _m_owner)
        (:then
          (bind (_isvalid_ _nearenemy) (Default|FGetNearEnemyfromPlayer _m_gamemanager (Transformation|GetActorLocation _m_owner) 8e+03))
          (if _isvalid_
            (bind _returnvalue (Game|ConstructObjectfromClass "/Game/Workspace/IoriFUKUNAKA/Blueprints/Characters/DataObject/BP_StatusData.BP_StatusData_C" (Variables|/Game/Workspace/Yamashita/Blueprint/Base/BP_EnemyBase.BP_EnemyBase_C|GetBPC_StatusManager _nearenemy) "NewEnumerator2" (Variables|Default|GetEffect%20Value) (Variables|Default|GetEffectLife%20Time)))
            (Default|EAddEffect (Variables|/Game/Workspace/Yamashita/Blueprint/Base/BP_EnemyBase.BP_EnemyBase_C|GetBPC_StatusManager _nearenemy) _returnvalue)
            (Default|EPlaySE _nearenemy "/Game/Workspace/IoriFUKUNAKA/Sounds/SC_StatusDown.SC_StatusDown" (Transformation|GetActorLocation _nearenemy) "/Game/Workspace/IoriFUKUNAKA/Sounds/SA_PlayerSE.SA_PlayerSE" 1.0)
            (Actor|DestroyActor)))
        (:else)))
    (:else)))