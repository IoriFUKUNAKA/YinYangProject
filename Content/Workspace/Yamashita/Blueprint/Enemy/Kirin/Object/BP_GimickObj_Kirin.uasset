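; Destructible lightning-rod (hiraishin) gimmick object for the Kirin enemy that strikes an area after a delay.
; Timers trigger the thunder effect and enable a per-tick sphere overlap through EnemyRef, then destroy the actor shortly after.
; Each IHitAttack lowers Life and destroys the actor at zero.
; RoS events relay Life and HP updates through MC events to a world widget that faces the player camera.
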(event Custom|E_Attack
  (Variables|Default|SetCollision true)
  ;[1 1 1] デバッグ
  (Variables|Default|SetDebugBool true)
  (Default|RoSSpawnEffect (Variables|Default|GetEnemyRef) "/Game/Workspace/Azuma/Effect/Kirin_gimikku/NS_Kirin_sander.NS_Kirin_sander" (Transformation|GetActorLocation) "1.000000,1.000000,1.000000")
  (Class|BPIEnemy|IPlaySE(Message) (Components|GetOwner) "/Game/Workspace/Yamashita/SoundQue/Enemy/SQ_Hanni_Cue.SQ_Hanni_Cue" (Transformation|GetActorLocation) 0 1.0)
  (Components|DestroyComponent (Variables|Default|GetNiagara)))

(event Custom|E_Destroy
  (Actor|DestroyActor))

(event Custom|Ros_SetLife
  (params (Life :type Integer))
  ;[1 1 1] ライフを設定
  (CallFunction|MCSetLife Life))

(event Custom|MC_SetLife
  (params (Life :type Integer))
  ;[1 1 1] ライフを設定
  (Variables|Default|SetLife Life))

(event Custom|PlaySE_Hiraishin
  (Default|EPlaySE (Variables|Default|GetEnemyRef) "/Game/Assets/Sounds/SE/SE_Skill_roop.SE_Skill_roop" (Transformation|GetActorLocation) 0 0.3))

(event Custom|MC_SetMaxHP
  (Class|BPIEnemy|ISetGimickMaxHP(Message) (Variables|Default|GetUI) (Variables|Default|GetLife)))

(event Custom|RoS_UpdateUI
  (CallFunction|MCUpdateUI))

(event Custom|RoS_SetMaxHP
  (CallFunction|MCSetMaxHP))

(event Custom|MC_UpdateUI
  (Class|BPIEnemy|ISetGimickHP(Message) (Variables|Default|GetUI) (Variables|Default|GetLife)))

(event EventBeginPlay
  (|CallParentFunction)
  (Utilities|Time|SetTimerbyEvent (delegate Custom|E_Attack) (Variables|Default|GetAttackDelay))
  (Utilities|Time|SetTimerbyEvent (delegate Custom|E_Destroy) (+ (Variables|Default|GetAttackDelay) 0.2))
  (CallFunction|PlaySEHiraishin)
  (Utilities|Time|SetTimerbyEvent (delegate Custom|PlaySE_Hiraishin) 3.0 true)
  (bind _aswbp_gimick_hp (Utilities|Casting|CastToWBP_GimickHP (UserInterface|GetUserWidgetObject (Variables|Default|GetWidget))))
  (Variables|Default|SetUI _aswbp_gimick_hp)
  (CallFunction|RoSSetMaxHP))

(event EventTick
  (params (DeltaSeconds :type Float%20%28single-precision%29))
  (bind _returnvalue (Transformation|GetActorLocation))
  (|CallParentFunction DeltaSeconds)
  (CallFunction|RoSUpdateUI)
  (Transformation|SetWorldRotation (Variables|Default|GetWidget) (Math|Rotator|FindLookatRotation (Transformation|GetWorldLocation (Variables|Default|GetWidget)) (Camera|GetCameraLocation (Variables|/Script/Engine.PlayerController|GetPlayerCameraManager (Game|GetPlayerController 0)))) false false)
  (if (Variables|Default|GetCollision)
    (Default|FSphereOverlap (Variables|Default|GetEnemyRef) (Math|Vector|MakeVector (.x _returnvalue) (.y _returnvalue) 7e+01) (Variables|Default|GetAttackRange) false false 5)))

(event EventIHitAttack
  (params (DamageCauser :type Actor%20Object%20Reference) (AttackMagnification :type Float%20%28single-precision%29) (Weight :type Float%20%28single-precision%29))
  (CallFunction|RosSetLife (- (Variables|Default|GetLife) 1))
  (if (== (Variables|Default|GetLife) 0)
    (Actor|DestroyActor)))

(fn ConstructionScript)