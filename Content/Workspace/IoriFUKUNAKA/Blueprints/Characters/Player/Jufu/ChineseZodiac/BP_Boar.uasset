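; BP_Boar is the Boar variant of the player's Chinese zodiac Jufu, which temporarily sets a movable area for its owner.
; On initialize it sets its life span and messages the owner with a movable area of a given radius, centered on the owner's current XY position at zero height.
; On destroy it messages the owner to reset that area, so the effect lasts only as long as this actor lives.
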(fn ConstructionScript
  (|CallParentFunction))

(fn FonInitialize
  (bind _returnvalue (Components|GetOwner))
  (bind _returnvalue_2 (Transformation|GetActorLocation _returnvalue))
  (bind (_x _y) (Math|Vector|BreakVector _returnvalue_2))
  (|CallParentFunction)
  (Actor|SetLifeSpan (Variables|コンフィグ|GetLifeTime))
  (Class|BPIEnemy|ISetMovableArea(Message) _returnvalue (Math|Vector|MakeVector _x _y 0.0) (Variables|Config|GetAreaRadius)))

(fn FonDestroy
  (|CallParentFunction)
  (Class|BPIEnemy|IResetMovableArea(Message) (Components|GetOwner)))