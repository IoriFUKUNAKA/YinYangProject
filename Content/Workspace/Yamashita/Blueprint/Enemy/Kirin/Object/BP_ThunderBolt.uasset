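; Telegraphed thunderbolt strike for the Kirin enemy, shown as a warning decal scaled to the strike radius before it falls.
; Init sets radius and fall timer; Tick fills the decal material, then plays an emissive/alpha timeline shortly before impact.
; The fall event removes the decal, spawns Niagara through server-to-multicast RPCs and asks EnemyRef for a sphere overlap.
; The actor destroys itself when the effect finishes.
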(event Custom|RoS_SpawnThunderBolt
  ;[1 1 1] エフェクト生成
  (CallFunction|MCSpawnThunderBolt))

(event Custom|MC_SpawnThunderBolt
  ;[1 1 1] エフェクト生成
  (bind _returnvalue (Niagara|SpawnSystematLocation "/Game/Workspace/Azuma/Effect/Kirin_gimikku/NS_Kirin_sander.NS_Kirin_sander" (Transformation|GetActorLocation)))
  (EventDispatchers|BindEventtoOnSystemFinished _returnvalue (delegate Custom|E_OnEffectEnd)))

(event Custom|E_FallThunder
  (Components|DestroyComponent (Variables|Default|GetDecal))
  (CallFunction|RoSSpawnThunderBolt)
  (bind _enemyref (Variables|Default|GetEnemyRef)
    (:then
      (Default|FSphereOverlap _enemyref (Transformation|GetActorLocation) (Variables|Default|GetRadiusOfThunderBolt) false false 5))
    (:else)))

(event Custom|E_OnEffectEnd
  (params (PSystem :type Niagara%20Component%20Object%20Reference))
  ;[1 1 1] エフェクト生成
  (Actor|DestroyActor))

(event Custom|E_UpdateTimer
  (bind _output_get (Variables|Default|Settimer (Math|Float|Min(Float) (+ (Variables|Default|Gettimer) (Utilities|Time|GetWorldDeltaSeconds)) (- (Variables|Default|GetTimeForFall) 0.8))))
  (Rendering|Material|SetScalarParameterValue (Variables|Default|GetM_DecalMat) "Rate" (/ _output_get (- (Variables|Default|GetTimeForFall) 0.8)) :!class /Script/Engine.MaterialInstanceDynamic)
  (if (>= (/ _output_get (- (Variables|Default|GetTimeForFall) 0.8)) 1.0)
    (Utilities|IsValid (Variables|Default|GetDecal)
      (:Is%20Valid
        (Utilities|FlowControl|DoOnce false
          (:Completed
            (bind (_direction _pow _alpha) (Timeline|Emissive Play)
              (:Update
                (Rendering|Material|SetScalarParameterValue (Variables|Default|GetM_DecalMat) "EmissivePow" _pow :!class /Script/Engine.MaterialInstanceDynamic)
                (Rendering|Material|SetScalarParameterValue (Variables|Default|GetM_DecalMat) "alpha" _alpha :!class /Script/Engine.MaterialInstanceDynamic))
              (:Finished
                (Rendering|SetVisibility (Variables|Default|GetDecal) false false)))))))))

(event Custom|E_SetInit
  (params (TimeForFall :type Float%20%28single-precision%29) (RadiusOfThunderBolt :type Float%20%28single-precision%29))
  (bind _returnvalue (* RadiusOfThunderBolt 0.01))
  ;[1 1 1] 初期化
  (Variables|Default|SetTimeForFall TimeForFall)
  (Variables|Default|SetRadiusOfThunderBolt RadiusOfThunderBolt)
  (CallFunction|MCSetDecalScale (Math|Vector|MakeVector _returnvalue _returnvalue _returnvalue))
  (Utilities|Time|SetTimerbyEvent (EventDispatchers|CreateEvent :!event Custom|E_FallThunder) (Variables|Default|GetTimeForFall)))

(event Custom|MC_SetDecalScale
  (params (NewScale3D :type Vector))
  ;[1 1 1] 初期化
  (Transformation|SetRelativeScale3D (Variables|Default|GetDecal) NewScale3D))

(event EventBeginPlay
  (|CallParentFunction)
  (bind _returnvalue (Rendering|Material|CreateDynamicMaterialInstance (Variables|Default|GetDecal) :!class /Script/Engine.DecalComponent))
  (Variables|Default|SetM_DecalMat _returnvalue))

(event EventTick
  (params (DeltaSeconds :type Float%20%28single-precision%29))
  (|CallParentFunction DeltaSeconds)
  (CallFunction|EUpdateTimer))

(fn ConstructionScript
  (|CallParentFunction))