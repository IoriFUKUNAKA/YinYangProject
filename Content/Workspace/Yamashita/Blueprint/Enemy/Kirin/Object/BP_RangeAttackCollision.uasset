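; Telegraphed thunderbolt area attack for the Kirin enemy, marking a circle on the ground with a decal before it strikes.
; Init scales the decal to the radius and starts a timer; the attack runs the owning enemy's sphere overlap.
; Tick fills the decal material, then a timeline drives emissive and alpha before hiding it.
; A multicast spawns the Niagara strike, and the actor destroys itself when that finishes.
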(event Custom|MC_SpawnEffect
  ;[1 1 1] エフェクト生成
  (bind _returnvalue (Niagara|SpawnSystematLocation "/Game/Workspace/Azuma/Effect/Kirin_hani_attack/NS_kirin_hani_attack.NS_kirin_hani_attack" (Transformation|GetActorLocation)))
  (Rendering|SetReceivesDecals _returnvalue false)
  (EventDispatchers|BindEventtoOnSystemFinished _returnvalue (delegate Custom|E_OnEffectEnd)))

(event Custom|E_OnEffectEnd
  (params (PSystem :type Niagara%20Component%20Object%20Reference))
  ;[1 1 1] エフェクト生成
  (Actor|DestroyActor))

(event Custom|E_Attack
  ;[1 1 1] 攻撃
  (Default|FSphereOverlap (Variables|Default|GetEnemyRef) (Transformation|GetActorLocation) (Variables|Default|GetRadiusOfThunderBolt) false false 5)
  (CallFunction|RoSSpawnEffect))

(event Custom|E_SetInit
  (params (TimeForFall :type Float%20%28single-precision%29) (RadiusOfThunderBolt :type Float%20%28single-precision%29))
  ;[1 1 1] 初期化
  (Variables|Default|SetRadiusOfThunderBolt RadiusOfThunderBolt)
  (CallFunction|MCSetDecalScale (Math|Conversions|ToVector(Float) (* RadiusOfThunderBolt 0.01)))
  (Utilities|Time|SetTimerbyEvent (EventDispatchers|CreateEvent :!event Custom|E_Attack) (Variables|Default|GetTimeForFall)))

(event Custom|MC_SetDecalScale
  (params (NewScale3D :type Vector))
  ;[1 1 1] 初期化
  (Transformation|SetRelativeScale3D (Variables|Default|GetDecal) NewScale3D))

(event Custom|E_UpdateDecal
  ;[1 1 1] デカール　マテリアルパラメータ更新
  (bind _output_get (Variables|Default|Settimer (Math|Float|Min(Float) (+ (Variables|Default|Gettimer) (Utilities|Time|GetWorldDeltaSeconds)) (- (Variables|Default|GetTimeForFall) 0.8))))
  (Rendering|Material|SetScalarParameterValue (Variables|Default|GetM_Decal) "Rate" (/ _output_get (- (Variables|Default|GetTimeForFall) 0.8)) :!class /Script/Engine.MaterialInstanceDynamic)
  (if (>= (/ _output_get (- (Variables|Default|GetTimeForFall) 0.8)) 1.0)
    (Utilities|IsValid (Variables|Default|GetDecal)
      (:Is%20Valid
        (Utilities|FlowControl|DoOnce false
          (:Completed
            (bind (_direction _pow _alpha) (Timeline|Emmisive Play)
              (:Update
                (Rendering|Material|SetScalarParameterValue (Variables|Default|GetM_Decal) "EmissivePow" _pow :!class /Script/Engine.MaterialInstanceDynamic)
                (Rendering|Material|SetScalarParameterValue (Variables|Default|GetM_Decal) "alpha" _alpha :!class /Script/Engine.MaterialInstanceDynamic))
              (:Finished
                (Rendering|SetVisibility (Variables|Default|GetDecal) false false)))))))))

(event Custom|RoS_SpawnEffect
  ;[1 1 1] エフェクト生成
  (CallFunction|MCSpawnEffect))

(event EventBeginPlay
  (|CallParentFunction)
  (bind _returnvalue (Rendering|Material|CreateDynamicMaterialInstance (Variables|Default|GetDecal) :!class /Script/Engine.DecalComponent))
  (Variables|Default|SetM_Decal _returnvalue))

(event EventTick
  (params (DeltaSeconds :type Float%20%28single-precision%29))
  (|CallParentFunction DeltaSeconds)
  (CallFunction|EUpdateDecal))

(fn ConstructionScript)