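; BP_LoginPlayer drives the login screen UI, switching between the login menu and the server list, and opens the menu with the mouse cursor shown on BeginPlay.
; Show events call a transition macro that removes the current screen, updates the state enum, and rejects repeated or invalid states with a printed error.
; Each widget is created lazily, cached for reuse, then added to the viewport with UI-only input.
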(event EventBeginPlay
  (CallFunction|IShowLoginMenu)
  (Variables|/Script/Engine.PlayerController|SetbShowMouseCursor (Game|GetPlayerController 0) true))

(event EventIShowLoginMenu
  (bind _returnvalue (Game|GetPlayerController 0))
  (Utilities|MTransitionState "NewEnumerator0"
    (:NewState
      (Utilities|IsValid (Variables|Default|GetLoginMenu)
        (:Is%20Valid
          _)
        (:Is%20Not%20Valid
          (bind _returnvalue_2 (UserInterface|CreateWidget "/Game/Workspace/IoriFUKUNAKA/Blueprints/HeadUpDisplays/LoginHUD/WBP_LoginMenu.WBP_LoginMenu_C" _returnvalue))
          (Variables|Default|SetLoginMenu _returnvalue_2)))
      (Input|SetInputModeUIOnly _returnvalue (Variables|Default|GetLoginMenu) "DoNotLock")
      (UserInterface|Viewport|AddtoViewport (Variables|Default|GetLoginMenu) 0))))

(event EventIShowServerList
  (bind _returnvalue (Game|GetPlayerController 0))
  (Utilities|MTransitionState "NewEnumerator1"
    (:NewState
      (Utilities|IsValid (Variables|Default|GetServerList)
        (:Is%20Valid
          _)
        (:Is%20Not%20Valid
          (bind _returnvalue_2 (UserInterface|CreateWidget "/Game/Workspace/IoriFUKUNAKA/Blueprints/HeadUpDisplays/LoginHUD/WBP_ServerList.WBP_ServerList_C" _returnvalue))
          (Variables|Default|SetServerList _returnvalue_2)))
      (Input|SetInputModeUIOnly _returnvalue (Variables|Default|GetServerList) "DoNotLock")
      (UserInterface|Viewport|AddtoViewport (Variables|Default|GetServerList) 0))))

(fn ConstructionScript)