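; BP_YinYangPlayer_Girl is the girl variant of the Yin Yang player character, extending a parent player Blueprint.
; On per-player initialization, it runs the parent logic, then applies a dynamic instance of the girl's emissive material to mesh slot 1, colored by the player's element.
; It also plays the girl-specific footstep sound at its location when the footstep interface event fires.
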(event EventIPlayFootStepSE
  (CallFunction|ROSSpawnSoundatLocation "/Game/Workspace/Katsuhara/SoundCue/SC_FootStep_Girl.SC_FootStep_Girl" (Transformation|GetActorLocation) "0, 0, 0" 1.0 1.0 0.0))

(fn ConstructionScript
  (|CallParentFunction))

(fn FInitilizeEachPlayer
  (params (MyElement :type En_Elements%20Enum :default "NewEnumerator6"))
  (|CallParentFunction MyElement)
  (bind _returnvalue (Rendering|Material|CreateDynamicMaterialInstance (Variables|Character|GetMesh) 1 "/Game/Workspace/IoriFUKUNAKA/Materials/Lighting/YinYangCharacters/MI_Girl_Emissive.MI_Girl_Emissive" "None" :!class /Script/Engine.PrimitiveComponent))
  (bind _output_get (LocalVariables|SetEmissiveMI _returnvalue))
  (Rendering|Material|SetVectorParameterValue _output_get "EmissiveColor" (Utilities|Array|Get(acopy) (LocalVariables|GetElementEmissiveColor) (Math|Conversions|ToInteger(Byte) MyElement)) :!class /Script/Engine.MaterialInstanceDynamic)
  (Rendering|Material|SetMaterial (Variables|Character|GetMesh) 1 (LocalVariables|GetEmissiveMI)))