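; Base class for networked enemies, handling stats, health stages, attacks and a per-player hate table.
; Player skill use within notice range and incoming hits add hate, prompting the GameManager to re-evaluate targets.
; Overridable collision checks, enabled by animation, feed overlap helpers that apply server-side damage and build Juryoku (curse energy), which special attacks spend.
; Interface functions connect behavior tree tasks and the AnimBP, with multicasts syncing state, montages and effects.
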(event Custom|MC_PlayMontage
  (params (MontageToPlay :type Anim%20Montage%20Object%20Reference) (InPlayRate :type Float%20%28single-precision%29))
  (bind _mesh (Variables|Character|GetMesh))
  (bind _returnvalue (Components|SkeletalMesh|GetAnimInstance _mesh))
  ;[1 1 1] モンタージュ再生
  (Class|BPIEnemy|IMontageStart(Message) _returnvalue)
  (Animation|Montage|MontagePlay _returnvalue MontageToPlay InPlayRate "MontageLength" 0.0 true))

(event Custom|RoS_SetAlreadyJuryokuUp
  (params (AlreadyJuryokuUp :type Boolean))
  ;[1 1 1] 被ダメ・攻撃による呪力アップフラグを設定
  (CallFunction|MCSetAlreadyJuryokuUP AlreadyJuryokuUp))

(event Custom|MC_SetHealthState
  (params (HealthState :type En_EnemyStageState%20Enum :default "NewEnumerator0"))
  ;[1 1 1] 体力の段階を設定
  (Variables|ステート|SetHealthState HealthState))

(event Custom|RoS_SpawnEffect
  (params (SystemTemplate :type Niagara%20System%20Object%20Reference) (Location :type Vector) (Scale :type Vector))
  ;[1 1 1] エフェクト生成
  (CallFunction|MCSpawnEffect SystemTemplate Location Scale))

(event Custom|MC_SpawnEffect
  (params (SystemTemplate :type Niagara%20System%20Object%20Reference) (Location :type Vector) (Scale :type Vector))
  ;[1 1 1] エフェクト生成
  (Niagara|SpawnSystematLocation SystemTemplate Location "0, 0, 0" Scale))

(event Custom|MC_SetAlreadyJuryokuUP
  (params (AlreadyJuryokuUp :type Boolean))
  ;[1 1 1] 被ダメ・攻撃による呪力アップフラグを設定
  (Variables|呪力|SetAlreadyJuryokuUp AlreadyJuryokuUp))

(event Custom|E_AddHate
  (params (hate :type Float%20%28single-precision%29) (isUseSkill? :type Boolean))
  ;[1 1 1] プレイヤーとの距離によって呪符スキル使用時イベントをバインド
  (CallFunction|FAddHate hate isUseSkill? (.Player (Utilities|Struct|BreakST_PlayerHate (stale EventTick _array_element)))))

(event Custom|RoS_SetInSightCharacter
  (params (InSightCharacter :type Array%20of%20Actor%20Object%20References))
  ;[1 1 1] 視野内のプレイヤー設定
  (CallFunction|MCSetinSightCharacter InSightCharacter))

(event Custom|MC_SetInSightCharacter
  (params (InSightCharacter :type Array%20of%20Actor%20Object%20References))
  ;[1 1 1] 視野内のプレイヤー設定
  (Utilities|Array|Clear (Variables|Default|GetInSightCharacter))
  (Variables|Default|SetInSightCharacter InSightCharacter))

(event Custom|E_Init
  (params (GameManager :type BP%20Game%20Manager%20Object%20Reference))
  ;[1 1 1] 初期化処理
  (Variables|Default|Setm_GameManager GameManager))

(event Custom|RoS_SetAttackHit?
  (params (AttackHit? :type Boolean))
  ;[1 1 1] 攻撃がプレイヤーに当たったかフラグを設定
  (CallFunction|MCSetAttackHit? AttackHit?))

(event Custom|MC_SetAttackHit?
  (params (AttackHit? :type Boolean))
  ;[1 1 1] 攻撃がプレイヤーに当たったかフラグを設定
  (Variables|Collision|SetAttackHit? AttackHit?))

(event Custom|RoS_SetHealthState
  (params (HealthState :type En_EnemyStageState%20Enum :default "NewEnumerator0"))
  ;[1 1 1] 体力の段階を設定
  (CallFunction|MCSetHealthState HealthState))

(event EventBeginPlay
  (Variables|/Game/Workspace/IoriFUKUNAKA/Blueprints/Characters/BPC_StatusManager.BPC_StatusManager_C|SetAttack (Variables|Default|GetBPC_StatusManager) 1e+02)
  (Variables|/Game/Workspace/IoriFUKUNAKA/Blueprints/Characters/BPC_StatusManager.BPC_StatusManager_C|SetDefence (Variables|Default|GetBPC_StatusManager) 5e+01)
  (bind _output_get (Variables|/Game/Workspace/IoriFUKUNAKA/Blueprints/Characters/BPC_StatusManager.BPC_StatusManager_C|SetSpeed (Variables|Default|GetBPC_StatusManager) 5e+02))
  (Variables|/Script/Engine.CharacterMovementComponent|SetMaxWalkSpeed (Variables|Character|GetCharacterMovement) _output_get)
  (Variables|呪力|SetCurrentJuryoku (Variables|呪力|GetMaxJuryoku%20))
  (bind _output_get_2 (Variables|パラメータ|SetCurrentHealth (Variables|パラメータ|GetMaxHealth)))
  (CallFunction|FSetHealthState _output_get_2))

(event EventTick
  (params (DeltaSeconds :type Float%20%28single-precision%29))
  (Utilities|FlowControl|Sequence
    (:then_0
      ;[1 1 1] 当たり判定
      (if (Variables|コリジョン|GetCollisionEnable)
        (CallFunction|FOverrideCollision)
        (else
          (CallFunction|RoSSetAlreadyJuryokuUp false))))
    (:then_1
      ;[1 1 1] プレイヤーとの距離によって呪符スキル使用時イベントをバインド
      (for _array_element (Variables|Default|GetPlayersHate)
        (Utilities|IsValid (.Player (Utilities|Struct|BreakST_PlayerHate _array_element))
          (:Is%20Valid
            (Development|PrintString (Utilities|String|ToString(Text) (Utilities|Text|FormatText "{playername} : {hate}" (Utilities|GetObjectName (.Player (Utilities|Struct|BreakST_PlayerHate _array_element))) (.Hate (Utilities|Struct|BreakST_PlayerHate _array_element)))) true true "(R=0.000000,G=0.660000,B=1.000000,A=1.000000)" 0.0)
            (if (< (Class|KismetMathLibrary|VectorDistanceSquared (Transformation|GetActorLocation (.Player (Utilities|Struct|BreakST_PlayerHate _array_element))) (Transformation|GetActorLocation)) (* (Variables|プランナー編集可|GetNoticeRange) (Variables|プランナー編集可|GetNoticeRange)))
              (EventDispatchers|BindEventtoOnUseSkill (.Player (Utilities|Struct|BreakST_PlayerHate _array_element)) (delegate Custom|E_AddHate))
              (else
                (EventDispatchers|UnbindEventfromOnUseSkill (.Player (Utilities|Struct|BreakST_PlayerHate _array_element)) (delegate Custom|E_AddHate))))))))
    (:then_2
      ;[1 1 1] ヘイトが一番高いプレイヤーの位置を取得
      (Networking|SwitchHasAuthority
        (:Authority
          (bind _m_gamemanager (Variables|Default|Getm_GameManager)
            (:then
              (bind _loc (Default|FGetEnemyTargetLoc _m_gamemanager (Variables|ステート|GetMyFightingStage)))
              (Variables|Default|SetHighestHateCharacterLoc _loc))
            (:else)))))
    (:then_3
      ;[1 1 1] ステータスを更新
      (Default|EStatusManagerUpdate (Variables|Default|GetBPC_StatusManager))
      (bind _status (Default|FGetStatus (Variables|Default|GetBPC_StatusManager) "NewEnumerator2"))
      (Variables|/Script/Engine.CharacterMovementComponent|SetMaxWalkSpeed (Variables|Character|GetCharacterMovement) _status))))

(event Custom|MC_SetLookAtAlpha_ToABP
  (params (alpha :type Float%20%28single-precision%29))
  ;[1 0.03215 0.935] ビヘイビアツリーから
  ;;[1 1 1] 注視点のAlphaを設定
  (Class|BPIEnemy|ISetLookatAlpha(Message) (Components|SkeletalMesh|GetAnimInstance (Variables|Character|GetMesh)) alpha))

(event Custom|MC_SetTag
  (params (state :type Gameplay%20Tag%20Structure))
  ;[1 0.03215 0.935] ビヘイビアツリーから
  ;;[1 1 1] ステート変更
  (bind _output_get (Variables|ステート|Setstate state))
  (Class|BPIEnemy|ISetTag(Message) (Components|SkeletalMesh|GetAnimInstance (Variables|Character|GetMesh)) _output_get))

(event Custom|MC_SetAttackTag
  (params (AttackState :type Gameplay%20Tag%20Structure))
  ;[1 0.03215 0.935] ビヘイビアツリーから
  ;;[1 1 1] アタック用のタグを設定
  (Variables|ステート|SetAttackState AttackState))

(event EventISetTag
  (params (state :type Gameplay%20Tag%20Structure))
  ;[1 0.03215 0.935] ビヘイビアツリーから
  ;;[1 1 1] ステート変更
  (CallFunction|MCSetTag state))

(event EventISetTask
  (params (task :type Object%20Object%20Reference))
  ;[1 0.03215 0.935] ビヘイビアツリーから
  ;;[1 1 1] 実行中のＴａｓｋを設定
  (Variables|Default|SetTask task))

(event EventISetAttackTag
  (params (attackTag :type Gameplay%20Tag%20Structure))
  ;[1 0.03215 0.935] ビヘイビアツリーから
  ;;[1 1 1] アタック用のタグを設定
  (CallFunction|MCSetAttackTag attackTag))

(event EventISetSightCharacters
  (params (characters :type Array%20of%20Actor%20Object%20References))
  ;[0.03432 0.1103 1] From BPI
  ;;[1 1 1] 視野内のキャラクター配列
  (CallFunction|RoSSetinSightCharacter characters))

(event EventIMoveStart
  ;[1 0.477 0] アニメーションBPから
  ;;[1 1 1] 移動通知
  (Class|BPIEnemy|IMoveStart(Message) (Variables|Default|GetTask)))

(event EventIFirstAttack
  (params (Target :type Actor%20Object%20Reference))
  ;[1 0.03215 0.935] ビヘイビアツリーから
  ;;[1 1 1] 最初のプレイヤーにヘイトを加算
  (bind _asbp_player (Utilities|Casting|CastToBP_Player Target))
  (CallFunction|FAddHate 1.0 true _asbp_player))

(event EventIAttackStart
  (params (isNormalAttack? :type Boolean))
  ;[1 0.03215 0.935] ビヘイビアツリーから
  ;;[1 1 1] 攻撃開始
  (Utilities|Array|Clear (Variables|Default|GetDamagedActors))
  (CallFunction|RoSSetAttackHit? false)
  (if (not isNormalAttack?)
    (Variables|呪力|SetCurrentJuryoku (Math|Float|Clamp(Float) (- (Variables|呪力|GetCurrentJuryoku) 3e+01) 0.0 (Variables|呪力|GetMaxJuryoku%20)))))

(event EventICollisionEnable
  (params (CollisionEnable :type Boolean))
  ;[1 0.477 0] アニメーションBPから
  ;;[1 1 1] 攻撃用当たり判定フラグ　オン・オフ
  (Variables|コリジョン|SetCollisionEnable CollisionEnable))

(event EventIAnimationEnd
  ;[1 0.477 0] アニメーションBPから
  ;;[1 1 1] アニメーション開始・終了
  (Class|BPIEnemy|IAnimationEnd(Message) (Variables|Default|GetTask)))

(event EventIAnimationStart
  ;[1 0.477 0] アニメーションBPから
  ;;[1 1 1] アニメーション開始・終了
  (Class|BPIEnemy|IAnimationStart(Message) (Variables|Default|GetTask)))

(event EventISetMoveSpeed
  (params (MoveSpeed :type Float%20%28single-precision%29))
  ;[1 0.03215 0.935] ビヘイビアツリーから
  ;;[1 1 1] 歩行スピードを設定
  (Variables|/Script/Engine.CharacterMovementComponent|SetMaxWalkSpeed (Variables|Character|GetCharacterMovement) MoveSpeed))

(event EventISetLookatAlpha
  (params (alpha :type Float%20%28single-precision%29))
  ;[1 0.03215 0.935] ビヘイビアツリーから
  ;;[1 1 1] 注視点のAlphaを設定
  (CallFunction|MCSetLookatAlphatoABP alpha))

(event EventIHitAttack
  (params (DamageCauser :type Actor%20Object%20Reference) (Attack :type Float%20%28single-precision%29) (Weight :type Float%20%28single-precision%29))
  ;[1 1 1] ダメージ受フラグ
  (Networking|SwitchHasAuthority
    (:Authority
      (bind _damage (CallFunction|FCulcDamage Attack (Variables|/Game/Workspace/IoriFUKUNAKA/Blueprints/Characters/BPC_StatusManager.BPC_StatusManager_C|GetDefence (Variables|Default|GetBPC_StatusManager))))
      (bind _asbp_player (Utilities|Casting|CastToBP_Player DamageCauser))
      (CallFunction|FAddHate Weight false _asbp_player)
      (bind _output_get (Variables|パラメータ|SetCurrentHealth (- (Variables|パラメータ|GetCurrentHealth) _damage)))
      (CallFunction|FSetHealthState _output_get)
      ;[1 1 1] 呪力量加算
      (Variables|呪力|SetCurrentJuryoku (Math|Float|Clamp(Float) (+ (Variables|呪力|GetCurrentJuryoku) 1.0) 0.0 (Variables|呪力|GetMaxJuryoku%20))))))

(event EventISetRotationRate
  (params (rate :type Rotator :default "0, 0, 0"))
  ;[1 0.03215 0.935] ビヘイビアツリーから
  ;;[1 1 1] RotationRateを設定
  (Variables|/Script/Engine.CharacterMovementComponent|SetRotationRate (Variables|Character|GetCharacterMovement) rate))

(fn ConstructionScript)

(fn FOverrideCollision)

(fn FSphereOverlap
  (params (SpherePos :type Vector) (SphereRadius :type Float%20%28single-precision%29) (isNormalAttack :type Boolean) (Physical%20attack? :type Boolean) (MaxPlayer :type Integer))
  (LocalVariables|SetnormalAttack? isNormalAttack)
  (LocalVariables|SetPhysicalAttack? Physical%20attack?)
  (bind (_outactors _returnvalue) (Collision|SphereOverlapActors SpherePos SphereRadius (Utilities|Array|MakeArray "ObjectTypeQuery3") 0))
  (if _returnvalue
    (for _array_element _outactors
      (if (Actor|ActorHasTag _array_element "Player")
        (CallFunction|FonHitAction _array_element (LocalVariables|GetnormalAttack?) (LocalVariables|GetPhysicalAttack?) MaxPlayer)))))

(fn FBoxOverlap
  (params (BoxPos :type Vector) (BoxExtent :type Vector) (NormalAttack? :type Boolean) (PhysicsAttack? :type Boolean) (MaxPlayer :type Integer))
  (LocalVariables|SetNormalAtack? NormalAttack?)
  (LocalVariables|SetphysicsAttack PhysicsAttack?)
  (bind (_outactors _returnvalue) (Collision|BoxOverlapActors BoxPos BoxExtent (Utilities|Array|MakeArray "ObjectTypeQuery3") 0 :!class /Script/Engine.KismetSystemLibrary))
  (if _returnvalue
    (for _array_element _outactors
      (if (Actor|ActorHasTag _array_element "Player")
        (CallFunction|FonHitAction _array_element (LocalVariables|GetNormalAtack?) (LocalVariables|GetphysicsAttack) MaxPlayer)))))

(fn FSetHealthState
  (params (NewHealth :type Float%20%28single-precision%29))
  (if (> NewHealth 0.0)
    (for _array_element (Variables|プランナー編集可|GetHealthStateList)
      (if (and (< NewHealth (.LessThan (Utilities|Struct|BreakST_EnemyHealthState _array_element))) (>= NewHealth (.GreaterThanorEqualto (Utilities|Struct|BreakST_EnemyHealthState _array_element))))
        (CallFunction|RoSSetHealthState (.HealthState (Utilities|Struct|BreakST_EnemyHealthState _array_element)))
        (return)))
    (else
      ;[1 1 1] 死んだ
      (CallFunction|RoSSetHealthState "NewEnumerator7"))))

(fn FAddHate
  (params (Hate :type Float%20%28single-precision%29) (isJUHUSkill? :type Boolean) (Player :type BP%20Player%20Object%20Reference))
  (LocalVariables|SetBaseHatef Hate)
  (LocalVariables|SetJUHUSkill? isJUHUSkill?)
  (for (_array_element _array_index) (Variables|Default|GetPlayersHate)
    (if (== (.Player (Utilities|Struct|BreakST_PlayerHate _array_element)) Player)
      (if (LocalVariables|GetJUHUSkill?)
        (Utilities|Array|SetArrayElem (Variables|Default|GetPlayersHate) _array_index (Utilities|Struct|MakeST_PlayerHate Player (+ (.Hate (Utilities|Struct|BreakST_PlayerHate _array_element)) (LocalVariables|GetBaseHatef))))
        (bind _m_gamemanager (Variables|Default|Getm_GameManager)
          (:then
            (Default|EChangeTarget _m_gamemanager (Variables|ステート|GetMyFightingStage)))
          (:else))
        (else
          (bind _hate (CallFunction|FCalcHatefromDot (Transformation|GetActorLocation Player) 0.0)) ; 今は1を返す
          (Utilities|Array|SetArrayElem (Variables|Default|GetPlayersHate) _array_index (Utilities|Struct|MakeST_PlayerHate Player (+ (* _hate (LocalVariables|GetBaseHatef)) (.Hate (Utilities|Struct|BreakST_PlayerHate _array_element)))))
          (bind _m_gamemanager_2 (Variables|Default|Getm_GameManager)
            (:then
              (Default|EChangeTarget _m_gamemanager_2 (Variables|ステート|GetMyFightingStage)))
            (:else)))))))

(fn FCalcHatefromDot
  (params (PlayerLocation :type Vector) (SightAngeHalf :type Float%20%28single-precision%29))
  (LocalVariables|SetPlayerLoc PlayerLocation)
  (LocalVariables|SetHalfAngle SightAngeHalf)
  (if (> (Math|Vector2D|DotProduct(2D) (Math|Conversions|ToVector2D(Vector) (Transformation|GetActorForwardVector)) (Math|Conversions|ToVector2D(Vector) (Math|Vector|Normalize (- (LocalVariables|GetPlayerLoc) (Transformation|GetActorLocation))))) 0.0)
    (return 1.0) ; 通常
    (elif (> (* (Math|Float|Absolute(Float) (Math|Vector2D|DotProduct(2D) (Math|Conversions|ToVector2D(Vector) (Transformation|GetActorForwardVector)) (Math|Conversions|ToVector2D(Vector) (Math|Vector|Normalize (- (LocalVariables|GetPlayerLoc) (Transformation|GetActorLocation)))))) 9e+01) (- (LocalVariables|GetHalfAngle) 9e+01))
      (return 3.0) ; 乗算
      (else
        (return 1.0) ; 通常
      ))))

(fn FCheckJuryokuUp
  (params (gamePlayTag :type Array%20of%20Gameplay%20Tag%20Structures))
  (for _array_element gamePlayTag
    (if (GameplayTags|MatchesTag (Variables|ステート|GetAttackState) _array_element true)
      ;[1 1 1] 呪力量加算
      (Variables|呪力|SetCurrentJuryoku (Math|Float|Clamp(Float) (+ (Variables|呪力|GetCurrentJuryoku) 5.0) 0.0 (Variables|呪力|GetMaxJuryoku%20)))
      (CallFunction|RoSSetAlreadyJuryokuUp true))))

(fn FGetHightestHatePlayer
  (for _array_element (Variables|Default|GetPlayersHate)
    (if (and (>= (.Hate (Utilities|Struct|BreakST_PlayerHate _array_element)) (LocalVariables|GetHighestHateValue)) (Utilities|Enum|NotEqual(Enum) (Default|FGetCurrentPlayerState (.Player (Utilities|Struct|BreakST_PlayerHate _array_element))) "NewEnumerator6"))
      (LocalVariables|SetHighestHateValue (.Hate (Utilities|Struct|BreakST_PlayerHate _array_element)))
      (LocalVariables|SetHighestHatePlayer (.Player (Utilities|Struct|BreakST_PlayerHate _array_element)))))
  (return (LocalVariables|GetHighestHatePlayer)))

(fn FonHitAction
  (params (InputPin :type Actor%20Object%20Reference) (NormalAttack? :type Boolean) (PhysicsAttack? :type Boolean) (MaxPlayer :type Integer))
  (bind _asbp_player (Utilities|Casting|CastToBP_Player InputPin))
  (if (Math|Boolean|ANDBoolean (== (Utilities|Array|FindItem (Variables|Default|GetDamagedActors) InputPin) -1) (< (Utilities|Array|Length (Variables|Default|GetDamagedActors)) MaxPlayer) (> (Variables|/Game/Workspace/IoriFUKUNAKA/Blueprints/Characters/Player/BP_Player.BP_Player_C|GetCurrentHP _asbp_player) 0.0) (Utilities|Enum|NotEqual(Enum) (Default|FGetCurrentPlayerState _asbp_player) "NewEnumerator4"))
    (Networking|SwitchHasAuthority
      (:Authority
        (Class|BPIHitBoxtoCharacter|IHitAttack(Message) InputPin self (Variables|/Game/Workspace/IoriFUKUNAKA/Blueprints/Characters/BPC_StatusManager.BPC_StatusManager_C|GetAttack (Variables|Default|GetBPC_StatusManager)) 0.0)
        (CallFunction|RoSSpawnEffect "/Game/Workspace/Azuma/Effect/Kirin_hit/NS_kirin_hit.NS_kirin_hit" (CallFunction|FGetHitEffectSpawnPos (Transformation|GetActorLocation InputPin)) "2.000000,2.000000,2.000000")
        (Utilities|Array|Add (Variables|Default|GetDamagedActors) InputPin)
        (Utilities|FlowControl|Sequence
          (:then_0
            ;[1 1 1] 呪力加算
            (if (not (and (Variables|呪力|GetAlreadyJuryokuUp) NormalAttack?))
              (CallFunction|FCheckJuryokuUp (Variables|Default|GetNormalAttackList)) ; 呪力を加算
            ))
          (:then_1
            ;[1 1 1] ヒットしたか
            (if PhysicsAttack?
              (CallFunction|RoSSetAttackHit? true))))))))

(fn FGetHitEffectSpawnPos
  (params (playerLoc :type Vector))
  (bind _returnvalue (Transformation|GetActorLocation))
  (bind _returnvalue_2 (- _returnvalue playerLoc))
  (bind _returnvalue_3 (Math|Vector|Normalize _returnvalue_2))
  (bind _returnvalue_4 (* _returnvalue_3 1e+02))
  (bind _returnvalue_5 (+ playerLoc _returnvalue_4))
  (return (Math|Vector|MakeVector (.x _returnvalue_5) (.y _returnvalue_5) 4e+01)))

(fn IGetAttackHit?
  (return (Variables|Collision|GetAttackHit?)))

(fn IGetAttackRange
  (return (Variables|プランナー編集可|GetAttackRange)))

(fn IGetAttackStatus
  (params (tag :type Gameplay%20Tag%20Structure))
  (for _array_element (Variables|プランナー編集可|GetAttackStatusList)
    (if (GameplayTags|MatchesTag (.Tag (Utilities|Struct|BreakST_EnemyAttack _array_element)) tag true)
      (return _array_element true)))
  (return "" false))

(fn IGetAttackTag
  (return (Variables|ステート|GetAttackState)))

(fn IGetCurrentGameState
  (return (Variables|ステート|GetCurrentGameState)))

(fn IGetCurrentJuryoku
  (return (Variables|呪力|GetCurrentJuryoku)))

(fn IGetDefaultMoveSpeed
  (bind _status (Default|FGetStatus (Variables|Default|GetBPC_StatusManager) "NewEnumerator2"))
  (return _status))

(fn IGetEnemyHealthState
  (return (Variables|ステート|GetHealthState)))

(fn IGetEnemyLarge
  (return (Variables|パラメータ|GetEnemyLarge)))

(fn IGetGimickAppearNumKirin
  (return 0))

(fn IGetGimickRangeKirin
  (return 0.0))

(fn IGetHateStageBorder
  (params (Stage :type En_EnemyStageState%20Enum :default "NewEnumerator7"))
  (return 0.0 false))

(fn IGetHighestHateCharacterLoc
  (return (Variables|Default|GetHighestHateCharacterLoc)))

(fn IGetHP
  (return (Variables|パラメータ|GetCurrentHealth)))

(fn IGetLookatAlpha
  (bind _alpha (Class|BPIEnemy|IGetLookatAlpha(Message) (Components|SkeletalMesh|GetAnimInstance (Variables|Character|GetMesh))))
  (return _alpha))

(fn IGetNorticeRange
  (return (Variables|プランナー編集可|GetNoticeRange)))

(fn IGetPlayersHate
  (return (Variables|Default|GetPlayersHate)))

(fn IGetSightCharacters
  (return (Variables|Default|GetInSightCharacter)))

(fn IGetTag
  (return (Variables|ステート|Getstate)))

(fn IGetTimeforGimickActivateKirin
  (return 0.0))