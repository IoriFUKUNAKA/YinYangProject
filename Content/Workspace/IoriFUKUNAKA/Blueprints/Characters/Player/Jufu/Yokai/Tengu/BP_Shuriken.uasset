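; BP_Shuriken is the Tengu shuriken from the player's Jufu Yokai set, damaging the enemy it overlaps.
; On the server only, its Sphere overlap applies D_Tengu damage to Enemy-tagged actors, scaling the instigator's PlayerState Attack by AttackMag.
; It then has the instigator spawn a wind explosion Niagara effect at its transform through an interface message and destroys itself.
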(event OnComponentBeginOverlap(Sphere)
  (params (OverlappedComponent :type Primitive%20Component%20Object%20Reference) (OtherActor :type Actor%20Object%20Reference) (OtherComp :type Primitive%20Component%20Object%20Reference) (OtherBodyIndex :type Integer) (bFromSweep :type Boolean) (SweepResult :type Hit%20Result%20Structure%20%28by%20ref%29))
  (bind _returnvalue (Transformation|GetActorTransform))
  (Networking|SwitchHasAuthority
    (:Authority
      (if (Actor|ActorHasTag OtherActor "Enemy")
        (bind _instigator (Variables|Actor|GetInstigator)
          (:then
            (bind _playerstate (Variables|/Script/Engine.Pawn|GetPlayerState _instigator)
              (:then
                (bind _attack (Class|BPIControlPlayerState|IGetCurrentPlayerStatus(Message) _playerstate))
                (Game|Damage|ApplyDamage OtherActor (* _attack (Variables|Default|GetAttackMag)) (Pawn|GetController _instigator) self "/Game/Workspace/IoriFUKUNAKA/Blueprints/Characters/Player/DamageType/Jufu/D_Tengu.D_Tengu_C")
                (Class|BPIControlEmitter|ISpawnSystematLocation(Message) (Variables|Actor|GetInstigator) "/Game/YinYang_Ryo/NS/NS_E_CMN_WindExplosive.NS_E_CMN_WindExplosive" (.location _returnvalue) (.rotation _returnvalue) "1.000000,1.000000,1.000000")
                (Actor|DestroyActor))
              (:else)))
          (:else))))))

(fn ConstructionScript)