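; Enemy component that tracks the element applied to its owner and triggers Moku/Ka/Kin/Sui combination effects.
; A new element replaces the current one as a timed BP_ElementData object, which an update event ticks and clears on expiry.
; An order-independent pair match instead has the instigator spawn the combination actor at the owner's XY, Z zero, then clears the element.
; MC_SetElement mirrors the current element into HasElement for queries.
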(event Custom|E_GiveElement
  (params (GiveElement :type En_Elements%20Enum :default "NewEnumerator6") (ElementInstigator :type Pawn%20Object%20Reference) (LifeTime :type Float%20%28single-precision%29))
  (bind _returnvalue (Components|GetOwner))
  (bind _returnvalue_2 (Transformation|GetActorLocation _returnvalue))
  (bind _givenelement (Variables|Default|GetGivenElement)
    (:then
      (bind _elementcombinationclass (CallFunction|FCheckFormedCombination (Default|FGetElement _givenelement) GiveElement))
      (if (Utilities|IsValidClass _elementcombinationclass)
        (Class|BPIControlActor|ISpawnActorfromClass(Message) ElementInstigator _elementcombinationclass (Math|Transform|MakeTransform (Math|Vector|MakeVector (.x _returnvalue_2) (.y _returnvalue_2) 0.0) "0, 0, 0" "1,1,1") _returnvalue ElementInstigator)
        (Variables|Default|SetGivenElement 0)
        (CallFunction|MCSetElement "NewEnumerator6")
        (else
          (bind _returnvalue_3 (Game|ConstructObjectfromClass "/Game/Workspace/IoriFUKUNAKA/Blueprints/Characters/DataObject/BP_ElementData.BP_ElementData_C" (Components|GetOwner) GiveElement LifeTime :!label _label))
          (Variables|Default|SetGivenElement _returnvalue_3)
          (CallFunction|MCSetElement GiveElement))))
    (:else
      (goto _label))))

(event Custom|E_UpdateElementManager
  (bind _givenelement (Variables|Default|GetGivenElement)
    (:then
      (Default|EUpdateElementData _givenelement (Utilities|Time|GetWorldDeltaSeconds))
      (if (Default|FIsDead? _givenelement)
        (Variables|Default|SetGivenElement 0)
        (CallFunction|MCSetElement "NewEnumerator6")))
    (:else)))

(event Custom|MC_SetElement
  (params (HasElement :type En_Elements%20Enum :default "NewEnumerator6"))
  (Variables|Default|SetHasElement HasElement))

(fn FCheckFormedCombination
  (params (HasElement :type En_Elements%20Enum :default "NewEnumerator6") (GivenElement :type En_Elements%20Enum :default "NewEnumerator6"))
  (LocalVariables|SethasElem HasElement)
  (LocalVariables|SetgivenElem GivenElement)
  (Utilities|MCheckFormedCombination HasElement GivenElement (Utilities|Set|MakeSet "NewEnumerator0" "NewEnumerator1")
    (:true
      (return "/Game/Workspace/Yamashita/Blueprint/ElementEffect/BP_Moku_Ka.BP_Moku_Ka_C"))
    (:false
      (Utilities|MCheckFormedCombination (LocalVariables|GethasElem) (LocalVariables|GetgivenElem) (Utilities|Set|MakeSet "NewEnumerator0" "NewEnumerator4")
        (:true
          (return "/Game/Workspace/Yamashita/Blueprint/ElementEffect/BP_Moku_Sui.BP_Moku_Sui_C"))
        (:false
          (Utilities|MCheckFormedCombination (LocalVariables|GethasElem) (LocalVariables|GetgivenElem) (Utilities|Set|MakeSet "NewEnumerator1" "NewEnumerator3")
            (:true
              (return "/Game/Workspace/Yamashita/Blueprint/ElementEffect/BP_Ka_Kin.BP_Ka_Kin_C"))
            (:false
              (Utilities|MCheckFormedCombination (LocalVariables|GethasElem) (LocalVariables|GetgivenElem) (Utilities|Set|MakeSet "NewEnumerator1" "NewEnumerator4")
                (:true
                  (return "/Game/Workspace/Yamashita/Blueprint/ElementEffect/BP_Ka_Sui.BP_Ka_Sui_C"))
                (:false
                  (Utilities|MCheckFormedCombination (LocalVariables|GethasElem) (LocalVariables|GetgivenElem) (Utilities|Set|MakeSet "NewEnumerator3" "NewEnumerator0")
                    (:true
                      (return "/Game/Workspace/Yamashita/Blueprint/ElementEffect/BP_Kin_Moku.BP_Kin_Moku_C"))
                    (:false
                      (Utilities|MCheckFormedCombination (LocalVariables|GethasElem) (LocalVariables|GetgivenElem) (Utilities|Set|MakeSet "NewEnumerator3" "NewEnumerator4")
                        (:true
                          (return "/Game/Workspace/Yamashita/Blueprint/ElementEffect/BP_Kin_Sui.BP_Kin_Sui_C"))
                        (:false
                          (return 0))))))))))))))

(fn FGetHasElement
  (bind _haselement (Variables|Default|GetHasElement))
  (if (Utilities|Enum|NotEqual(Enum) _haselement "NewEnumerator6")
    (return true _haselement)
    (else
      (return false "NewEnumerator6"))))