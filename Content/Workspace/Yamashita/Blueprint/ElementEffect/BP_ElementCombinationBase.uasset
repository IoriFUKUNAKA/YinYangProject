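; Base actor for element combination effects, with empty initialize, effect and finalize functions that appear intended for child overrides.
; On BeginPlay, only the authority runs the combination effect.
; Continuous effects start a lifetime timer and a looping timer calling F_Effect by name, which is not defined in this graph.
; Non-continuous effects go straight to E_Destroy, which finalizes and destroys the actor.
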(event Custom|E_Destroy
  (CallFunction|FFinalize)
  (Actor|DestroyActor))

(event EventBeginPlay
  (Networking|SwitchHasAuthority
    (:Authority
      (CallFunction|FCombinationEffect)
      (if (Variables|Default|Getcontinuation)
        (Utilities|Time|SetTimerbyEvent (EventDispatchers|CreateEvent :!event Custom|E_Destroy) (Variables|Default|GetLifeTime))
        (Utilities|Time|SetTimerbyFunctionName self "F_Effect" (Variables|Default|GetEffectSpan) true)
        (else
          (CallFunction|EDestroy))))))

(fn ConstructionScript)

(fn FInitialize)

(fn FCombinationEffect)

(fn FFinalize)