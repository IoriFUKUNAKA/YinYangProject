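; Syutendouji yokai jufu actor that runs the player's multi-hit attack, driven by jufu animation notifies.
; On init it turns the player toward a nearby enemy, then spawns attack actors at notify begins, nudging rotation toward input for Attack 02.
; Attack 02 and 03 notify ends apply server-routed Kin-element damage to enemies in the Attack 02 area, with 03 adding a debuff.
; Animation completion has the player destroy it.
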(event Custom|E_OnJufuAnimCompleated
  (bind _instigatorplayer (Variables|Default|GetInstigatorPlayer)
    (:then
      (Default|IDestroyActor _instigatorplayer self))
    (:else)))

(event Custom|E_OnAnimNotifyEnd
  (params (NotifyName :type Name))
  (switch name NotifyName
    (:Attack02
      (bind _instigatorplayer (Variables|Default|GetInstigatorPlayer)
        (:then
          (bind _playerstate (Variables|/Script/Engine.Pawn|GetPlayerState _instigatorplayer)
            (:then
              (bind _attack (Class|BPIControlPlayerState|IGetCurrentPlayerStatus(Message) _playerstate))
              (bind _attackarea2 (Variables|Default|GetAttackArea2)
                (:then
                  (for _array_element (Variables|/Game/Workspace/IoriFUKUNAKA/Blueprints/Characters/Player/Jufu/Yokai/Syutendouji/BP_Syutendouji_Attack02.BP_Syutendouji_Attack02_C|GetEnemyList _attackarea2)
                    (CallFunction|ROSApplyDamage _array_element (* _attack (Variables|コンフィグ|GetAttackMagnification)) (Pawn|GetController _instigatorplayer) _attackarea2 "/Game/Workspace/IoriFUKUNAKA/Blueprints/Characters/Player/DamageType/D_GiveElementDamage_Kin.D_GiveElementDamage_Kin_C")))
                (:else)))
            (:else)))
        (:else)))
    (:Attack03
      (bind _instigatorplayer_2 (Variables|Default|GetInstigatorPlayer)
        (:then
          (bind _playerstate_2 (Variables|/Script/Engine.Pawn|GetPlayerState _instigatorplayer_2)
            (:then
              (bind _attack_2 (Class|BPIControlPlayerState|IGetCurrentPlayerStatus(Message) _playerstate_2))
              (bind _attackarea2_2 (Variables|Default|GetAttackArea2)
                (:then
                  (for _array_element_2 (Variables|/Game/Workspace/IoriFUKUNAKA/Blueprints/Characters/Player/Jufu/Yokai/Syutendouji/BP_Syutendouji_Attack02.BP_Syutendouji_Attack02_C|GetEnemyList _attackarea2_2)
                    (CallFunction|ROSApplyDamage _array_element_2 (* _attack_2 (Variables|コンフィグ|GetAttackMagnification)) (Pawn|GetController _instigatorplayer_2) _attackarea2_2 "/Game/Workspace/IoriFUKUNAKA/Blueprints/Characters/Player/DamageType/D_GiveElementDamage_Kin.D_GiveElementDamage_Kin_C")
                    (CallFunction|ROSDebuff _array_element_2)))
                (:else)))
            (:else)))
        (:else)))))

(event Custom|E_OnAnimNotifyBegin
  (params (NotifyName :type Name))
  (switch name NotifyName
    (:Attack01
      (bind _instigatorplayer (Variables|Default|GetInstigatorPlayer)
        (:then
          (Game|SpawnActorfromClass "/Game/Workspace/IoriFUKUNAKA/Blueprints/Characters/Player/Jufu/Yokai/Syutendouji/BP_Syutendouji_Attack01.BP_Syutendouji_Attack01_C" (Math|Transform|MakeTransform (+ (.location (Transformation|GetActorTransform _instigatorplayer)) (* (Math|Vector|GetForwardVector (.rotation (Transformation|GetActorTransform _instigatorplayer))) 2e+02)) (.rotation (Transformation|GetActorTransform _instigatorplayer)) "1,1,1") "Undefined" self _instigatorplayer))
        (:else)))
    (:Attack02
      (bind _instigatorplayer_2 (Variables|Default|GetInstigatorPlayer)
        (:then
          (Transformation|SetActorRotation _instigatorplayer_2 (Math|Rotator|Lerp(Rotator) (Math|Rotator|MakeRotator 0.0 0.0 (.Yaw (Math|Rotator|BreakRotator (Transformation|GetActorRotation _instigatorplayer_2)))) (Math|Rotator|MakeRotator 0.0 0.0 (.Yaw (Math|Rotator|BreakRotator (Default|FCalcInputRotate _instigatorplayer_2)))) 0.2 true))
          (Default|ROSSetActorRotation _instigatorplayer_2 (Math|Rotator|Lerp(Rotator) (Math|Rotator|MakeRotator 0.0 0.0 (.Yaw (Math|Rotator|BreakRotator (Transformation|GetActorRotation _instigatorplayer_2)))) (Math|Rotator|MakeRotator 0.0 0.0 (.Yaw (Math|Rotator|BreakRotator (Default|FCalcInputRotate _instigatorplayer_2)))) 0.2 true) false)
          (bind _returnvalue (Game|SpawnActorfromClass "/Game/Workspace/IoriFUKUNAKA/Blueprints/Characters/Player/Jufu/Yokai/Syutendouji/BP_Syutendouji_Attack02.BP_Syutendouji_Attack02_C" (Math|Transform|MakeTransform (+ (.location (Transformation|GetActorTransform _instigatorplayer_2)) (* (Math|Vector|GetForwardVector (.rotation (Transformation|GetActorTransform _instigatorplayer_2))) 8e+02)) (.rotation (Transformation|GetActorTransform _instigatorplayer_2)) "1,1,1") "Undefined" self _instigatorplayer_2))
          (Variables|Default|SetAttackArea2 _returnvalue))
        (:else)))))

(event Custom|E_BindOnJufuAnimNotifyEvent
  (bind _instigatorplayer (Variables|Default|GetInstigatorPlayer)
    (:then
      (EventDispatchers|BindEventtoOnJufuAnimNotifyBegin _instigatorplayer (EventDispatchers|CreateEvent :!event Custom|E_OnAnimNotifyBegin))
      (EventDispatchers|BindEventtoOnJufuAnimNotifyEnd _instigatorplayer (EventDispatchers|CreateEvent :!event Custom|E_OnAnimNotifyEnd))
      (EventDispatchers|BindEventtoOnJufuAnimCompleated _instigatorplayer (EventDispatchers|CreateEvent :!event Custom|E_OnJufuAnimCompleated)))
    (:else)))

(event Custom|MC_InitializeSyutendoji
  (bind _instigator (Variables|Default|GetInstigator)
    (:then
      (bind _asbp_yin_yang_player (Utilities|Casting|CastToBP_YinYangPlayer _instigator))
      (bind _output_get (Variables|Default|SetInstigatorPlayer _asbp_yin_yang_player))
      (bind _rotation (Default|FRotationtoNearEnemy _output_get 1e+03))
      (Transformation|SetActorRotation _output_get _rotation)
      (CallFunction|EBindonJufuAnimNotifyEvent))
    (:else)))

(event Custom|ROS_ApplyDamage
  (params (DamagedActor :type Actor%20Object%20Reference) (BaseDamage :type Float%20%28single-precision%29) (EventInstigator :type Controller%20Object%20Reference) (DamageCauser :type Actor%20Object%20Reference) (DamageTypeClass :type Damage%20Type%20Class%20Reference))
  (Game|Damage|ApplyDamage DamagedActor BaseDamage EventInstigator DamageCauser DamageTypeClass))

(event Custom|ROS_Debuff
  (params (TargetEnemy :type Actor%20Object%20Reference))
  (bind _returnvalue (Actor|GetComponentbyClass TargetEnemy "/Game/Workspace/IoriFUKUNAKA/Blueprints/Characters/BPC_BuffManager.BPC_BuffManager_C"))
  (Utilities|IsValid _returnvalue
    (:Is%20Valid
      (Default|ROCAddBuffEffect _returnvalue "NewEnumerator1" (Variables|Default|GetEffect%20Value) (Variables|Default|GetLife%20Time)))))

(fn ConstructionScript
  (|CallParentFunction))

(fn FonInitialize
  (|CallParentFunction)
  (CallFunction|MCInitializeSyutendoji))