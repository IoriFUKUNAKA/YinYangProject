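; Player skill actor that applies a timed status buff, named as a defence buff, to its owner.
; On initialization with a valid owner, it creates a status data object from its effect value and lifetime and adds it to the owner's status manager.
; It then plays a status-up sound at the owner's location and destroys itself, leaving the effect with the status manager.
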(fn ConstructionScript
  (|CallParentFunction))

(fn FInitialize
  (|CallParentFunction)
  (bind _m_owner (Variables|Default|Getm_Owner)
    (:then
      (bind _returnvalue (Game|ConstructObjectfromClass "/Game/Workspace/IoriFUKUNAKA/Blueprints/Characters/StatusData/BP_StatusData.BP_StatusData_C" (Variables|/Game/Workspace/IoriFUKUNAKA/Blueprints/Characters/Player/BP_Player.BP_Player_C|GetBPC_StatusManager _m_owner) "NewEnumerator1" (Variables|プランナー編集可|GetEffect%20Value) (Variables|プランナー編集可|GetEffectLife%20Time)))
      (Default|EAddEffect (Variables|/Game/Workspace/IoriFUKUNAKA/Blueprints/Characters/Player/BP_Player.BP_Player_C|GetBPC_StatusManager _m_owner) _returnvalue)
      (Default|MCPlaySE _m_owner "/Game/Workspace/IoriFUKUNAKA/Sounds/SC_StatusUp.SC_StatusUp" (Transformation|GetActorLocation _m_owner) 1.0 "/Game/Workspace/IoriFUKUNAKA/Sounds/SA_PlayerSE.SA_PlayerSE")
      (Actor|DestroyActor))
    (:else)))