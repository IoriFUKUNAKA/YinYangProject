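; Base Blueprint for a visual player character whose emissive color reflects the element of the player at a given PlayerArray index.
; On BeginPlay it creates a dynamic instance of MI_Boy_Emissive and applies the current element's color.
; Tick polls that PlayerState through an interface message and updates EmissiveColor from a color lookup when the element changes.
; The instance is created on a configurable slot, but recoloring always assigns it to slot 4.
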(event Custom|E_CheckAtrribute
  ;[1 1 1] 属性をチェック
  (bind _element (Class|BPIControlPlayerState|IGetElement(Message) (Utilities|Array|Get(acopy) (Variables|/Script/Engine.GameStateBase|GetPlayerArray (Game|GetGameState)) (Variables|Default|Getindex))))
  (if (Utilities|Enum|NotEqual(Enum) _element (Variables|Default|Getelement))
    (CallFunction|EChangeMaterialColor _element)
    (Variables|Default|Setelement _element)))

(event Custom|E_ChangeMaterialColor
  (params (NewParam :type En_Elements%20Enum :default "NewEnumerator6"))
  ;[1 1 1] マテリアルパラメータを変更
  (Rendering|Material|SetVectorParameterValue (Variables|Default|GetEmissiveMI) "EmissiveColor" (Utilities|Array|Get(acopy) (Variables|Default|GetElementColor) (Math|Conversions|ToInteger(Byte) NewParam)) :!class /Script/Engine.MaterialInstanceDynamic)
  (Rendering|Material|SetMaterial (Variables|Default|GetMesh) 4 (Variables|Default|GetEmissiveMI)))

(event Custom|E_setMaterial
  (params (ElementIndex :type Integer))
  ;[1 1 1] マテリアルインスタンスを設定
  (bind _returnvalue (Rendering|Material|CreateDynamicMaterialInstance (Variables|Default|GetMesh) ElementIndex "/Game/Workspace/IoriFUKUNAKA/Materials/LightingTest/YinYangCharacters/MI_Boy_Emissive.MI_Boy_Emissive" "None" :!class /Script/Engine.PrimitiveComponent))
  (Variables|Default|SetEmissiveMI _returnvalue))

(event EventTick
  (params (DeltaSeconds :type Float%20%28single-precision%29))
  (CallFunction|ECheckAtrribute))

(event EventBeginPlay
  (CallFunction|ESetMaterial (Variables|Default|GetmaterialElementIndex))
  (bind _element (Class|BPIControlPlayerState|IGetElement(Message) (Utilities|Array|Get(acopy) (Variables|/Script/Engine.GameStateBase|GetPlayerArray (Game|GetGameState)) (Variables|Default|Getindex))))
  (CallFunction|EChangeMaterialColor _element))

(fn ConstructionScript)