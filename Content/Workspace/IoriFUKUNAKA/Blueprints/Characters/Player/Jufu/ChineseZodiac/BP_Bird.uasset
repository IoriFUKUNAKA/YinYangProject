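; BP_Bird is the Bird entry of the player's Chinese zodiac Jufu set, a one-shot party resurrection effect.
; On initialization it reads Attack from the instigator's PlayerState, then sends a resurrection message to every PlayerState in the GameState's player array.
; Each message carries an amount scaled from Attack by HealMag with slight random variance.
; The actor then destroys itself, provided the instigator and its PlayerState were valid.
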(fn ConstructionScript
  (|CallParentFunction))

(fn FonInitialize
  (|CallParentFunction)
  (bind _instigator (Variables|Default|GetInstigator)
    (:then
      (bind _playerstate (Variables|/Script/Engine.Pawn|GetPlayerState _instigator)
        (:then
          (bind _attack (Class|BPIControlPlayerState|IGetCurrentPlayerStatus(Message) _playerstate))
          (for _array_element (Variables|/Script/Engine.GameStateBase|GetPlayerArray (Game|GetGameState))
            (Class|BPIControlPlayer|IRessurectionPlayer(Message) _array_element (Math|Float|Truncate (* (* _attack (Variables|Default|GetHealMag)) (Math|Random|RandomFloatinRange 0.9 1.1)))))
          (Actor|DestroyActor))
        (:else)))
    (:else)))