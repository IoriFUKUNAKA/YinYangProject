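; BP_GameManager is a manager Blueprint that keeps registries of player and enemy references and answers nearest-enemy queries.
; BeginPlay caches GM_Main through ROS_GetGameMode, while Tick prints gamepad connection status for debugging.
; The query compares squared 2D distances within a cutoff radius and returns a position and validity flag.
; Its closer-enemy branch reassigns NearEnemy to itself, so the first in-range enemy stays selected.
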(event EventTick
  (params (DeltaSeconds :type Float%20%28single-precision%29))
  (bind _returnvalue (Class|AppUtilBPLibrary|IsGamePadConnected))
  (Development|PrintText (Utilities|Text|FormatText "ゲームパッド接続判定：{0}" _returnvalue) true true "(R=1.000000,G=0.000000,B=0.901710,A=1.000000)" 0.0))

(event EventBeginPlay
  (CallFunction|ROSGetGameMode))

(event Custom|ROS_GetGameMode
  (bind _asgm_main (Utilities|Casting|CastToGM_Main (Game|GetGameMode)))
  (Variables|Ref|Setm_GM _asgm_main))

(fn ConstructionScript)

(fn FAddPlayerRef
  (params (PlayerRef :type BP%20Player%20Object%20Reference))
  (Utilities|Array|AddUnique (Variables|Ref|GetPlayersRef) PlayerRef))

(fn FAddEnemyRef
  (params (EnemyRef :type BP%20Enemy%20Test%20Object%20Reference))
  (Utilities|Array|AddUnique (Variables|Ref|GetEnemiesRef) EnemyRef))

(fn FResetRefArrays
  (Utilities|Array|Clear (Variables|Ref|GetPlayersRef))
  (Utilities|Array|Clear (Variables|Ref|GetEnemiesRef)))

(fn FGetNearEnemyfromPlayer
  (params (PlayerPos :type Vector))
  (for _array_element (Variables|Ref|GetEnemiesRef)
    (Utilities|IsValid _array_element
      (:Is%20Valid
        (bind __nearenemy (LocalVariables|Get_NearEnemy)
          (:then
            (if (< (Class|KismetMathLibrary|VectorDistance2DSquared PlayerPos (Transformation|GetActorLocation _array_element)) (LocalVariables|Get_SqrDistance))
              (LocalVariables|Set_NearEnemy __nearenemy)
              (LocalVariables|Set_SqrDistance (Class|KismetMathLibrary|VectorDistance2DSquared PlayerPos (Transformation|GetActorLocation _array_element)))))
          (:else
            (if (<= (Class|KismetMathLibrary|VectorDistance2DSquared PlayerPos (Transformation|GetActorLocation _array_element)) (Math|Float|Power (Variables|プロパティ|GetCheckDistanceDeadLine) 2.0))
              (LocalVariables|Set_NearEnemy _array_element)
              (LocalVariables|Set_SqrDistance (Class|KismetMathLibrary|VectorDistance2DSquared PlayerPos (Transformation|GetActorLocation _array_element)))))))))
  (bind __nearenemy_2 (LocalVariables|Get_NearEnemy)
    (:then
      (return (Transformation|GetActorLocation __nearenemy_2) true))
    (:else
      (return "0, 0, 0" false))))