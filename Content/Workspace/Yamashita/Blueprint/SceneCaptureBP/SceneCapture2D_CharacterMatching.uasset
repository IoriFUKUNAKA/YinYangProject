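; Scene capture actor for character matching that renders the character actors registered in its show-only list.
; A RoS event forwards each actor to an MC event, named as a server-to-multicast relay, which appends it to the capture component's ShowOnlyActors.
; Tick prints the actor's name and current list count as debug text.
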(event Custom|RoS_AddShowCharacter
  (params (ShowActor :type Actor%20Object%20Reference))
  (CallFunction|MCAddShowCharacter ShowActor))

(event Custom|MC_AddShowCharacter
  (params (NewItem :type Actor%20Object%20Reference%20%28by%20ref%29))
  (Utilities|Array|Add (Variables|/Script/Engine.SceneCaptureComponent|GetShowOnlyActors (Variables|DecalActor|GetCaptureComponent2D)) NewItem))

(event EventTick
  (params (DeltaSeconds :type Float%20%28single-precision%29))
  (Development|PrintText (Utilities|Text|FormatText "{thiname}:{num}" (Utilities|GetObjectName self) (Utilities|Array|Length (Variables|/Script/Engine.SceneCaptureComponent|GetShowOnlyActors (Variables|DecalActor|GetCaptureComponent2D)))) true true "(R=0.191844,G=1.000000,B=0.000000,A=1.000000)" 0.0))

(fn ConstructionScript)