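; Game Instance for the YinYang project that manages two-player online session create, join and destroy.
; Creating a session, with LAN use set by a variable, opens the debug level as a listen server.
; Destroying a session returns to the login level, while joining only reports its result.
; Session failures and network or travel errors are printed to screen for debugging.
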(event Custom|E_CreateSession
  ;[1 1 1] セッションを作成
  (|Session (Game|GetPlayerController 0) 2 (Variables|Default|GetUse%20LAN) ; 同時に2人まで
    (:OnSuccess
      (Game|OpenLevel(byName) "L_Debug" true "listen"))
    (:OnFailure
      (Development|PrintString "Create Session Failure" true true "(R=1.000000,G=0.000000,B=0.020907,A=1.000000)"))))

(event Custom|E_DestroySession
  (params (PlayerController :type Player%20Controller%20Object%20Reference))
  ;[1 1 1] セッションの破棄
  (|DestroySession PlayerController
    (:OnSuccess
      (Game|OpenLevel(byName) "L_Login"))
    (:OnFailure
      (Development|PrintString "Destroy Session Failure" true true "(R=1.000000,G=0.000000,B=0.000000,A=1.000000)"))))

(event Custom|E_JoinSession
  (params (PlayerController :type Player%20Controller%20Object%20Reference) (Session :type Blueprint%20Session%20Result%20Structure%20%28by%20ref%29))
  ;[1 1 1] セッションへの参加
  (|JoinSession PlayerController Session
    (:OnSuccess
      (Development|PrintString "join Session Success"))
    (:OnFailure
      (Development|PrintString "Join Session Failure" true true "(R=1.000000,G=0.000000,B=0.000000,A=1.000000)"))))

(event EventHandleNetworkError
  (params (FailureType :type ENetworkFailure%20Enum :default "NetDriverAlreadyExists") (bIsServer :type Boolean))
  ;[1 1 1] ネットワークエラーハンドリング
  (Development|PrintString (Utilities|String|EnumtoString FailureType) true true "(R=1.000000,G=0.000000,B=0.000000,A=1.000000)"))

(event EventHandleTravelError
  (params (FailureType :type ETravelFailure%20Enum :default "NoLevel"))
  ;[1 1 1] トラベルエラーハンドリング
  (Development|PrintString (Utilities|String|EnumtoString FailureType) true true "(R=1.000000,G=0.000000,B=0.000000,A=1.000000)"))