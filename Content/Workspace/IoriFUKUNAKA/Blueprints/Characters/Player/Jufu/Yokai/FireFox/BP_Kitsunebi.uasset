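; Fox-fire (Kitsunebi) projectile for the player's FireFox yokai that homes on a target and damages enemies.
; After a short random delay it launches along an injection direction and plays a timeline.
; The timeline blends velocity toward the target, zeroing vertical speed unless rising above a height threshold.
; On overlapping an Enemy, the server applies randomized fire-element damage scaled from the instigating player's Attack, then destroys it.
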(event OnComponentBeginOverlap(Collision)
  (params (OverlappedComponent :type Primitive%20Component%20Object%20Reference) (OtherActor :type Actor%20Object%20Reference) (OtherComp :type Primitive%20Component%20Object%20Reference) (OtherBodyIndex :type Integer) (bFromSweep :type Boolean) (SweepResult :type Hit%20Result%20Structure%20%28by%20ref%29))
  (Networking|SwitchHasAuthority
    (:Authority
      (if (Actor|ActorHasTag OtherActor "Enemy")
        (bind _instigator (Variables|Actor|GetInstigator)
          (:then
            (bind _playerstate (Variables|/Script/Engine.Pawn|GetPlayerState _instigator)
              (:then
                (bind _attack (Class|BPIControlPlayerState|IGetCurrentPlayerStatus(Message) _playerstate))
                (Game|Damage|ApplyDamage OtherActor (* _attack (Variables|Config|GetDamageMag) (Math|Random|RandomFloatinRange 0.9 1.1)) 0 self "/Game/Workspace/IoriFUKUNAKA/Blueprints/Characters/Player/DamageType/D_GiveElementDamage_Ka.D_GiveElementDamage_Ka_C")
                (Actor|DestroyActor))
              (:else)))
          (:else))))))

(event Custom|E_InitializeKitsunebi
  (Utilities|FlowControl|Delay (Math|Random|RandomFloatinRange 0.0 0.5))
  (Variables|/Script/Engine.MovementComponent|SetVelocity (Variables|Default|GetProjectileMovement) (* (Math|Vector|Normalize (Variables|プロパティ|GetInjectionDir)) (Variables|Config|GetSpeed)))
  (Components|Timeline|PlayfromStart (Variables|Default|GetHomingRate)))

(fn ConstructionScript)