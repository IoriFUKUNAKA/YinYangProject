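; BP_Boar is the Boar Chinese-zodiac jufu for the player, confining its owner to a circular movable area for a limited lifetime.
; On initialize it sets its life span and sends the owner an interface message with the area radius, centered on the owner's XY position at zero height.
; It scales BarrierPivot from that radius plus padding.
; On destroy it tells the owner to reset the movable area.
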(fn ConstructionScript
  (|CallParentFunction))

(fn FonInitialize
  (bind _returnvalue (Components|GetOwner))
  (bind _arearadius (Variables|Config|GetAreaRadius))
  (bind _returnvalue_2 (Transformation|GetActorLocation _returnvalue))
  (bind _returnvalue_3 (+ _arearadius 5e+02))
  (bind (_x _y) (Math|Vector|BreakVector _returnvalue_2))
  (bind _returnvalue_4 (/ _returnvalue_3 1e+02))
  (|CallParentFunction)
  (Actor|SetLifeSpan (Variables|コンフィグ|GetLifeTime))
  (Class|BPIEnemy|ISetMovableArea(Message) _returnvalue (Math|Vector|MakeVector _x _y 0.0) _arearadius)
  (Transformation|SetRelativeScale3D (Variables|Default|GetBarrierPivot) (Math|Vector|MakeVector _returnvalue_4 _returnvalue_4 4.0)))

(fn FonDestroy
  (|CallParentFunction)
  (Class|BPIEnemy|IResetMovableArea(Message) (Components|GetOwner)))