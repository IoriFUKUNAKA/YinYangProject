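; Barrier skill actor that grants super armor to players standing inside its sphere.
; On the server, sphere overlap begin adds each BP_Player to an in-area list and turns super armor on through its status manager component.
; Overlap end removes the player from the list and turns super armor off only if the removal succeeds.
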(event OnComponentBeginOverlap(Sphere)
  (params (OverlappedComponent :type Primitive%20Component%20Object%20Reference) (OtherActor :type Actor%20Object%20Reference) (OtherComp :type Primitive%20Component%20Object%20Reference) (OtherBodyIndex :type Integer) (bFromSweep :type Boolean) (SweepResult :type Hit%20Result%20Structure%20%28by%20ref%29))
  (Networking|SwitchHasAuthority
    (:Authority
      (bind _asbp_player (Utilities|Casting|CastToBP_Player OtherActor))
      (Utilities|Array|AddUnique (Variables|Default|GetInAreaPlayers) _asbp_player)
      (Default|FShiftSuperArmor (Variables|/Game/Workspace/IoriFUKUNAKA/Blueprints/Characters/Player/BP_Player.BP_Player_C|GetBPC_StatusManager _asbp_player) true))))

(event OnComponentEndOverlap(Sphere)
  (params (OverlappedComponent :type Primitive%20Component%20Object%20Reference) (OtherActor :type Actor%20Object%20Reference) (OtherComp :type Primitive%20Component%20Object%20Reference) (OtherBodyIndex :type Integer))
  (Networking|SwitchHasAuthority
    (:Authority
      (bind _asbp_player (Utilities|Casting|CastToBP_Player OtherActor))
      (bind _returnvalue (Utilities|Array|RemoveItem (Variables|Default|GetInAreaPlayers) _asbp_player))
      (if _returnvalue
        (Default|FShiftSuperArmor (Variables|/Game/Workspace/IoriFUKUNAKA/Blueprints/Characters/Player/BP_Player.BP_Player_C|GetBPC_StatusManager _asbp_player) false)))))

(fn ConstructionScript
  (|CallParentFunction))