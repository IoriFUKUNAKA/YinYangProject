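; BP_CallThunder is a delayed lightning strike for the Kirin enemy, telegraphed by a ground decal scaled to the attack radius.
; A server init call multicasts radius and delay, then starts the attack timer.
; Tick fills the decal material over the delay, then a timeline animates emissive and alpha before hiding it.
; The attack spawns a Niagara thunder effect, runs EnemyRef's sphere overlap check, and destroys the actor shortly afterward.
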(event Custom|MC_SetInit
  (params (AttackRadius :type Float%20%28single-precision%29) (AttackDelay :type Float%20%28single-precision%29))
  (bind _returnvalue (* AttackRadius 0.01))
  ;[1 1 1] 初期化
  (Variables|Default|SetAttackRadius AttackRadius)
  (Variables|Default|SetAttackDelay AttackDelay)
  (Transformation|SetRelativeScale3D (Variables|Default|GetDecal) (Math|Vector|MakeVector _returnvalue _returnvalue _returnvalue))
  (Utilities|Time|SetTimerbyEvent (EventDispatchers|CreateEvent :!event Custom|E_Attack) AttackDelay))

(event Custom|E_Attack
  ;[1 1 1] 攻撃
  (CallFunction|MCSpawnEffect)
  (Default|FSphereOverlap (Variables|Default|GetEnemyRef) (Transformation|GetActorLocation) (Variables|Default|GetAttackRadius) false false 5)
  (Utilities|FlowControl|Delay 2.0)
  (Actor|DestroyActor))

(event Custom|RoS_SetInit
  (params (AttackRadius :type Float%20%28single-precision%29) (AttackDelay :type Float%20%28single-precision%29))
  ;[1 1 1] 初期化
  (CallFunction|MCSetInit AttackRadius AttackDelay))

(event Custom|E_UpdateTimer
  ;[1 1 1] デカールマテリアルパラメータ調整
  (bind _output_get (Variables|Default|Settimer (Math|Float|Min(Float) (+ (Variables|Default|Gettimer) (Utilities|Time|GetWorldDeltaSeconds)) (Variables|Default|GetAttackDelay))))
  (Rendering|Material|SetScalarParameterValue (Variables|Default|GetM_Decal) "Rate" (/ _output_get (Variables|Default|GetAttackDelay)) :!class /Script/Engine.MaterialInstanceDynamic)
  (if (>= (/ _output_get (- (Variables|Default|GetAttackDelay) 0.0)) 1.0)
    (Utilities|FlowControl|DoOnce false
      (:Completed
        (bind (_direction _pow _alpha) (Timeline|Emissive Play)
          (:Update
            (Rendering|Material|SetScalarParameterValue (Variables|Default|GetM_Decal) "EmissivePow" _pow :!class /Script/Engine.MaterialInstanceDynamic)
            (Rendering|Material|SetScalarParameterValue (Variables|Default|GetM_Decal) "alpha" _alpha :!class /Script/Engine.MaterialInstanceDynamic))
          (:Finished
            (Rendering|SetVisibility (Variables|Default|GetDecal) false false)))))))

(event Custom|MC_SpawnEffect
  ;[1 1 1] エフェクト生成
  (bind _returnvalue (Niagara|SpawnSystematLocation "/Game/YinYang_Ryo/NS/NS_E_CMN_FallTuhnder001_00.NS_E_CMN_FallTuhnder001_00" (Transformation|GetActorLocation)))
  (Effects|Components|ParticleSystem|SetFloatParameter _returnvalue "Size_Area" 0.3))

(event EventBeginPlay
  (|CallParentFunction)
  (bind _returnvalue (Rendering|Material|CreateDynamicMaterialInstance (Variables|Default|GetDecal) :!class /Script/Engine.DecalComponent))
  (Variables|Default|SetM_Decal _returnvalue))

(event EventTick
  (params (DeltaSeconds :type Float%20%28single-precision%29))
  (|CallParentFunction DeltaSeconds)
  (CallFunction|EUpdateTimer))

(fn ConstructionScript
  (|CallParentFunction))