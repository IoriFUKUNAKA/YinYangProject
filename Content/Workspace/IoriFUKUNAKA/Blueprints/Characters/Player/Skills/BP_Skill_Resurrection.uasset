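; BP_Skill_Resurrection is a player skill that resurrects one other player when the skill initializes.
; After the parent initialization, it runs on authority only and requires a valid owner.
; It walks the game manager's player list in reverse, skipping the owner, calls EResurrection on the first player found in a specific player state, then stops.
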(fn ConstructionScript
  (|CallParentFunction))

(fn FInitialize
  (|CallParentFunction)
  (Networking|SwitchHasAuthority
    (:Authority
      (bind _m_owner (Variables|Default|Getm_Owner)
        (:then
          (bind _arrayelement (Utilities|MReverseForeachRef (Default|FGetPlayersRef (Variables|/Game/Workspace/IoriFUKUNAKA/Blueprints/Characters/Player/BP_Player.BP_Player_C|Getm_GameManager _m_owner)) :!label _label)
            (:LoopBody
              (if (!= _arrayelement (Variables|Default|Getm_Owner))
                (if (Utilities|Enum|Equal(Enum) (Default|FGetCurrentPlayerState _arrayelement) "NewEnumerator6")
                  (Default|EResurrection _arrayelement)
                  (goto _label Break))))))
        (:else)))))