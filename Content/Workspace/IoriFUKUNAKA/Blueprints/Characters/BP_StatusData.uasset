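; BP_StatusData holds a single timed status effect for characters, with a type, effect value, lifetime and elapsed time.
; An update event adds delta time to the elapsed time until the lifetime is reached, at which point the effect reports itself dead.
; A lifetime of zero never expires, and a positive effect value counts as a buff.
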(event Custom|E_UpdateStatus
  (params (_DeltaTIme :type Float%20%28single-precision%29))
  (if (> (Variables|Default|Getm_LifeTime) 0.0)
    (if (not (CallFunction|FIsDead?))
      (Variables|Default|Setm_Elapsed (+ _DeltaTIme (Variables|Default|Getm_Elapsed))))))

(fn FIsDead?
  (bind _m_lifetime (Variables|Default|Getm_LifeTime))
  (return (and (>= (Variables|Default|Getm_Elapsed) _m_lifetime) (!= _m_lifetime 0.0))))

(fn FIsBuff?
  (return (> (Variables|Default|Getm_EffectValue) 0.0)))

(fn FGetType
  (return (Variables|Default|Getm_Type)))

(fn FGetEffectValue
  (return (Variables|Default|Getm_EffectValue)))