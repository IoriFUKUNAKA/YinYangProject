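; BPC_SkillHolder is a player component that holds a single skill with its chant time, cooldown, mana cost and hate value.
; An init event copies these from skill data if the class is valid, and getters expose most of them with readiness.
; Activation clears readiness and spawns the skill actor at the owning BP_Player's mesh location, then initializes it.
; An externally called update event accumulates delta time until the cooldown restores readiness.
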(event Custom|E_initializeSkillHolder
  (params (StoringSkillData :type ST%20Skill%20Data%20Structure))
  (bind (_name _id _chanttime _cooltime _usemana _hate _detail _characterimage _skillthumbnail _cutintexture _skill) (Utilities|Struct|BreakST_SkillData StoringSkillData))
  ;[1 1 1] 初期化処理
  (if (Utilities|IsValidClass _skill)
    (Variables|詠唱時間|SetChantTime _chanttime)
    (Variables|冷却時間|SetCoolTime _cooltime)
    (Variables|スキル|SetUseMana _usemana)
    (Variables|スキル|SetHate%20Value _hate)
    (Variables|スキル|SetStoredSkill _skill)))

(event Custom|E_CoolingUpdate
  ;[1 1 1] 冷却時間
  (if (not (Variables|冷却時間|GetisReady?))
    (if (>= (+ (Variables|冷却時間|GetCoolingElapsed) (Utilities|Time|GetWorldDeltaSeconds)) (Variables|冷却時間|GetCoolTime))
      (Variables|冷却時間|SetisReady? true)
      (Variables|冷却時間|SetCoolingElapsed 0.0)
      (else
        (Variables|冷却時間|SetCoolingElapsed (+ (Variables|冷却時間|GetCoolingElapsed) (Utilities|Time|GetWorldDeltaSeconds)))))))

(event Custom|ROS_SpawnSkill
  (bind _returnvalue (Components|GetOwner))
  ;[1 1 1] スキルの使用
  (bind _asbp_player (Utilities|Casting|CastToBP_Player _returnvalue))
  (bind _returnvalue_2 (Game|SpawnActorfromClass (Variables|スキル|GetStoredSkill) (Math|Transform|MakeTransform (Transformation|GetWorldLocation (Variables|/Script/Engine.Character|GetMesh _asbp_player)) "0, 0, 0" "1,1,1") "Undefined" _returnvalue 0))
  (Default|EInitialize _returnvalue_2))

(event Custom|E_SkillActivate
  ;[1 1 1] スキルの使用
  (Variables|冷却時間|SetisReady? false)
  (CallFunction|ROSSpawnSkill))

(event Custom|E_Update
  ;[1 1 1] 更新処理
  (CallFunction|ECoolingUpdate))

(fn FIsStoredSkiill?
  (return (Utilities|IsValidClass (Variables|スキル|GetStoredSkill))))

(fn FGetMana
  (return (Variables|スキル|GetUseMana)))

(fn FGetChantTime
  (return (Variables|詠唱時間|GetChantTime)))

(fn FGetisReady?
  (return (Variables|冷却時間|GetisReady?)))

(fn FGetCoolingTime
  (return (Variables|冷却時間|GetCoolTime)))

(fn FGetCoolingElapsed
  (return (Variables|冷却時間|GetCoolingElapsed)))