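; PC_Login is the player controller for the login flow, showing and hiding the login menu and server list widgets.
; Show events create each widget on first use, cache it, switch to UI-only input and add it to the viewport, also initializing the login menu.
; A separate event replaces any existing fade widget with a new one at the given alpha, layered at a higher Z-order.
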(event Custom|RoC_CreateFadeWidget
  (params (Alpha :type Float%20%28single-precision%29))
  (Utilities|IsValid (Variables|Default|GetFadeUI)
    (:Is%20Valid
      (Widget|RemovefromParent (Variables|Default|GetFadeUI)))
    (:Is%20Not%20Valid
      _))
  (bind _returnvalue (UserInterface|CreateWidget "/Game/Workspace/Yamashita/Blueprint/UI/WBP_Fade.WBP_Fade_C" self Alpha))
  (bind _output_get (Variables|Default|SetFadeUI _returnvalue))
  (UserInterface|Viewport|AddtoViewport _output_get 10))

(event EventIShowLoginMenu
  ;[1 1 1] LoginMenuを表示する
  (Utilities|IsValid (Variables|Default|GetLoginMenu)
    (:Is%20Valid
      _)
    (:Is%20Not%20Valid
      (bind _returnvalue (UserInterface|CreateWidget "/Game/Workspace/IoriFUKUNAKA/Blueprints/HeadUpDisplays/LoginHUD/WBP_LoginMenu.WBP_LoginMenu_C" self))
      (Variables|Default|SetLoginMenu _returnvalue)))
  (Input|SetInputModeUIOnly self (Variables|Default|GetLoginMenu) "DoNotLock")
  (UserInterface|Viewport|AddtoViewport (Variables|Default|GetLoginMenu) 0)
  (Default|EInitializeLoginMenu (Variables|Default|GetLoginMenu)))

(event EventIShowServerList
  ;[1 1 1] ServerListを表示する
  (Utilities|IsValid (Variables|Default|GetServerList)
    (:Is%20Valid
      _)
    (:Is%20Not%20Valid
      (bind _returnvalue (UserInterface|CreateWidget "/Game/Workspace/IoriFUKUNAKA/Blueprints/HeadUpDisplays/LoginHUD/WBP_ServerList.WBP_ServerList_C" self))
      (Variables|Default|SetServerList _returnvalue)))
  (Input|SetInputModeUIOnly self (Variables|Default|GetServerList) "DoNotLock")
  (UserInterface|Viewport|AddtoViewport (Variables|Default|GetServerList) 0))

(event EventIRemoveServerList
  ;[1 1 1] ServerListを非表示にする
  (Widget|RemovefromParent (Variables|Default|GetServerList)))

(event EventIRemoveLoginMenu
  ;[1 1 1] LoginMenuを非表示にする
  (Widget|RemovefromParent (Variables|Default|GetLoginMenu)))

(fn ConstructionScript)