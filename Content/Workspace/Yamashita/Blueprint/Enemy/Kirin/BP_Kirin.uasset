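; Kirin boss enemy, a lightning-themed creature with melee, rush, jump, area and thunder attacks.
; Interface events play montages, camera shake and sound, relay timing to the active task, and use server/multicast events for replication; overlap hit shapes follow the attack tag.
; The gimmick attack spawns a center object plus a ring around world origin; breaking enough crystals stuns Kirin and clears enemy objects.
; Timeline-driven sine offsets on the mesh fake jump arcs.
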(event Custom|MC_SpawnAfterImage
  ;[1 1 1] 残像を生成
  (Game|SpawnActorfromClass "/Game/Workspace/Yamashita/Blueprint/Enemy/Kirin/Object/BP_RushAfterImage.BP_RushAfterImage_C" (Transformation|GetActorTransform) "Undefined" self 0))

(event Custom|MC_SetBrokedCristalNum
  (params (BrokedCristalNum :type Integer))
  ;[1 1 1] 避雷針
  (Variables|Default|SetBrokedCristalNum BrokedCristalNum))

(event Custom|RoS_AddBrokedristalNum
  (params (BrokedCristalNum :type Integer))
  ;[1 1 1] 避雷針
  (CallFunction|MCSetBrokedCristalNum BrokedCristalNum))

(event Custom|RoS_SpawnIndiscriminateCollision
  (params (SpawnTransform :type Transform))
  ;[1 1 1] 無差別範囲攻撃コリジョン生成
  (Game|SpawnActorfromClass "/Game/Workspace/Yamashita/Blueprint/Enemy/Kirin/Object/BP_IndiscriminateCollision.BP_IndiscriminateCollision_C" SpawnTransform "Undefined" self 0.0 0))

(event Custom|MC_StopMovement
  (bind _self self)
  (bind _returnvalue (AI|GetAIController _self))
  ;[1 1 1] 移動を止める
  (Utilities|IsValid _returnvalue
    (:Is%20Valid
      (AI|Navigation|StopMovement _returnvalue))))

(event Custom|E_BreadCristal
  (bind _mesh (Variables|Character|GetMesh))
  (bind _returnvalue (Components|SkeletalMesh|GetAnimInstance _mesh))
  ;[1 1 1] 避雷針
  (if (== (+ (Variables|Default|GetBrokedCristalNum) 1) (Variables|編集可|GetGimickNum))
    (CallFunction|MCSetTag "(TagName=\"Enemy.Stan\")")
    (Animation|Montage|MontageStop _returnvalue 0.0 (Animation|Montage|GetCurrentActiveMontage _returnvalue))
    (bind _outactors (Actor|GetAllActorsOfClass "/Game/Workspace/Yamashita/Blueprint/Base/BP_EnemyObjectBase.BP_EnemyObjectBase_C"))
    (for _array_element _outactors
      (Actor|DestroyActor _array_element)))
  (CallFunction|RoSAddBrokedristalNum (+ (Variables|Default|GetBrokedCristalNum) 1)))

(event Custom|E_ResetBrokenCristalNum
  ;[1 1 1] 避雷針
  (CallFunction|RoSAddBrokedristalNum))

(event Custom|MC_MeshJump
  (params (Height :type Float%20%28single-precision%29) (time :type Float%20%28single-precision%29))
  ;[1 1 1] ジャンプイベント
  (CallFunction|MCSetElapsed (+ (Variables|Default|Getelapsed) (Utilities|Time|GetWorldDeltaSeconds)))
  (Transformation|SetRelativeLocation (Variables|Character|GetMesh) (Math|Vector|MakeVector 0.0 0.0 (+ (* Height (Math|Trig|Sin(Radians) (* (Variables|Default|Getelapsed) (/ (Math|Trig|GetPI) time)))) -376.0)) false false))

(event Custom|MC_RushFinish_Kirin
  (params (ターゲット :type Object%20Object%20Reference))
  ;[1 0 0.9549] 使ってない
  ;;[1 1 1] 突進終了
  (bind _outactors (Actor|GetAllActorsOfClass "/Game/Workspace/Yamashita/Blueprint/Enemy/Kirin/Object/BP_RushCollision.BP_RushCollision_C"))
  (for _array_element _outactors
    (Class|BPIEnemy|IRushFinishKirin(Message) _array_element)))

(event Custom|RoS_SpawnRushCollision
  (params (StartLoc :type Vector) (TargetLoc :type Vector))
  ;[1 0 0.9549] 使ってない
  ;;[1 1 1] 突進攻撃（スキル強化後）
  (Game|SpawnActorfromClass "/Game/Workspace/Yamashita/Blueprint/Enemy/Kirin/Object/BP_RushCollision.BP_RushCollision_C" (Math|Conversions|ToTransform(Vector) StartLoc) "Undefined" self StartLoc TargetLoc 0.0 0))

(event Custom|MC_SetElapsed
  (params (elapsed :type Float%20%28single-precision%29))
  ;[1 1 1] ジャンプイベント
  (Variables|Default|Setelapsed elapsed))

(event Custom|MC_SetIsWalkWait
  (params (isWalkWait :type Boolean))
  ;[1 0 0.9549] 使ってない
  ;;[1 1 1] 歩く待機か
  (Class|BPIEnemy|ISetIsWalkWait(Message) (Components|SkeletalMesh|GetAnimInstance (Variables|Character|GetMesh)) isWalkWait))

(event Custom|Ros_StopMontage
  ;[1 1 1] 回転
  (CallFunction|MCStopMontage))

(event Custom|MC_StopMontage
  (bind _mesh (Variables|Character|GetMesh))
  (bind _returnvalue (Components|SkeletalMesh|GetAnimInstance _mesh))
  ;[1 1 1] 回転
  (Animation|Montage|MontageStop _returnvalue 0.5 (Animation|Montage|GetCurrentActiveMontage _returnvalue)))

(event Custom|MC_SpawnGimick
  (bind _returnvalue (Transformation|GetActorTransform))
  (bind _self self)
  ;[1 1 1] ギミック攻撃
  (bind _returnvalue_2 (Game|SpawnActorfromClass "/Game/Workspace/Yamashita/Blueprint/Enemy/Kirin/Object/BP_GimickObj_Kirin.BP_GimickObj_Kirin_C" (Math|Transform|MakeTransform (Math|Vector|MakeVector (.x (.location _returnvalue)) (.y (.location _returnvalue)) 1e+01) "0, 0, 0" "1,1,1") "Undefined" _self 0.0 _self))
  (Default|RoSSetInit _returnvalue_2 1.08e+03 (Variables|編集可|GetTimeForGimickActivate) true)
  (GimickAttack|FSpawnGimick (Variables|編集可|GetGimickNum) (Variables|編集可|GetTimeForGimickActivate)))

(event Custom|RoS_SetCustomTimeDilation
  (params (Custom%20Time%20Dilation :type Float%20%28single-precision%29))
  ;[1 1 1] あとすき
  (CallFunction|MCSetCustomTimeDilation Custom%20Time%20Dilation))

(event Custom|MC_SetCustomTimeDilation
  (params (Custom%20Time%20Dilation :type Float%20%28single-precision%29))
  ;[1 1 1] あとすき
  (Variables|Default|SetCustomTimeDilation Custom%20Time%20Dilation))

(event Custom|E_OnDamagemotionPlay
  (Utilities|FlowControl|Sequence
    (:then_0
      ;[1 1 1] ジャンプ攻撃
      (Timeline|タイムライン_0 Stop
        (:Update
          (CallFunction|MCMeshJump 6.5e+02 1.0))))
    (:then_1
      (Timeline|タイムライン_1 Stop
        (:Update
          (CallFunction|MCMeshJump (stale EventISimpleJump height) (stale EventISimpleJump time)))))))

(event Custom|MC_SetMeshLocation
  (params (NewLocation :type Vector))
  ;[1 1 1] メッシュ移動
  (Transformation|SetRelativeLocation (Variables|Character|GetMesh) NewLocation false false)
  (Networking|SwitchHasAuthority))

(event EventINormalAttackKirin
  ;[1 1 1] 通常攻撃　通知
  (CallFunction|EPlayMontage "/Game/Workspace/Yamashita/Animation/Kirin/Montage/NormalAttack/ForwardAttack/AM_Kirin_NormalAttack.AM_Kirin_NormalAttack" 1.0))

(event EventIIndiscriminateAttackKirin
  ;[1 1 1] 無差別範囲攻撃　通知
  (CallFunction|EPlayMontage "/Game/Workspace/Yamashita/Animation/Kirin/Montage/AM_Kirin_Indiscriminate.AM_Kirin_Indiscriminate" 1.5))

(event EventISpawnAfterImageKirin
  ;[1 1 1] 直進突進攻撃
  (CallFunction|MCSpawnAfterImage))

(event EventITurnEnd
  ;[1 1 1] 回転
  (CallFunction|RosStopMontage))

(event EventITurnStart
  (params (isLeft? :type Boolean) (Facing? :type Boolean) (PlayRate :type Float%20%28single-precision%29))
  ;[1 1 1] 回転
  (if Facing?
    (CallFunction|EPlayMontage (select isLeft? "/Game/Workspace/Yamashita/Animation/Kirin/Montage/Turn/AM_Kirin_BackMove_Left.AM_Kirin_BackMove_Left" "/Game/Workspace/Yamashita/Animation/Kirin/Montage/Turn/AM_Kirin_BackMove_Right.AM_Kirin_BackMove_Right") PlayRate)
    (else
      (CallFunction|EPlayMontage (select isLeft? "/Game/Workspace/Yamashita/Animation/Kirin/Montage/Turn/AM_Kirin_BackMove_Left.AM_Kirin_BackMove_Left" "/Game/Workspace/Yamashita/Animation/Kirin/Montage/Turn/AM_Kirin_BackMove_Right.AM_Kirin_BackMove_Right") PlayRate))))

(event EventILineRushStart
  ;[1 1 1] 直進突進攻撃
  (Class|BPIEnemy|ILineRushStart(Message) (Variables|Default|GetTask)))

(event EventIGimickAttackCollision
  ;[1 1 1] ギミック攻撃　雷が落ちる
  (Game|Feedback|ClientStartCameraShake (Game|GetPlayerController 0) "/Game/Workspace/Yamashita/Blueprint/CameraShake/BP_EnemyCameraShake.BP_EnemyCameraShake_C" 3.0 "CameraLocal" "0, 0, 0")
  (Game|Feedback|ClientPlayForceFeedback (Game|GetPlayerController 0) "/Game/Workspace/Yamashita/Blueprint/ForceBack/ForceFeedbackEffect_GimickAttack.ForceFeedbackEffect_GimickAttack" "None" false false false))

(event EventIBackAttackKirin
  (params (isLong :type Boolean))
  ;[1 1 1] 後ろ蹴り攻撃　通知
  (CallFunction|EPlayMontage (select isLong "/Game/Workspace/Yamashita/Animation/Kirin/Montage/NormalAttack/BackAttack/AM_Kirin_BackAttack.AM_Kirin_BackAttack" "/Game/Workspace/Yamashita/Animation/Kirin/Montage/NormalAttack/BackAttack/AM_Kirin_BackAttack_Second.AM_Kirin_BackAttack_Second") 1.0))

(event EventILineRushKirin
  (params (Preparation :type Boolean))
  ;[1 1 1] 直進突進攻撃
  (if Preparation
    (CallFunction|EPlayMontage "/Game/Workspace/Yamashita/Animation/Kirin/Montage/LineRush/AM_Kirin_Crouching.AM_Kirin_Crouching" 1.0)
    (else
      (CallFunction|EPlayMontage "/Game/Workspace/Yamashita/Animation/Kirin/Montage/AM_Kirin_RushStop.AM_Kirin_RushStop" 1.4))))

(event EventISlashingAttackKirin
  ;[1 1 1] 斬撃攻撃
  (CallFunction|EPlayMontage "/Game/Workspace/Yamashita/Animation/Kirin/Montage/SlashingAttack/AM_SlashingAttack.AM_SlashingAttack" 1.5))

(event EventISlashingAttackSpawnWall
  ;[1 1 1] 斬撃攻撃
  (Class|BPIEnemy|ISlashingAttackSpawnWall(Message) (Variables|Default|GetTask)))

(event EventISlashingAttackSlash
  ;[1 1 1] 斬撃攻撃
  (Class|BPIEnemy|ISlashingAttackSlash(Message) (Variables|Default|GetTask))
  (Game|Feedback|ClientStartCameraShake (Game|GetPlayerController 0) "/Game/Workspace/Yamashita/Blueprint/CameraShake/BP_EnemyCameraShake.BP_EnemyCameraShake_C" 1.0 "CameraLocal" "0, 0, 0")
  (Game|Feedback|ClientPlayForceFeedback (Game|GetPlayerController 0) "/Game/Workspace/Yamashita/Blueprint/ForceBack/ForceFeedbackEffect_Indiscriminate.ForceFeedbackEffect_Indiscriminate" "None" false false false))

(event EventIRangeAttackKirin
  ;[1 1 1] 範囲攻撃
  (CallFunction|EPlayMontage "/Game/Workspace/Yamashita/Animation/Kirin/Montage/AM_Kirin_RangeAttack.AM_Kirin_RangeAttack" 1.2))

(event EventISetEnemyCustomDiration
  (params (diration :type Float%20%28single-precision%29))
  ;[1 1 1] カスタムデュレーションを設定
  (CallFunction|RoSSetCustomTimeDilation diration))

(event EventIJumpTakeOff
  ;[1 1 1] 斬撃攻撃
  ;;[1 1 1] ジャンプ
  (Class|BPIEnemy|IJumpTakeOff(Message) (Variables|Default|GetTask)))

(event EventIJumpMove
  (params (Rate :type Float%20%28single-precision%29) (TargetPoint :type Vector :default "0, 0, 0"))
  ;[1 1 1] 斬撃攻撃
  ;;[1 1 1] ジャンプ
  (Utilities|MJump TargetPoint))

(event EventIThunderBoltKirin
  ;[1 1 1] サンダーボルト
  (CallFunction|EPlayMontage "/Game/Workspace/Yamashita/Animation/Kirin/Montage/ThunderBolt/AM_Kirin_ThunderBolt.AM_Kirin_ThunderBolt" 1.0)
  (Utilities|FlowControl|Delay (- (Variables|編集可|GetTimeForFallThunderBolt) (Math|Float|MakeLiteralFloat 3.5)))
  (CallFunction|MCMontageJump "/Game/Workspace/Yamashita/Animation/Kirin/Montage/ThunderBolt/AM_Kirin_ThunderBolt.AM_Kirin_ThunderBolt" "LoopEnd"))

(event EventISimpleJump
  (params (isLanding :type Boolean) (height :type Float%20%28single-precision%29) (time :type Float%20%28single-precision%29) (gap :type Boolean))
  (if isLanding
    (CallFunction|EPlayMontage (select gap "/Game/Workspace/Yamashita/Animation/Kirin/Montage/Gimick/AM_Kirin_JumpLand_Gimick.AM_Kirin_JumpLand_Gimick" "/Game/Workspace/Yamashita/Animation/Kirin/Montage/Jump/AM_TakedistanceLanding.AM_TakedistanceLanding") 1.0) ; 着地
    (Transformation|SetRelativeLocation (Variables|Character|GetMesh) "0,0.000000,-376.000000" false false)
    (Timeline|タイムライン_1 Stop
      (:Update
        (CallFunction|MCMeshJump height time)))
    (else
      (CallFunction|EPlayMontage "/Game/Workspace/Yamashita/Animation/Kirin/Montage/Jump/AM_Kirin_JumpStart.AM_Kirin_JumpStart" 1.0) ; start
      (CallFunction|MCSetElapsed 0.0)
      (Timeline|タイムライン_1 PlayFromStart))))

(event EventIAttackStart
  (params (isNormalAttack? :type Boolean))
  ;[1 1 1] 攻撃開始
  (|CallParentFunction isNormalAttack?)
  (CallFunction|EResetBrokenCristalNum))

(event EventICallThunderKirin
  ;[1 1 1] CallThunder
  (CallFunction|EPlayMontage "/Game/Workspace/Yamashita/Animation/Kirin/Montage/CallThunder/AM_Kirin_CallThunder.AM_Kirin_CallThunder" 1.0))

(event EventICallThunderTiming
  ;[1 1 1] CallThunder
  (Class|BPIEnemy|ICallThunderTiming(Message) (Variables|Default|GetTask))
  (Game|Feedback|ClientStartCameraShake (Game|GetPlayerController 0) "/Game/Workspace/Yamashita/Blueprint/CameraShake/BP_EnemyCameraShake.BP_EnemyCameraShake_C" 1.0 "CameraLocal" "0, 0, 0"))

(event EventIJumpAttackKirin
  (params (landing :type Boolean))
  ;[1 1 1] ジャンプ攻撃
  (if landing
    (CallFunction|EPlayMontage "/Game/Workspace/Yamashita/Animation/Kirin/Montage/Jump/AM_Kirin_JumpLand.AM_Kirin_JumpLand" 1.0)
    (Transformation|SetRelativeLocation (Variables|Character|GetMesh) "0, 0,-376.000000" false false)
    (Timeline|タイムライン_0 Stop
      (:Update
        (CallFunction|MCMeshJump 6.5e+02 1.0)))
    (else
      (CallFunction|EPlayMontage "/Game/Workspace/Yamashita/Animation/Kirin/Montage/Jump/AM_Kirin_JumpStart.AM_Kirin_JumpStart" 1.0)
      (CallFunction|MCSetElapsed 0.0)
      (Timeline|タイムライン_0 PlayFromStart))))

(event EventITakeDistance
  (params (landing :type Boolean))
  ;[1 1 1] 距離をとるタスク
  (if landing
    (CallFunction|EPlayMontage "/Game/Workspace/Yamashita/Animation/Kirin/Montage/Jump/AM_Kirin_JumpEnd.AM_Kirin_JumpEnd" 1.0)
    (else
      (CallFunction|EPlayMontage "/Game/Workspace/Yamashita/Animation/Kirin/Montage/Jump/AM_Kirin_JumpStart.AM_Kirin_JumpStart" 1.0))))

(event EventIRushAttackKirin
  (params (startLoc :type Vector :default "0, 0, 0") (targetLoc :type Vector :default "0, 0, 0"))
  ;[1 0 0.9549] 使ってない
  ;;[1 1 1] 突進攻撃（スキル強化後）
  (CallFunction|EPlayMontage "/Game/Workspace/Yamashita/Animation/Kirin/Montage/AM_Kirin_Run.AM_Kirin_Run" 1.0)
  (if (Utilities|Enum|Equal(Enum) (Variables|Default|GetHealthState) "NewEnumerator1")
    (CallFunction|RoSSpawnRushCollision startLoc targetLoc)))

(event EventIThunderBoltTiming
  ;[1 1 1] サンダーボルト
  (Game|Feedback|ClientStartCameraShake (Game|GetPlayerController 0) "/Game/Workspace/Yamashita/Blueprint/CameraShake/BP_EnemyCameraShake.BP_EnemyCameraShake_C" 1.0 "CameraLocal" "0, 0, 0"))

(event EventIMotionStop
  ;[1 1 1] あとすき
  (CallFunction|RoSSetCustomTimeDilation 0.1)
  (bind _damage (Class|BPIEnemy|IGetAttackStatus(Message) self (Variables|Default|GetAttackState)))
  (Utilities|FlowControl|Delay (.WaitTime (Utilities|Struct|BreakST_EnemyAttack _damage)))
  (CallFunction|RoSSetCustomTimeDilation 1.0))

(event EventISetMeshLocation
  (params (loc :type Vector :default "0, 0, 0"))
  ;[1 1 1] メッシュ移動
  (CallFunction|MCSetMeshLocation loc))

(event EventIEnemyStan
  ;[1 1 1] スタン
  (CallFunction|EPlayMontage (select (Math|Random|RandomBool) "/Game/Workspace/Yamashita/Animation/Kirin/Montage/Damage/AM_Kirin_Damage_Right.AM_Kirin_Damage_Right" "/Game/Workspace/Yamashita/Animation/Kirin/Montage/Damage/AM_Kirin_Damage_Left.AM_Kirin_Damage_Left") 1.0))

(event EventIStanFinish
  ;[1 1 1] スタン
  (Class|BPIEnemy|IStanFinish(Message) (Variables|Default|GetTask)))

(event EventISideAttackKirin
  ;[1 1 1] 横振り攻撃
  (CallFunction|EPlayMontage "/Game/Workspace/Yamashita/Animation/Kirin/Montage/SideAttack/AM_SeriesAttack.AM_SeriesAttack" 0.8))

(event EventIThunderWeatherAnim
  (CallFunction|EPlayMontage "/Game/Workspace/Yamashita/Animation/Kirin/Montage/AM_ThunderWeather.AM_ThunderWeather" 1.0))

(event EventIHiraishinTiming
  ;[1 1 1] ギミック攻撃
  (CallFunction|MCSpawnGimick)
  (Utilities|FlowControl|Delay (CallFunction|FGetNextSection (- (Variables|編集可|GetTimeForGimickActivate) 0.15)))
  (CallFunction|MCMontageJump "/Game/Workspace/Yamashita/Animation/Kirin/Montage/AM_GimickAttack.AM_GimickAttack" "LoopEnd"))

(event EventIRushFinishKirin
  ;[1 0 0.9549] 使ってない
  ;;[1 1 1] 突進終了
  (CallFunction|MCRushFinishKirin))

(event EventISetIsWalkWait
  (params (isWalkWait :type Boolean))
  ;[1 0 0.9549] 使ってない
  ;;[1 1 1] 歩く待機か
  (CallFunction|MCSetIsWalkWait isWalkWait))

(event EventIDead
  ;[1 1 1] 死ぬ
  (CallFunction|EPlayMontage "/Game/Workspace/Yamashita/Animation/Kirin/Montage/AM_Kirin_Dead.AM_Kirin_Dead" 1.0))

(event EventIGimickAttackKirin
  ;[1 1 1] ギミック攻撃
  (Game|Feedback|ClientStartCameraShake (Game|GetPlayerController 0) "/Game/Workspace/Yamashita/Blueprint/CameraShake/BP_EnemyCameraShake.BP_EnemyCameraShake_C" 0.5 "CameraLocal" "0, 0, 0")
  (CallFunction|EPlayMontage "/Game/Workspace/Yamashita/Animation/Kirin/Montage/AM_GimickAttack.AM_GimickAttack" 1.0))

(event EventISpawnRangeAttack
  ;[1 1 1] 範囲攻撃
  (Game|Feedback|ClientStartCameraShake (Game|GetPlayerController 0) "/Game/Workspace/Yamashita/Blueprint/CameraShake/BP_EnemyCameraShake.BP_EnemyCameraShake_C" 1.0 "CameraLocal" "0, 0, 0")
  (CallFunction|EPlaySE "/Game/Workspace/Yamashita/SoundQue/Enemy/SQ_Hanni_Cue.SQ_Hanni_Cue" (Transformation|GetActorLocation) 0 2.0))

(event EventISpawnIndiscriminateColl
  ;[1 1 1] 無差別範囲攻撃　通知
  (Game|Feedback|ClientStartCameraShake (Game|GetPlayerController 0) "/Game/Workspace/Yamashita/Blueprint/CameraShake/BP_EnemyCameraShake.BP_EnemyCameraShake_C" 1.0 "CameraLocal" "0, 0, 0")
  (Game|Feedback|ClientPlayForceFeedback (Game|GetPlayerController 0) "/Game/Workspace/Yamashita/Blueprint/ForceBack/ForceFeedbackEffect_Indiscriminate.ForceFeedbackEffect_Indiscriminate" "None" false false false)
  (CallFunction|EPlaySE "/Game/Workspace/Yamashita/SoundQue/Enemy/SQ_EnemySkill.SQ_EnemySkill" (Transformation|GetActorLocation) 0 1.0)
  (Utilities|FlowControl|Delay 0.5)
  (Class|BPIEnemy|ISpawnIndiscriminateColl(Message) (Variables|Default|GetTask))
  (CallFunction|EPlaySE "/Game/Workspace/Yamashita/SoundQue/Enemy/SQ_Indiscriminate00.SQ_Indiscriminate00" (Transformation|GetActorLocation) 0 1.0))

(fn ConstructionScript
  (|CallParentFunction))

(fn FOverrideCollision
  (|CallParentFunction)
  (|SwitchGameplayTag (Variables|Default|GetAttackState)
    (:Enemy.Attack.Kirin.NormalAttack
      (CallFunction|FSphereOverlap (Transformation|GetSocketLocation (Variables|Character|GetMesh) "Head") (Variables|編集可|GetAttackRange_NormalAttack) true true 1))
    (:Enemy.Attack.Kirin.RushAttack
      (CallFunction|FBoxOverlap (Transformation|GetActorLocation) "350.000000,250.000000,350.000000" false true 3))
    (:Enemy.Attack.Kirin.BackAttack
      (CallFunction|FSphereOverlap (+ (Transformation|GetSocketLocation (Variables|Character|GetMesh) "Right_Foreleg") (* (Transformation|GetActorRightVector) 2.0)) (Variables|編集可|GetAttackRange_BackAttack) true true 1))
    (:Enemy.Attack.Kirin.SideAttack
      (CallFunction|FSphereOverlap (Transformation|GetSocketLocation (Variables|Character|GetMesh) "Head") (Variables|編集可|GetAttackRange_NormalAttack) true true 1))))

(fn IGetHateStageBorder
  (params (Stage :type En_EnemyStageState%20Enum :default "NewEnumerator7"))
  (for (_array_element _array_index) (Variables|編集可|GetHateStage)
    (if (Utilities|Enum|Equal(Enum) (.stage (Utilities|Struct|BreakST_HateStage _array_element)) Stage)
      (return (.hate (Utilities|Struct|BreakST_HateStage _array_element)) (== _array_index (Utilities|Array|LastIndex (Variables|編集可|GetHateStage))))))
  (return 0.0 false))

(fn FWrapAngle0to360
  (params (A :type Float%20%28single-precision%29))
  (bind _returnvalue (Math|Float|%(Float) A 3.6e+02))
  (return (Math|Float|SelectFloat (+ _returnvalue 3.6e+02) _returnvalue (< _returnvalue 0.0))))

(fn FFindEnemyAroundLocation
  (params (InInt :type Integer) (CurrentTargetDegree :type Float%20%28single-precision%29))
  (bind _returnvalue (Math|Vector|MakeVector 0.0 0.0 0.0))
  (bind _attackrange_gimickattack (Variables|編集可|GetAttackRange_GimickAttack))
  (bind _returnvalue_2 (Math|Float|MakeLiteralFloat _attackrange_gimickattack))
  (LocalVariables|SetNowTargetDegree CurrentTargetDegree)
  (return (Math|Vector|MakeVector (+ (* (Math|Trig|Cos(Degrees) (LocalVariables|GetNowTargetDegree)) _returnvalue_2) (.x _returnvalue)) (+ (* (Math|Trig|Sin(Degrees) (LocalVariables|GetNowTargetDegree)) _returnvalue_2) (.y _returnvalue)) (- (.z _returnvalue) 2e+02)) (GimickAttack|FWrapAngle0to360 (+ (Math|Float|MakeLiteralFloat (/ 3.6e+02 (Math|Conversions|ToFloat(Integer) InInt))) (LocalVariables|GetNowTargetDegree)))))

(fn FSpawnGimick
  (params (AppearNum :type Integer) (AttackDelay :type Float%20%28single-precision%29))
  (bind _self self)
  (LocalVariables|SetTargetDegree 0.0)
  (for _index (range 0 (- AppearNum 1))
    (bind (_targetloc _calcedtargetdegree) (GimickAttack|FFindEnemyAroundLocation AppearNum (LocalVariables|GetTargetDegree)))
    (LocalVariables|SetTargetDegree _calcedtargetdegree)
    (bind _returnvalue (Game|SpawnActorfromClass "/Game/Workspace/Yamashita/Blueprint/Enemy/Kirin/Object/BP_GimickObj_Kirin.BP_GimickObj_Kirin_C" (Math|Conversions|ToTransform(Vector) (Math|Vector|MakeVector (.X (Math|Vector|BreakVector _targetloc)) (.Y (Math|Vector|BreakVector _targetloc)) 0.0)) "Undefined" _self 0.0 _self))
    (Default|RoSSetInit _returnvalue (Variables|編集可|GetGimickAttackRange) AttackDelay false)))

(fn FGetNextSection
  (params (AttackDelay :type Float%20%28single-precision%29))
  (return (- AttackDelay (Math|Float|MakeLiteralFloat 3.45))))

(fn FDead
  (|CallParentFunction)
  (Rendering|SetVisibility (Variables|Default|GetNS_kirin_autra) false true))

(fn IGetTimeforFallThunderBolt
  (return (Variables|編集可|GetTimeForFallThunderBolt)))

(fn IGetRadiusOfThunderBolt
  (return (Variables|編集可|GetRadiusOfThunderBolt)))

(fn FGotDeathblow
  (params (fromLoc :type Vector :default "0, 0, 0"))
  (|CallParentFunction fromLoc)
  (LocalVariables|Setfrom fromLoc)
  (CallFunction|MCStopMovement)
  (CallFunction|MCSetTag "(TagName=\"Enemy.Damage\")")
  (CallFunction|EPlayMontage (select (> (Class|KismetMathLibrary|CrossProduct2D (Math|Conversions|ToVector2D(Vector) (Transformation|GetActorForwardVector)) (Math|Vector2D|Normalize2D (Math|Conversions|ToVector2D(Vector) (- (LocalVariables|Getfrom) (Transformation|GetActorLocation))))) 0.0) "/Game/Workspace/Yamashita/Animation/Kirin/Montage/Damage/AM_Kirin_Damage_Right.AM_Kirin_Damage_Right" "/Game/Workspace/Yamashita/Animation/Kirin/Montage/Damage/AM_Kirin_Damage_Left.AM_Kirin_Damage_Left") 1.0)
  (CallFunction|EClearEnemyObject))

(fn IGetJumpAttackRange
  (return (Variables|編集可|GetRadius_JumpAttack)))

(fn IGetCallThunderParam
  (return (Variables|編集可|GetAttackRadius_CallThunder) (Variables|編集可|GetAttackDelay_CallThunder)))

(fn IGetRangeAttackParam
  (return (Variables|編集可|GetRadius_RangeAttack) 0.0))

(fn FStopJump
  (|CallParentFunction)
  (CallFunction|EonDamagemotionPlay))

(fn IGetTurnSpeed
  (return (Variables|編集可|GetTurnSpeed_Face) (Variables|編集可|GetTurnSpeed_Back) (Variables|編集可|GetTurnSpeed_GimickJump)))