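; BP_JufuImagePop is a short-lived pop-up actor that shows a Jufu (talisman) image in the world.
; The construction script creates a dynamic instance of M_JufuImage, sets the JufuImage texture on it and applies it to the Jufu component.
; A timeline started on BeginPlay drives the component's relative position and material alpha, then destroys the actor.
; Tick billboards the whole actor toward the player camera.
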(event EventBeginPlay
  ;[1 1 1] 初期化処理
  (bind (_direction _position _alpha) (Timeline|JufuAnimation Play)
    (:Update
      (Transformation|SetRelativeLocation (Variables|Default|GetJufu) (Math|Vector|MakeVector 0.0 0.0 _position) false false)
      (Rendering|Material|SetScalarParameterValue (Variables|Default|GetMI_JufuImage) "Alpha" _alpha :!class /Script/Engine.MaterialInstanceDynamic))
    (:Finished
      (Actor|DestroyActor))))

(event EventTick
  (params (DeltaSeconds :type Float%20%28single-precision%29))
  ;[1 1 1] ビルボード処理
  (Transformation|SetActorRotation (Math|Rotator|FindLookatRotation (Transformation|GetActorLocation) (Camera|GetCameraLocation (Game|GetPlayerCameraManager 0)))))

(fn ConstructionScript
  (bind _returnvalue (Rendering|Material|CreateDynamicMaterialInstance (Variables|Default|GetJufu) 0 "/Game/Workspace/IoriFUKUNAKA/Materials/UserInterface/M_JufuImage.M_JufuImage" "None" :!class /Script/Engine.PrimitiveComponent))
  (bind _output_get (Variables|Default|SetMI_JufuImage _returnvalue))
  (Rendering|Material|SetTextureParameterValue _output_get "MainTexture" (Variables|Default|GetJufuImage))
  (Rendering|Material|SetMaterial (Variables|Default|GetJufu) 0 _output_get))