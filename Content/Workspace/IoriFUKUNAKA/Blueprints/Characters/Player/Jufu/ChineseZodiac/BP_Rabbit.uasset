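; Rabbit Chinese zodiac jufu that performs a one-shot heal on all players when initialized.
; Extends its parent's initialization, reading the instigator's Attack via a player status interface and multiplying it by a BPC_BuffManager buff value and HealMag.
; Sends each pawn in the GameState PlayerArray that amount, randomized by about ±10% per player, through a heal interface message, then destroys itself.
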(fn ConstructionScript
  (|CallParentFunction))

(fn FInitialize
  (|CallParentFunction)
  (bind _instigator (Variables|Default|GetInstigator)
    (:then
      (bind _attack (Class|BPIControlPlayerInfo|IGetPlayerDefaultStatus(Message) _instigator))
      (Utilities|IsValid (Actor|GetComponentbyClass _instigator "/Game/Workspace/IoriFUKUNAKA/Blueprints/Characters/BPC_BuffManager.BPC_BuffManager_C")
        (:Is%20Valid
          (for _array_element (Variables|/Script/Engine.GameStateBase|GetPlayerArray (Game|GetGameState))
            (Class|BPIControlPlayerInfo|IHealPlayer(Message) (Variables|/Script/Engine.PlayerState|GetPawnPrivate _array_element) (Math|Float|Truncate (* (* _attack (Default|FGetBuffValue (Actor|GetComponentbyClass _instigator "/Game/Workspace/IoriFUKUNAKA/Blueprints/Characters/BPC_BuffManager.BPC_BuffManager_C") "NewEnumerator0") (Variables|Default|GetHealMag)) (Math|Random|RandomFloatinRange 0.9 1.1))) false))
          (Actor|DestroyActor))))
    (:else)))