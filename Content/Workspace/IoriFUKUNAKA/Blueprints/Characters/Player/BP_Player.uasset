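; Player character Blueprint for networked action combat: movement, montage combo attacks, dodge, gauge-based special attack and four cast-time skills.
; Interface events drive actions gated by CanAction/CanMove, and most replicate animation, rotation and hits through run-on-server to multicast event pairs.
; Weapon overlaps trigger hit stop, camera shake, damage and enemy hate.
; Tick regenerates energy, advances casting with movement cancel, updates skill holder components and prints debug state.
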(event OnComponentBeginOverlap(WeaponCol)
  (params (OverlappedComponent :type Primitive%20Component%20Object%20Reference) (OtherActor :type Actor%20Object%20Reference) (OtherComp :type Primitive%20Component%20Object%20Reference) (OtherBodyIndex :type Integer) (bFromSweep :type Boolean) (SweepResult :type Hit%20Result%20Structure%20%28by%20ref%29))
  ;[1 1 1] 通常攻撃
  ;;[1 1 1] 攻撃の当たり判定
  (if (Actor|ActorHasTag OtherActor "Enemy")
    (攻撃|FWeaponColSwitch false)
    ;;;[1 0 0.01665] めっちゃ仮処理
    (Variables|必殺技|SetCurrentSpecial (+ 1.0 (Variables|必殺技|GetCurrentSpecial)))
    (Game|Feedback|ClientStartCameraShake (Game|GetPlayerController 0) "/Game/Workspace/IoriFUKUNAKA/Blueprints/System/BP_HitCamShake.BP_HitCamShake_C" 2.0 "CameraLocal" "0, 0, 0")
    (CallFunction|ROSHit 3 OtherActor)))

(event Custom|E_PlayComboAction
  (bind _returnvalue (Pawn|GetControlRotation :!class /Script/Engine.Pawn))
  ;[1 1 1] 通常攻撃
  ;;[1 1 1] 攻撃処理
  (if (> (Utilities|Array|Length (Variables|攻撃|GetComboAMs)) 0)
    (攻撃|FWeaponColSwitch false)
    (Utilities|MInputValid?
      (:true
        (CallFunction|RosSetActorRotation (Math|Rotator|FindLookatRotation (Math|Vector|MakeVector 0.0 0.0 0.0) (+ (* (Math|Vector|GetForwardVector (Math|Rotator|MakeRotator 0.0 0.0 (.yaw _returnvalue))) (Variables|移動|GetMoveForwardValue)) (* (Math|Vector|GetRightVector (Math|Rotator|MakeRotator 0.0 0.0 (.yaw _returnvalue))) (Variables|移動|GetMoveRightValue)))) false))
      (:false
        _))
    (CallFunction|ROSPlayAnimMontage 1.2 (Utilities|Array|Get(acopy) (Variables|攻撃|GetComboAMs) (Math|Integer|%(Integer) (Variables|攻撃|GetComboCounter) (Utilities|Array|Length (Variables|攻撃|GetComboAMs)))))
    (Math|Integer|IncrementInt (Variables|攻撃|GetComboCounter))))

(event Custom|E_CloseComboGate
  ;[1 1 1] 通常攻撃
  (Utilities|FlowControl|Gate true) ; enters at Close
)

(event Custom|ROS_ChangeIsCasting?
  (params (isCasting? :type Boolean))
  ;[1 1 1] スキル
  (CallFunction|MCChangeIsCasting? isCasting?))

(event Custom|MC_ChangeIsCasting?
  (params (IsCasting? :type Boolean))
  ;[1 1 1] スキル
  (Class|BPIPlayertoAnimation|IChangeIsCasting?(Message) (Components|SkeletalMesh|GetAnimInstance (Variables|Character|GetMesh)) IsCasting?))

(event Custom|ROS_PlaySpecialAttack
  ;[1 1 1] 必殺技
  (CallFunction|MCPlaySpecialAttack))

(event Custom|MC_PlaySpecialAttack
  ;[1 1 1] 必殺技
  (Animation|Montage|PlayMontage (Variables|Character|GetMesh) (Variables|必殺技|GetSpecialAM) 1.2
    (:OnCompleted
      (Variables|フラグ|SetCanAction? true)
      (Variables|フラグ|SetCanMove? true))))

(event Custom|E_CastingUpdate
  ;[1 1 1] スキル
  ;;[1 1 1] 詠唱処理
  (if (Variables|スキル|GetisCasting?)
    (if (>= (+ (Variables|スキル|GetCastingElapsed) (Utilities|Time|GetWorldDeltaSeconds)) (Variables|スキル|GetCastingTime))
      (Default|ESkillActivate (Variables|スキル|GetUseSkillHolder))
      (詠唱|FStopCasting)
      (CallFunction|ROSChangeIsCasting? false)
      (CallFunction|ROSPlayCastFinishAnim "/Game/Workspace/IoriFUKUNAKA/Animations/Player/AnimMontage/AM_CastFinish.AM_CastFinish")
      (else
        (Utilities|FlowControl|Sequence
          (:then_0
            (bind _output_get (Variables|スキル|SetCastingElapsed (+ (Variables|スキル|GetCastingElapsed) (Utilities|Time|GetWorldDeltaSeconds))))
            (Development|PrintString (Utilities|String|ToString(Float) _output_get) true true "(R=0.000000,G=1.000000,B=0.022421,A=1.000000)" 0.0))
          (:then_1
            ;;[1 1 1] 詠唱キャンセル処理
            (Utilities|MInputValid?
              (:true
                (if (Variables|スキル|GetCanSkillCancel?)
                  (詠唱|FStopCasting)
                  (Variables|フラグ|SetCanMove? true)
                  (CallFunction|ROSChangeIsCasting? false)))
              (:false
                (Variables|スキル|SetCanSkillCancel? true)))))))))

(event Custom|E_Initialize
  ;[1 1 1] 初期化処理
  (Variables|/Script/Engine.CharacterMovementComponent|SetMaxWalkSpeed (Variables|Character|GetCharacterMovement) (Variables|移動|GetMoveSpeed))
  (Variables|ステータス|SetCurrentHP (Variables|ステータス|GetMaxHP))
  (攻撃|FWeaponColSwitch false)
  (bind _asbp_player_controller (Utilities|Casting|CastToBP_PlayerController (Pawn|GetController)))
  (Default|EUpdateBattleScoreUI _asbp_player_controller))

(event Custom|ROS_PlayCastFinishAnim
  (params (CastFinishAnim :type Anim%20Montage%20Object%20Reference))
  ;[1 1 1] スキル
  (CallFunction|MCPlayCastFinishAnim CastFinishAnim))

(event Custom|MC_PlayCastFinishAnim
  (params (CastFinishAnim :type Anim%20Montage%20Object%20Reference))
  ;[1 1 1] スキル
  (Animation|Montage|PlayMontage (Variables|Character|GetMesh) CastFinishAnim
    (:OnCompleted
      (Variables|フラグ|SetCanMove? true))))

(event Custom|ROS_PlayAvoidAnim
  ;[1 1 1] 回避
  (CallFunction|MCPlayAvoidAnim))

(event Custom|MC_PlayAvoidAnim
  ;[1 1 1] 回避
  (Animation|Montage|PlayMontage (Variables|Character|GetMesh) (Variables|回避|GetAvoidAM)
    (:OnCompleted
      (Variables|フラグ|SetCanAction? true)
      (Variables|フラグ|SetCanMove? true))))

(event Custom|ROS_Hit
  (params (DelayFrame :type Integer) (OtherActor :type Object%20Object%20Reference))
  ;[1 1 1] 通常攻撃
  ;;[1 1 1] 攻撃の当たり判定
  (CallFunction|MCHit DelayFrame OtherActor)
  (bind _asbp_player_controller (Utilities|Casting|CastToBP_PlayerController (Components|GetOwner)))
  (Default|FAddHate (Variables|Default|GetFightingEnemyRef) _asbp_player_controller 5.0 false))

(event Custom|MC_Hit
  (params (DelayFrame :type Integer) (OtherActor :type Object%20Object%20Reference))
  ;[1 1 1] 通常攻撃
  ;;[1 1 1] 攻撃の当たり判定
  (Utilities|MHitStop DelayFrame)
  (Class|BPIHitBoxtoCharacter|IHitAttack(Message) OtherActor)
  (bind _aspawn (Utilities|Casting|CastToPawn OtherActor))
  (Game|Damage|ApplyDamage _aspawn 1e+01 (Pawn|GetController) self))

(event EventIMoveForward
  (params (Value :type Float%20%28single-precision%29))
  ;[1 1 1] 移動処理
  (bind _output_get (Variables|移動|SetMoveForwardValue Value))
  (if (Variables|フラグ|GetCanMove?)
    (移動|FMoveForward _output_get)))

(event EventIMoveRight
  (params (Value :type Float%20%28single-precision%29))
  ;[1 1 1] 移動処理
  (bind _output_get (Variables|移動|SetMoveRightValue Value))
  (if (Variables|フラグ|GetCanMove?)
    (移動|FMoveRight _output_get)))

(event EventIOpenComboGate
  ;[1 1 1] 通常攻撃
  (Utilities|FlowControl|Gate true) ; enters at Open
)

(event EventICloseComboGate
  ;[1 1 1] 通常攻撃
  (CallFunction|ECloseComboGate)
  (攻撃|FFinishCombo)
  (攻撃|FWeaponColSwitch false)
  (Variables|フラグ|SetCanMove? true))

(event EventIHitSpecial
  (params (HitActor :type Actor%20Object%20Reference))
  ;[1 1 1] 必殺技
  (if (and (Actor|ActorHasTag HitActor "Enemy") (!= HitActor self))
    (Class|BPIHitBoxtoCharacter|IHitAttack(Message) HitActor)
    (Game|Feedback|ClientStartCameraShake (Game|GetPlayerController 0) "/Game/Workspace/IoriFUKUNAKA/Blueprints/System/BP_HitCamShake.BP_HitCamShake_C" 2e+01 "CameraLocal" "0, 0, 0")
    (Utilities|MHitStop 8)))

(event EventINormalAttack
  ;[1 1 1] 通常攻撃
  (if (Variables|フラグ|GetCanAction?)
    (if (Variables|攻撃|GetisAttack?)
      (Utilities|FlowControl|Gate true
        (:Exit
          (CallFunction|EPlayComboAction)
          (CallFunction|ECloseComboGate)))
      (else
        (Variables|攻撃|SetisAttack? true)
        (Variables|フラグ|SetCanMove? false)
        (CallFunction|EPlayComboAction)))))

(event EventISkill
  (params (UseSkillNo :type Integer))
  ;[1 1 1] スキル
  (if (Variables|フラグ|GetCanAction?)
    (if (not (Variables|スキル|GetisCasting?))
      (bind _startcasting_ (詠唱|FStartCasting UseSkillNo))
      (if _startcasting_
        (攻撃|FFinishCombo)
        (攻撃|FWeaponColSwitch false)
        (Variables|フラグ|SetCanMove? false)
        (CallFunction|ROSChangeIsCasting? true)))))

(event EventIAvoid
  (bind _returnvalue (Pawn|GetControlRotation :!class /Script/Engine.Pawn))
  ;[1 1 1] 回避
  (if (Variables|フラグ|GetCanAction?)
    (攻撃|FFinishCombo)
    (攻撃|FWeaponColSwitch false)
    (詠唱|FStopCasting)
    (Variables|フラグ|SetCanAction? false)
    (Variables|フラグ|SetCanMove? false)
    (Utilities|MInputValid?
      (:true
        (CallFunction|RosSetActorRotation (Math|Rotator|FindLookatRotation (Math|Vector|MakeVector 0.0 0.0 0.0) (+ (* (Math|Vector|GetForwardVector (Math|Rotator|MakeRotator 0.0 0.0 (.yaw _returnvalue))) (Variables|移動|GetMoveForwardValue)) (* (Math|Vector|GetRightVector (Math|Rotator|MakeRotator 0.0 0.0 (.yaw _returnvalue))) (Variables|移動|GetMoveRightValue)))) false))
      (:false
        _))
    (CallFunction|ROSPlayAvoidAnim)))

(event Game|Damage|EventAnyDamage
  (params (Damage :type Float%20%28single-precision%29) (DamageType :type Damage%20Type%20Object%20Reference) (InstigatedBy :type Controller%20Object%20Reference) (DamageCauser :type Actor%20Object%20Reference))
  (Variables|ステータス|SetCurrentHP (Math|Float|Max(Float) 0.0 (- (Variables|ステータス|GetCurrentHP) Damage)))
  ;[1 0 0.01665] めっちゃ仮処理
  (Variables|必殺技|SetCurrentSpecial (+ 1.0 (Variables|必殺技|GetCurrentSpecial))))

(event EventISpecialAttack
  ;[1 1 1] 必殺技
  (if (Variables|フラグ|GetCanAction?)
    (if (>= (Variables|必殺技|GetCurrentSpecial) (Variables|必殺技|GetMaxSpecial))
      (CallFunction|ECloseComboGate)
      (攻撃|FFinishCombo)
      (攻撃|FWeaponColSwitch false)
      (詠唱|FStopCasting)
      (Variables|フラグ|SetCanAction? false)
      (Variables|フラグ|SetCanMove? false)
      (Variables|必殺技|SetCurrentSpecial 0.0)
      (CallFunction|ROSPlaySpecialAttack))))

(event EventISpawnHitBox
  (params (AttackType :type En_AttackType%20Enum :default "NewEnumerator0"))
  ;[1 1 1] 通常攻撃
  ;;[1 1 1] 攻撃の当たり判定
  (if (Pawn|IsLocallyControlled self)
    (攻撃|FWeaponColSwitch true)))

(event EventBeginPlay
  ;[1 1 1] 初期化処理
  (CallFunction|EInitialize))

(event EventISpawnSpecial
  ;[1 1 1] 必殺技
  (CallFunction|ROSSpawnActorfromClass (Variables|必殺技|GetSpecialAttackClass) (Math|Transform|MakeTransform (Transformation|GetActorLocation) "0, 0, 0" "1,1,1") "Undefined" self))

(event Custom|MC_SetActorRotation
  (params (NewRotation :type Rotator) (bTeleportPhysics :type Boolean))
  (Transformation|SetActorRotation NewRotation bTeleportPhysics))

(event Custom|ROS_SetActorRotation
  (params (NewRotation :type Rotator) (bTeleportPhysics :type Boolean))
  (CallFunction|MCSetActorRotation NewRotation bTeleportPhysics))

(event Custom|ROS_SpawnActorFromClass
  (params (Class :type Actor%20Class%20Reference) (SpawnTransform :type Transform) (CollisionHandlingOverride :type ESpawnActorCollisionHandlingMethod%20Enum :default "Undefined") (Owner :type Actor%20Object%20Reference) (Instigator :type Pawn%20Object%20Reference))
  (Game|SpawnActorfromClass Class SpawnTransform CollisionHandlingOverride Owner Instigator))

(event Custom|ROS_PlayAnimMontage
  (params (PlayRate :type Float%20%28single-precision%29) (MontageToPlay :type Anim%20Montage%20Object%20Reference))
  (CallFunction|MCPlayAnimMontage PlayRate MontageToPlay))

(event Custom|MC_PlayAnimMontage
  (params (PlayRate :type Float%20%28single-precision%29) (MontageToPlay :type Anim%20Montage%20Object%20Reference))
  (Animation|Montage|PlayMontage (Variables|Character|GetMesh) MontageToPlay PlayRate))

(event EventTick
  (params (DeltaSeconds :type Float%20%28single-precision%29))
  ;[1 1 1] 更新処理
  (Utilities|FlowControl|Sequence
    (:then_0
      (if (< (Variables|スキル|GetCurrentEnergy) (Variables|スキル|GetMaxEnergy))
        (if (>= (Variables|スキル|GetIncreaseElapsed) (Variables|スキル|GetIncreaseInterval))
          (Variables|スキル|SetIncreaseElapsed 0.0)
          (bind _output_get (CallFunction|FSetCurrentSP (Math|Integer|Clamp(Integer) (+ (Variables|スキル|GetCurrentEnergy) 1) 0 (Variables|スキル|GetMaxEnergy))))
          (else
            (Variables|スキル|SetIncreaseElapsed (+ (Variables|スキル|GetIncreaseElapsed) (Utilities|Time|GetWorldDeltaSeconds)))))))
    (:then_1
      (CallFunction|ECastingUpdate)
      (Default|EUpdate (Variables|Default|GetBPC_SkillHolder01))
      (Default|EUpdate (Variables|Default|GetBPC_SkillHolder02))
      (Default|EUpdate (Variables|Default|GetBPC_SkillHolder03))
      (Default|EUpdate (Variables|Default|GetBPC_SkillHolder04)))
    (:then_3
      (|DebugLog_2))))

(fn ConstructionScript)

(fn FMoveForward
  (params (Value :type Float%20%28single-precision%29))
  (Pawn|Input|AddMovementInput (Math|Vector|GetForwardVector (Math|Rotator|MakeRotator 0.0 0.0 (.Yaw (Math|Rotator|BreakRotator (Pawn|GetControlRotation :!class /Script/Engine.Pawn))))) Value false))

(fn FMoveRight
  (params (Value :type Float%20%28single-precision%29))
  (Pawn|Input|AddMovementInput (Math|Vector|GetRightVector (Math|Rotator|MakeRotator 0.0 0.0 (.Yaw (Math|Rotator|BreakRotator (Pawn|GetControlRotation :!class /Script/Engine.Pawn))))) Value false))

(fn FWeaponColSwitch
  (params (isAttacking? :type Boolean))
  (Collision|SetCollisionEnabled (Variables|Default|GetWeaponCol) (select isAttacking? "QueryOnly" "NoCollision")))

(fn FRotationtoNearEnemy
  (params (NearEnemyPos :type Vector))
  (Transformation|SetActorRotation (Math|Rotator|MakeRotator 0.0 0.0 (.yaw (Math|Rotator|FindLookatRotation (Transformation|GetActorLocation) NearEnemyPos)))))

(fn FFinishCombo
  (Variables|攻撃|SetComboCounter 0)
  (Variables|攻撃|SetisAttack? false))

(fn FStartCasting
  (params (Selection :type Integer))
  (bind _bpc_skillholder01 (Variables|Default|GetBPC_SkillHolder01))
  (bind _bpc_skillholder02 (Variables|Default|GetBPC_SkillHolder02))
  (bind _bpc_skillholder03 (Variables|Default|GetBPC_SkillHolder03))
  (bind _bpc_skillholder04 (Variables|Default|GetBPC_SkillHolder04))
  (switch int Selection
    (:0
      (Utilities|MCanUseSkill? _bpc_skillholder01
        (:true
          (Variables|スキル|SetUseSkillHolder _bpc_skillholder01)
          (Variables|スキル|SetCastingTime (Default|FGetCastingTime _bpc_skillholder01))
          (Variables|スキル|SetCastingElapsed 0.0 :!label _label)
          (Variables|スキル|SetisCasting? true)
          (Variables|スキル|SetCanSkillCancel? false)
          (return true))
        (:false
          _)))
    (:1
      (Utilities|MCanUseSkill? _bpc_skillholder02
        (:true
          (Variables|スキル|SetUseSkillHolder _bpc_skillholder02)
          (Variables|スキル|SetCastingTime (Default|FGetCastingTime _bpc_skillholder02))
          (goto _label))
        (:false
          _)))
    (:2
      (Utilities|MCanUseSkill? _bpc_skillholder03
        (:true
          (Variables|スキル|SetUseSkillHolder _bpc_skillholder03)
          (Variables|スキル|SetCastingTime (Default|FGetCastingTime _bpc_skillholder03))
          (goto _label))
        (:false
          _)))
    (:3
      (Utilities|MCanUseSkill? _bpc_skillholder04
        (:true
          (Variables|スキル|SetUseSkillHolder _bpc_skillholder04)
          (Variables|スキル|SetCastingTime (Default|FGetCastingTime _bpc_skillholder04))
          (goto _label))
        (:false
          _))))
  (return false))

(fn FStopCasting
  (Variables|スキル|SetisCasting? false)
  (Variables|スキル|SetCastingElapsed 0.0))

(fn FGetSkillReMaining
  (params (holder :type BPC%20Skill%20Holder%20Object%20Reference))
  (return (Default|FGetCoolingElapsed holder) (Default|FGetCoolingTime holder)))

(fn FSetCurrentSP
  (params (CurrentEnergy :type Integer))
  (bind _output_get (Variables|スキル|SetCurrentEnergy CurrentEnergy))
  (bind _asbp_player_controller (Utilities|Casting|CastToBP_PlayerController (Pawn|GetController)))
  (Default|EUpdateBattleScoreUI _asbp_player_controller)
  (return _output_get))

(fn IGetCastingElapsedTime
  (bind _useskillholder (Variables|スキル|GetUseSkillHolder)
    (:then
      (return (Variables|/Game/Workspace/IoriFUKUNAKA/Blueprints/Characters/Player/BPC_SkillHolder.BPC_SkillHolder_C|GetHolderIndex _useskillholder) (Variables|スキル|GetisCasting?) (Variables|スキル|GetCastingElapsed) (Variables|スキル|GetCastingTime)))
    (:else)))

(fn IGetCoolingElapsedTime
  (bind _bpc_skillholder01 (Variables|Default|GetBPC_SkillHolder01))
  (bind _bpc_skillholder02 (Variables|Default|GetBPC_SkillHolder02))
  (bind _bpc_skillholder03 (Variables|Default|GetBPC_SkillHolder03))
  (bind _bpc_skillholder04 (Variables|Default|GetBPC_SkillHolder04))
  (bind (_elapsedtime _coolingtime) (詠唱|FGetSkillReMaining _bpc_skillholder04))
  (bind (_elapsedtime_2 _coolingtime_2) (詠唱|FGetSkillReMaining _bpc_skillholder01))
  (bind (_elapsedtime_3 _coolingtime_3) (詠唱|FGetSkillReMaining _bpc_skillholder02))
  (bind (_elapsedtime_4 _coolingtime_4) (詠唱|FGetSkillReMaining _bpc_skillholder03))
  (return _elapsedtime_2 _coolingtime_2 _elapsedtime_3 _coolingtime_3 _elapsedtime_4 _coolingtime_4 _elapsedtime _coolingtime))

(fn IGetFightingEnemyInfo
  (bind _fightingenemyref (Variables|Default|GetFightingEnemyRef)
    (:then
      (return (Variables|/Game/Workspace/Yamashita/Blueprint/Base/BP_EnemyBase.BP_EnemyBase_C|GetMyFightingStage _fightingenemyref) (Variables|/Game/Workspace/Yamashita/Blueprint/Base/BP_EnemyBase.BP_EnemyBase_C|Gethealth _fightingenemyref)))
    (:else
      (return "NewEnumerator0" 0.0))))

(fn IGetSpecial
  (return (Variables|必殺技|GetCurrentSpecial) (Variables|必殺技|GetMaxSpecial)))