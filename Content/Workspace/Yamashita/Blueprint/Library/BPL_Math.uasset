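; BPL_Math is a math Blueprint library with one function, which finds the angle between two 2D vectors.
; FGetRot2D divides their dot product by the product of their lengths, then takes the arccosine.
; It returns the angle in both radians and degrees.
; The result is unsigned, and zero-length inputs are not guarded.
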(fn FGetRot2D
  (params (VectorA :type Vector%202D%20Structure) (VectorB :type Vector%202D%20Structure))
  (LocalVariables|SetA VectorA)
  (LocalVariables|SetB VectorB)
  (LocalVariables|Setlength_A (Math|Vector2D|Vector2DLength (LocalVariables|GetA)))
  (LocalVariables|Setlength_B (Math|Vector2D|Vector2DLength (LocalVariables|GetB)))
  (LocalVariables|Setcos_sita (/ (Math|Vector2D|DotProduct(2D) (LocalVariables|GetA) (LocalVariables|GetB)) (* (LocalVariables|Getlength_A) (LocalVariables|Getlength_B))))
  (bind _output_get (LocalVariables|Setsita (Math|Trig|Acos(Degrees) (LocalVariables|Getcos_sita))))
  (return _output_get (Math|Trig|RadiansToDegrees _output_get)))