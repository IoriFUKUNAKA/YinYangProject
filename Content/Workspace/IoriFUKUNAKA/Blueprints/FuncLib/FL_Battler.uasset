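; Blueprint function library for battlers, providing a single battle damage formula in FCulcDamage.
; It subtracts Defence from Attack, each offset by one so the offsets cancel, then scales the difference by one minus the clamped damage cut rate.
; A non-positive result is replaced with 1, so damage is always positive.
; Two random integer nodes are left unconnected, so the result is deterministic.
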(fn FCulcDamage
  (params (Attack :type Float%20%28single-precision%29) (Defence :type Float%20%28single-precision%29) (DamageCutRate :type Float%20%28single-precision%29))
  (bind _returnvalue (Math|Float|Clamp(Float) DamageCutRate))
  (bind _returnvalue_2 (+ Defence 1.0))
  (bind _returnvalue_3 (+ Attack 1.0))
  (bind _returnvalue_4 (- _returnvalue_3 _returnvalue_2))
  (bind _returnvalue_5 (- 1.0 _returnvalue))
  (bind _returnvalue_6 (* _returnvalue_5 _returnvalue_4))
  (return (Math|Float|SelectFloat _returnvalue_6 1.0 (> _returnvalue_6 0.0))))