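; BP_ElementData is a data object that holds an Element with a lifetime and tracks how long it has existed.
; E_UpdateElementData adds delta time to Elapsed while LifeTime is positive, calling OnDead on each update that finds Elapsed has already reached LifeTime.
; A LifeTime of zero never expires.
; Getters expose the Element, its lifetime and the remaining time, clamped to non-negative.
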(event Custom|E_UpdateElementData
  (params (_DeltaTIme :type Float%20%28single-precision%29))
  (if (> (Variables|Default|GetLifeTime) 0.0)
    (if (CallFunction|FIsDead?)
      (Default|CallOnDead)
      (else
        (Variables|Default|SetElapsed (+ _DeltaTIme (Variables|Default|GetElapsed)))))))

(fn FIsDead?
  (bind _lifetime (Variables|Default|GetLifeTime))
  (return (and (>= (Variables|Default|GetElapsed) _lifetime) (!= _lifetime 0.0))))

(fn FGetElement
  (return (Variables|Default|GetElement)))

(fn FGetRemainTime
  (return (Math|Float|Max(Float) (- (Variables|Default|GetLifeTime) (Variables|Default|GetElapsed)) 0.0)))

(fn FGetLifeTime
  (return (Variables|Default|GetLifeTime)))