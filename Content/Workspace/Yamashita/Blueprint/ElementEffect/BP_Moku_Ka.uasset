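; BP_Moku_Ka is an element effect, apparently for the Moku-Ka (wood-fire) combination, that deals damage to its owner.
; It extends a parent effect, caching the instigator's Attack from the PlayerState interface during initialization.
; When the combination effect fires, it applies penetrate-type damage equal to that attack times a base multiplier, with ±10% random variance.
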(fn ConstructionScript
  (|CallParentFunction))

(fn FInitialize
  (|CallParentFunction)
  (bind _instigator (Variables|Default|GetInstigator)
    (:then
      (bind _playerstate (Variables|/Script/Engine.Pawn|GetPlayerState _instigator)
        (:then
          (bind _attack (Class|BPIControlPlayerState|IGetCurrentPlayerStatus(Message) _playerstate))
          (Variables|Default|SetInstigatorAttack _attack))
        (:else)))
    (:else)))

(fn FCombinationEffect
  (|CallParentFunction)
  (Game|Damage|ApplyDamage (Components|GetOwner) (* (Variables|Default|GetInstigatorAttack) (Variables|Default|GetBaseMag) (Math|Random|RandomFloatinRange 0.9 1.1)) 0 self "/Game/Workspace/IoriFUKUNAKA/Blueprints/Characters/Player/DamageType/Combination/D_PenetrateDamage.D_PenetrateDamage_C"))