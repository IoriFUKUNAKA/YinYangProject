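; BP_Skill_AttackDebuff is a player skill that, going by its name, applies a temporary attack debuff to an enemy near the player.
; On initialization it asks the owner's game manager for a near enemy within a fixed distance of the owner.
; If one is found, it adds a timed, negative-value BP_StatusData to that enemy's status manager and destroys itself.
; Otherwise it only prints a "too far" message and is not destroyed here.
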(event EventBeginPlay)

(event Collision|EventActorBeginOverlap
  (params (OtherActor :type Actor%20Object%20Reference)))

(event EventTick
  (params (DeltaSeconds :type Float%20%28single-precision%29))
  (|CallParentFunction DeltaSeconds) ; このノードは無効になっているため呼び出せません。\n機能をビルドするにはピンをドラッグしてください。
)

(fn ConstructionScript
  (|CallParentFunction))

(fn FInitialize
  (|CallParentFunction)
  (bind _m_owner (Variables|Default|Getm_Owner)
    (:then
      (bind _m_gamemanager (Variables|/Game/Workspace/IoriFUKUNAKA/Blueprints/Characters/Player/BP_Player.BP_Player_C|Getm_GameManager _m_owner)
        (:then
          (bind (_isvalid_ _nearenemy) (Default|FGetNearEnemyfromPlayer _m_gamemanager (Transformation|GetActorLocation _m_owner) 8e+03))
          (if _isvalid_
            (bind _returnvalue (Game|ConstructObjectfromClass "/Game/Workspace/IoriFUKUNAKA/Blueprints/Characters/BP_StatusData.BP_StatusData_C" (Variables|/Game/Workspace/Yamashita/Blueprint/Base/BP_EnemyBase.BP_EnemyBase_C|GetBPC_StatusManager _nearenemy) "NewEnumerator0" -5e+02 1e+01))
            (Default|EAddEffect (Variables|/Game/Workspace/Yamashita/Blueprint/Base/BP_EnemyBase.BP_EnemyBase_C|GetBPC_StatusManager _nearenemy) _returnvalue)
            (Actor|DestroyActor)
            (else
              (Development|PrintString "遠いよ！"))))
        (:else)))
    (:else)))