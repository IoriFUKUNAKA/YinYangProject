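; BP_Moku_Sui is the Moku and Sui (wood and water) element combination effect, which heals every player in the game.
; On initialization it caches the instigator's current Attack through a player status interface call on its PlayerState.
; When the combination fires, it loops over the GameState PlayerArray and sends each pawn a heal message with over-heal enabled.
; Each heal scales that Attack by HealMag with slight random variance.
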(fn ConstructionScript
  (|CallParentFunction))

(fn FInitialize
  (|CallParentFunction)
  (bind _instigator (Variables|Default|GetInstigator)
    (:then
      (bind _playerstate (Variables|/Script/Engine.Pawn|GetPlayerState _instigator)
        (:then
          (bind _attack (Class|BPIControlPlayerState|IGetCurrentPlayerStatus(Message) _playerstate))
          (Variables|Default|SetInstigatorAttack _attack))
        (:else)))
    (:else)))

(fn FCombinationEffect
  (|CallParentFunction)
  (for _array_element (Variables|/Script/Engine.GameStateBase|GetPlayerArray (Game|GetGameState))
    (Class|BPIControlPlayer|IHealPlayer(Message) (Variables|/Script/Engine.PlayerState|GetPawnPrivate _array_element) (Math|Float|Truncate (* (Variables|Default|GetInstigatorAttack) (Variables|Default|GetHealMag) (Math|Random|RandomFloatinRange 0.9 1.1))) true)))