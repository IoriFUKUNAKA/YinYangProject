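; Afterimage decoy from the player's Dog zodiac ability that draws the Qilin's targeting onto itself.
; On spawn it copies the owner character's mesh and pose into a poseable mesh with afterimage materials.
; The server locks the Qilin's target to it every tick and releases the lock when it is destroyed.
; It expires after its lifespan or when damage depletes its HP.
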(event Custom|E_MeshSetting
  ;[1 1 1] ポーズとマテリアルを設定する
  (bind _ascharacter (Utilities|Casting|CastToCharacter (Components|GetOwner)))
  (Variables|Default|SetOwnerMesh (Variables|/Script/Engine.Character|GetMesh _ascharacter))
  (Class|SkinnedMeshComponent|SetSkeletalMesh (Variables|Default|GetPoseableMesh) (Variables|/Script/Engine.SkinnedMeshComponent|GetSkeletalMesh (Variables|/Script/Engine.Character|GetMesh _ascharacter)) true)
  (Class|PoseableMeshComponent|CopyPosefromSkeletalComponent (Variables|Default|GetPoseableMesh) (Variables|Default|GetOwnerMesh))
  (for (_ _array_index) (Rendering|Material|GetMaterials (Variables|Default|GetPoseableMesh))
    (bind _returnvalue (Rendering|Material|CreateDynamicMaterialInstance "/Game/Workspace/IoriFUKUNAKA/Materials/LightingTest/YinYangCharacters/MI_DogAfterImage.MI_DogAfterImage" "None" "None" :!class /Script/Engine.KismetMaterialLibrary))
    (Rendering|Material|SetMaterial (Variables|Default|GetPoseableMesh) _array_index _returnvalue)))

(event Custom|E_OnDestroy
  (params (Actor :type Actor%20Object%20Reference) (EndPlayReason :type EEndPlayReason%20Enum :default "Destroyed"))
  ;[1 1 1] 破棄時に麒麟のタゲロック解除
  (switch Utilities|FlowControl|Switch|SwitchonEEndPlayReason EndPlayReason
    (:Destroyed
      (CallFunction|ELockQilinTarget false))))

(event Custom|ROS_AnyDamage
  (params (Damage :type Float%20%28single-precision%29))
  ;[1 1 1] 被弾処理
  (Development|PrintString "残像だ…" true true "(R=1.000000,G=0.756586,B=0.000000,A=1.000000)" 5.0)
  (bind _output_get (Variables|プロパティ|SetCurrentHP (Math|Integer|Clamp(Integer) (- (Variables|プロパティ|GetCurrentHP) (CallFunction|FCalculateDamage Damage 0.0)) 0 (Variables|プロパティ|GetAfterImageHP))))
  (if (<= _output_get 0)
    (Actor|DestroyActor)))

(event Custom|E_LockQilinTarget
  (params (Lock? :type Boolean))
  ;[1 1 1] 麒麟のタゲの固定のオンオフ
  (Variables|Ref|GetQilin%20Ref
    (:then
      _)
    (:else
      (bind _asgs_main (Utilities|Casting|CastToGS_Main (Game|GetGameState)))
      (Variables|Ref|SetQilin%20Ref (Default|FGetQilinRef _asgs_main))))
  (Utilities|IsValid (Variables|Ref|GetQilin%20Ref)
    (:Is%20Valid
      (bind _target (Default|IGetEnemyTarget (Variables|Ref|GetQilin%20Ref)))
      (Utilities|IsValid _target
        (:Is%20Valid
          (if Lock?
            (Default|FLockEnemyTarget _target self)
            (else
              (bind _targetactor (Variables|/Game/Workspace/IoriFUKUNAKA/Blueprints/Characters/Enemy/BP_EnemyTarget.BP_EnemyTarget_C|GetTargetActor _target)
                (:then
                  (if (== _targetactor self)
                    (Default|FUnLockEnemyTarget _target)))
                (:else)))))))))

(event EventBeginPlay
  ;[1 1 1] 初期化
  (CallFunction|EMeshSetting)
  (Networking|SwitchHasAuthority
    (:Authority
      (Actor|SetLifeSpan (Variables|プロパティ|GetLifeTime))
      (Variables|プロパティ|SetCurrentHP (Variables|プロパティ|GetAfterImageHP))
      (Game|BindEventtoOnEndPlay (EventDispatchers|CreateEvent :!event Custom|E_OnDestroy)))))

(event Game|Damage|EventAnyDamage
  (params (Damage :type Float%20%28single-precision%29) (DamageType :type Damage%20Type%20Object%20Reference) (InstigatedBy :type Controller%20Object%20Reference) (DamageCauser :type Actor%20Object%20Reference))
  ;[1 1 1] 被弾処理
  (CallFunction|ROSAnyDamage Damage))

(event EventTick
  (params (DeltaSeconds :type Float%20%28single-precision%29))
  ;[1 1 1] 更新処理
  (Networking|SwitchHasAuthority
    (:Authority
      (CallFunction|ELockQilinTarget true))))

(fn ConstructionScript)