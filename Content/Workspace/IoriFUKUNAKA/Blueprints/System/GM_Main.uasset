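; Main game mode that gives each joining player a character and drives the match flow through a state machine.
; PostLogin registers each controller, uses its array index as PlayerID, then spawns and possesses the matching class from PlayerClassArray, replacing any existing pawn.
; Tick dispatches on MState: Ready resets the timer, sets game-only input and switches to Play, which counts and prints play time.
; Select and Result updates are empty stubs.
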(event Custom|E_PlayerCreate
  (params (ConectPlayerController :type BP%20Player%20Controller%20Object%20Reference))
  (bind _returnvalue (Pawn|GetControlledPawn ConectPlayerController))
  (bind _playerclassarray (Variables|General|GetPlayerClassArray))
  (bind _playerid (Variables|/Game/Workspace/IoriFUKUNAKA/Blueprints/Characters/Player/BP_PlayerController.BP_PlayerController_C|GetPlayerID ConectPlayerController))
  ;[1 1 1] IDに応じてプレイヤーキャラクターを生成してコントローラーを接続する
  (Utilities|IsValid _returnvalue
    (:Is%20Valid
      (Pawn|UnPossess ConectPlayerController)
      (Actor|DestroyActor _returnvalue))
    (:Is%20Not%20Valid
      _))
  (if (and (>= _playerid 0) (< _playerid (Utilities|Array|Length _playerclassarray)))
    (bind _returnvalue_2 (Game|SpawnActorfromClass (Utilities|Array|Get(acopy) _playerclassarray _playerid) (Math|Transform|MakeTransform "-800.000000,0.000000,120.000000" "0, 0, 0" "1,1,1") "Undefined" 0 0))
    (Pawn|Possess ConectPlayerController _returnvalue_2)
    (else
      (Development|PrintString "Error:PlayerSpawnFailed" true true "(R=1.000000,G=0.000000,B=0.000000,A=1.000000)"))))

(event EventPostLogin
  (params (NewPlayer :type Player%20Controller%20Object%20Reference))
  ;[1 1 1] ログイン時の処理
  (Development|PrintString "OnPostLogin")
  (bind _asbp_player_controller (Utilities|Casting|CastToBP_PlayerController NewPlayer))
  (bind _returnvalue (Utilities|Array|AddUnique (Variables|Ref|GetPlayerControllerArrey) _asbp_player_controller))
  (Variables|/Game/Workspace/IoriFUKUNAKA/Blueprints/Characters/Player/BP_PlayerController.BP_PlayerController_C|SetPlayerID _asbp_player_controller _returnvalue)
  (CallFunction|EPlayerCreate _asbp_player_controller))

(event Custom|E_SelectUpdate
  (params (DeltaSeconds :type Float%20%28single-precision%29)))

(event Custom|E_ReadyUpdate
  (params (DeltaSeconds :type Float%20%28single-precision%29))
  (Variables|Play|SetPlayTime 0.0)
  (for _array_element (Variables|Ref|GetPlayerControllerArrey)
    ;[1 1 1] ゲームUIができたら変更
    (Input|SetInputModeGameOnly _array_element))
  (Variables|General|Setm_State "NewEnumerator1"))

(event Custom|E_PlayUpdate
  (params (DeltaSeconds :type Float%20%28single-precision%29))
  (Utilities|FlowControl|Sequence
    (:then_0
      (bind _output_get (Variables|Play|SetPlayTime (+ (Variables|Play|GetPlayTime) (Utilities|Time|GetWorldDeltaSeconds))))
      (Development|PrintText (Utilities|Text|FormatText "PlayTime:{0}" (Utilities|Text|ToText(Float) _output_get "HalfToEven")) true true "(R=0.000000,G=0.660000,B=1.000000,A=1.000000)" 0.0))))

(event Custom|E_ResultUpdate
  (params (DeltaSeconds :type Float%20%28single-precision%29)))

(event EventTick
  (params (DeltaSeconds :type Float%20%28single-precision%29))
  (switch Utilities|FlowControl|Switch|SwitchonEn_GameState (Variables|General|Getm_State)
    (:NewEnumerator0
      (CallFunction|ESelectUpdate DeltaSeconds))
    (:NewEnumerator3
      (CallFunction|EReadyUpdate DeltaSeconds))
    (:NewEnumerator1
      (CallFunction|EPlayUpdate DeltaSeconds))
    (:NewEnumerator2
      (CallFunction|EResultUpdate DeltaSeconds))))

(fn ConstructionScript)