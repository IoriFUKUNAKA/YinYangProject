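; Telegraphed area attack for the Kirin enemy's jump, showing a ground decal and then striking on a landing timer.
; Init scales the decal to the attack radius and starts the timer, while Tick feeds elapsed time into the decal material's Rate parameter.
; The attack removes the decal, spawns Niagara through a server-to-multicast event pair, and delegates the sphere overlap to the owning enemy before destroying itself.
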(event Custom|MC_SetDecalScale
  (params (NewScale :type Float%20%28single-precision%29))
  ;[1 1 1] デカールサイズ変更
  (Transformation|SetWorldScale3D (Variables|Default|GetDecal) (Math|Conversions|ToVector(Float) (* NewScale 0.01))))

(event Custom|E_SetInit
  (params (timeForLanding :type Float%20%28single-precision%29) (RadiusOfJumpAttack :type Float%20%28single-precision%29))
  ;[1 1 1] 初期化
  (Variables|Default|SettimeForLanding timeForLanding)
  (bind _output_get (Variables|Default|SetRadiusOfJumpAttack RadiusOfJumpAttack))
  (CallFunction|MCSetDecalScale _output_get)
  (Utilities|Time|SetTimerbyEvent (EventDispatchers|CreateEvent :!event Custom|E_Attack) (Variables|Default|GettimeForLanding)))

(event Custom|E_UpdateDecal
  ;[1 1 1] デカールマテリアル　パラメーター設定
  (bind _output_get (Variables|Default|Settimer (+ (Variables|Default|Gettimer) (Utilities|Time|GetWorldDeltaSeconds))))
  (Rendering|Material|SetScalarParameterValue (Variables|Default|GetM_Decal) "Rate" _output_get :!class /Script/Engine.MaterialInstanceDynamic))

(event Custom|E_Attack
  ;[1 1 1] 攻撃エフェクト・コリジョン生成
  (Components|DestroyComponent (Variables|Default|GetDecal))
  (CallFunction|RoSSpawnEffect)
  (bind _enemyref (Variables|Default|GetEnemyRef)
    (:then
      (Default|FSphereOverlap _enemyref (Transformation|GetActorLocation) (Variables|Default|GetRadiusOfJumpAttack) false false 5)
      (Utilities|FlowControl|Delay 2.0)
      (Actor|DestroyActor))
    (:else)))

(event Custom|RoS_SpawnEffect
  ;[1 1 1] エフェクト生成
  (CallFunction|MCSpawnEffect))

(event Custom|MC_SpawnEffect
  ;[1 1 1] エフェクト生成
  (Niagara|SpawnSystematLocation "/Game/Workspace/Azuma/Effect/Kirin_hani_attack/NS_kirin_hani_attack.NS_kirin_hani_attack" (Transformation|GetActorLocation))
  (Development|PrintString "spawn"))

(event EventBeginPlay
  (|CallParentFunction)
  (bind _returnvalue (Rendering|Material|CreateDynamicMaterialInstance (Variables|Default|GetDecal) :!class /Script/Engine.DecalComponent))
  (Variables|Default|SetM_Decal _returnvalue))

(event EventTick
  (params (DeltaSeconds :type Float%20%28single-precision%29))
  (CallFunction|EUpdateDecal))

(fn ConstructionScript
  (|CallParentFunction))