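; BP_ElementEffectBase is a base Blueprint for element effects, with empty effect and finish functions as hooks for children.
; On BeginPlay it prints a debug message and runs F_Effect once.
; If Continuation is set, timers repeat F_Effect every EffectSpan and handle the LifeTime expiry; otherwise it calls E_Destroy immediately.
; E_Destroy runs F_FinishAction, then destroys the actor.
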(event Custom|E_Destroy
  (CallFunction|FFinishAction)
  (Actor|DestroyActor))

(event EventBeginPlay
  (Development|PrintString "Spawn" true true "(R=0.217018,G=0.000000,B=1.000000,A=1.000000)")
  (CallFunction|FEffect)
  (if (Variables|Default|Getcontinuation)
    (Utilities|Time|SetTimerbyEvent (EventDispatchers|CreateEvent :!event Custom|E_Destroy) (Variables|Default|GetLifeTime))
    (Utilities|Time|SetTimerbyFunctionName self "F_Effect" (Variables|Default|GetEffectSpan) true)
    (else
      (CallFunction|EDestroy))))

(fn ConstructionScript)

(fn FEffect)

(fn FFinishAction)