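; BPC_JufuHolder is a player-character component that stores one Jufu skill and manages its cooldown, activation and hate generation.
; Initialization multicasts the skill class, caching mana, chant, cooldown, hate, targeting and animation values from its class defaults for getters.
; An externally driven update advances the cooldown.
; Activation uses server events to spawn the Jufu at either the Qilin enemy or target player, then add hate to Qilin by controller ID.
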(event Custom|E_initializeJufuHolder
  (params (StoringSkillData :type ST%20Juhul%20Data%20Structure))
  (bind _jufuclass (Utilities|Struct|BreakST_JuhulData StoringSkillData))
  ;[1 1 1] 初期化処理
  (bind _asbp_jufu_base (Utilities|Casting|CastToBP_JufuBaseClass (Class|KismetMathLibrary|SelectClass _jufuclass "/Game/Workspace/IoriFUKUNAKA/Blueprints/Characters/Player/Jufu/BP_JufuBase.BP_JufuBase_C" (Utilities|IsValidClass _jufuclass))))
  (CallFunction|MCSetUseSkillData _asbp_jufu_base))

(event Custom|E_CoolingUpdate
  ;[1 1 1] 冷却時間
  (if (not (Variables|冷却時間|GetisReady?))
    (if (< (+ (Variables|冷却時間|GetCoolingElapsed) (Utilities|Time|GetWorldDeltaSeconds)) (Variables|冷却時間|GetCoolTime))
      (Variables|冷却時間|SetCoolingElapsed (+ (Variables|冷却時間|GetCoolingElapsed) (Utilities|Time|GetWorldDeltaSeconds)))
      (else
        (Variables|冷却時間|SetisReady? true)
        (Variables|冷却時間|SetCoolingElapsed 0.0)))))

(event Custom|ROS_SpawnSkill
  (params (OwnerActor :type Actor%20Object%20Reference))
  ;[1 1 1] スキルの使用
  (if (Utilities|IsValidClass (Variables|呪符|GetStoredJufu))
    (bind _returnvalue (Game|SpawnActorfromClass (Variables|呪符|GetStoredJufu) (Math|Transform|MakeTransform (Transformation|GetActorLocation OwnerActor) "0, 0, 0" "1,1,1") "Undefined" OwnerActor (.AsPawn (Utilities|Casting|CastToPawn (Components|GetOwner)))))
    (Default|EInitialize _returnvalue)))

(event Custom|E_SkillActivate
  ;[1 1 1] スキルの使用
  (Variables|冷却時間|SetisReady? false)
  (if (Variables|呪符|GetIsEnemyTargetJufu?)
    (bind _asgs_main (Utilities|Casting|CastToGS_Main (Game|GetGameState)))
    (CallFunction|ROSSpawnSkill (Default|FGetQilinRef _asgs_main))
    (else
      (bind _targetplayer (Class|BPIControlPlayer|IGetTargetPlayer(Message) (Components|GetOwner)))
      (CallFunction|ROSSpawnSkill _targetplayer)))
  (CallFunction|ROSAddHate (Variables|呪符|GetHateValue)))

(event Custom|E_UpdateJufuHolder
  ;[1 1 1] 更新処理
  (CallFunction|ECoolingUpdate))

(event Custom|MC_SetUseSkillData
  (params (JufuClass :type BP%20Jufu%20Base%20Class%20Reference))
  ;[1 1 1] 初期化処理
  (bind _output_get (Variables|呪符|SetStoredJufu JufuClass))
  (Variables|呪符|SetIsEnemyTargetJufu? (.isEnemyTargetJufu? (Utilities|GetClassDefaults _output_get)))
  (Variables|呪符|SetUseMana (.ManaCost (Utilities|GetClassDefaults _output_get)))
  (Variables|詠唱時間|SetChantTime (.ChantTime (Utilities|GetClassDefaults _output_get)))
  (Variables|冷却時間|SetCoolTime (.CoolTime (Utilities|GetClassDefaults _output_get)))
  (Variables|呪符|SetHateValue (.HateValue (Utilities|GetClassDefaults _output_get)))
  (Variables|呪符|SetChant%20Fin%20Anim (.ChantFinAnim (Utilities|GetClassDefaults _output_get))))

(event Custom|ROS_AddHate
  (params (HateValue :type Float%20%28single-precision%29))
  ;[1 1 1] スキルの使用
  (bind _asgs_main (Utilities|Casting|CastToGS_Main (Game|GetGameState)))
  (bind _playerstate (Variables|/Script/Engine.Controller|GetPlayerState (Pawn|GetController (.AsPawn (Utilities|Casting|CastToPawn (Components|GetOwner)))))
    (:then
      (bind _controllerid (Class|BPIControlPlayerState|IGetControllerID(Message) _playerstate))
      (Default|FAddHate (Default|FGetQilinRef _asgs_main) _controllerid HateValue))
    (:else)))

(fn FIsStoredSkiill?
  (return (Utilities|IsValidClass (Variables|呪符|GetStoredJufu))))

(fn FGetMana
  (return (Variables|呪符|GetUseMana)))

(fn FGetChantTime
  (return (Variables|詠唱時間|GetChantTime)))

(fn FGetisReady?
  (return (Variables|冷却時間|GetisReady?)))

(fn FGetCoolingTime
  (return (Variables|冷却時間|GetCoolTime)))

(fn FGetCoolingElapsed
  (return (Variables|冷却時間|GetCoolingElapsed)))

(fn FGetChantFinAnim
  (return (Variables|呪符|GetChant%20Fin%20Anim)))