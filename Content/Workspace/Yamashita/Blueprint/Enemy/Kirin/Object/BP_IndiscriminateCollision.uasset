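; Short-lived hitbox actor for the Kirin enemy's indiscriminate attack, covering a tall box around its location.
; Timers started on BeginPlay switch collision on after a brief delay, off later, then destroy the actor.
; While active, Tick calls FBoxOverlap on the referenced enemy to run the overlap check, rather than using overlap events.
; Tick also draws debug boxes, adding a differently colored one during the active window.
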(event Custom|E_CollisionOn
  (Variables|Default|SetCollision true))

(event Custom|E_Destroy
  (Actor|DestroyActor))

(event Custom|E_CollisionOff
  (Variables|Default|SetCollision false))

(event EventBeginPlay
  (|CallParentFunction)
  (Utilities|Time|SetTimerbyEvent (delegate Custom|E_CollisionOn) 0.3)
  (Utilities|Time|SetTimerbyEvent (delegate Custom|E_CollisionOff) 2.22)
  (Utilities|Time|SetTimerbyEvent (delegate Custom|E_Destroy) 3.0))

(event Collision|EventActorBeginOverlap
  (params (OtherActor :type Actor%20Object%20Reference)))

(event EventTick
  (params (DeltaSeconds :type Float%20%28single-precision%29))
  (bind _returnvalue (Transformation|GetActorLocation))
  (Rendering|Debug|DrawDebugBox _returnvalue "100.000000,100.000000,500.000000" "(R=1.000000,G=1.000000,B=1.000000,A=1.000000)" "0, 0, 0" 0.0 0.0)
  (if (Variables|Default|GetCollision)
    (Default|FBoxOverlap (Variables|Default|GetEnemyRef) _returnvalue "100.000000,100.000000,500.000000" false false 10)
    (Rendering|Debug|DrawDebugBox _returnvalue "100.000000,100.000000,500.000000" "(R=1.000000,G=0.052581,B=0.000000,A=1.000000)" "0, 0, 0" 0.0 0.0)))

(fn ConstructionScript
  (|CallParentFunction))