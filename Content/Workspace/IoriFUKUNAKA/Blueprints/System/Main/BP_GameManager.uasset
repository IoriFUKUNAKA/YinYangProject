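; Multiplayer game manager that spawns player pawns by controller ID and runs the Select-to-Play game flow.
; In Select, the server counts down while all players are ready, then switches to Play, propagating the state to enemies and moving players to the battle start.
; It registers enemies and players' hate entries, spawning target actors mapped by fighting stage that can retarget to the highest-hate player unless locked.
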(event Custom|E_PlayerCreate
  (params (ConectPlayerController :type BP%20Player%20Controller%20Object%20Reference))
  (bind _returnvalue (Pawn|GetControlledPawn ConectPlayerController))
  (bind _playerclassarray (Variables|Default|GetPlayerClassArray))
  (bind _playerid (Variables|/Game/Workspace/IoriFUKUNAKA/Blueprints/Characters/Player/BP_PlayerController.BP_PlayerController_C|GetPlayerID ConectPlayerController))
  ;[1 1 1] IDに応じてプレイヤーキャラクターを生成する
  (Utilities|IsValid _returnvalue
    (:Is%20Valid
      (Pawn|UnPossess ConectPlayerController)
      (Actor|DestroyActor _returnvalue))
    (:Is%20Not%20Valid
      _))
  (if (and (>= _playerid 0) (< _playerid (Utilities|Array|Length _playerclassarray)))
    (bind _returnvalue_2 (Game|SpawnActorfromClass (Utilities|Array|Get(acopy) _playerclassarray _playerid) (Math|Transform|MakeTransform "0.000000,200.000000,-400.000000" "0, 0, 0" "1,1,1") "Undefined" 0 0))
    (Pawn|Possess ConectPlayerController _returnvalue_2)
    (Default|EInitialize _returnvalue_2 self)
    (CallFunction|EAddHateData _returnvalue_2)
    ;;[1 0.05021 0] あとで場所変える
    (switch Utilities|FlowControl|Switch|SwitchonEn_GameState (Variables|Default|Getm_State)
      (:NewEnumerator0
        (Default|ESelectInitialize ConectPlayerController))
      (:NewEnumerator1
        (CallFunction|FonPlayStart ConectPlayerController) ; 今は途中から入ったら呪符選択なしでそのまま戦いの場に放り出される
      ))
    (else
      (Development|PrintString "Error:PlayerSpawnFailed" true true "(R=1.000000,G=0.000000,B=0.000000,A=1.000000)"))))

(event Custom|E_PlayUpdate
  ;[1 1 1] Player ステートUpate
  (Networking|SwitchHasAuthority
    (:Authority
      (bind _asgm_main (Utilities|Casting|CastToGM_Main (Game|GetGameMode)))
      (for _array_element (Default|FGetPlayerControllerRef _asgm_main)
        (Default|EMainUpdate _array_element)))))

(event Custom|E_ChangeState
  (params (m_State :type En_GameState%20Enum :default "NewEnumerator0"))
  ;[1 1 1] ゲームステート変更
  (bind _output_get (Variables|Default|Setm_State m_State))
  (CallFunction|FSetEnemyGameState _output_get)
  (switch Utilities|FlowControl|Switch|SwitchonEn_GameState (Variables|Default|Getm_State)
    (:NewEnumerator1
      (CallFunction|EPlayStateInit))))

(event Custom|E_PlayStateInit
  ;[1 1 1] Playステートになったときの初期化
  (bind _asgm_main (Utilities|Casting|CastToGM_Main (Game|GetGameMode)))
  (for _array_element (Default|FGetPlayerControllerRef _asgm_main)
    (CallFunction|FonPlayStart _array_element)))

(event Custom|ROS_InitializeController
  (bind _asgm_main (Utilities|Casting|CastToGM_Main (Game|GetGameMode)))
  (for _array_element (Default|FGetPlayerControllerRef _asgm_main)
    (CallFunction|MCInitializeController _array_element)))

(event Custom|MC_InitializeController
  (params (ターゲット :type BP%20Player%20Controller%20Object%20Reference))
  (Default|EMainInitialize ターゲット))

(event Custom|E_AddHateData
  (params (Player :type BP%20Player%20Object%20Reference))
  ;[1 1 1] ログインしたプレイヤーのヘイト情報を追加する
  (for _array_element (Variables|Ref|GetEnemiesRef)
    (Utilities|Array|AddUnique (Variables|/Game/Workspace/Yamashita/Blueprint/Base/BP_EnemyBase.BP_EnemyBase_C|GetPlayersHate _array_element) (Utilities|Struct|MakeST_PlayerHate Player 0.0))))

(event Custom|E_InitEnemy
  ;[1 1 1] 敵を取得（取得方法は変える?）
  (for _array_element (Variables|Ref|GetEnemiesRef)
    (bind _asbp_enemy_base (Utilities|Casting|CastToBP_EnemyBase _array_element))
    (Default|EInit _asbp_enemy_base self)
    (CallFunction|FAddEnemyRef _asbp_enemy_base)
    (CallFunction|RoSSpawnEnemyTarget (Variables|/Game/Workspace/Yamashita/Blueprint/Base/BP_EnemyBase.BP_EnemyBase_C|GetMyFightingStage _asbp_enemy_base))))

(event Custom|E_SelectUpdate
  ;[1 1 1] Select ステートUpdate
  (Networking|SwitchHasAuthority
    (:Authority
      (bind _asgm_main (Utilities|Casting|CastToGM_Main (Game|GetGameMode)))
      (Select|FSetTimeforStartGame _asgm_main)
      (Select|FUpdateSelectUI _asgm_main)
      (if (<= (Variables|Select|GetTimeForStartGame) 0.0)
        (CallFunction|EChangeState "NewEnumerator1")))))

(event Custom|MC_SpawnEnemyTarget
  (params (enemyState :type En_FightingEnemyState%20Enum :default "NewEnumerator0"))
  (CallFunction|RoSSpawnEnemyTarget enemyState))

(event EventTick
  (params (DeltaSeconds :type Float%20%28single-precision%29))
  (Utilities|FlowControl|Sequence
    (:then_0
      ;[1 1 1] Debug
      (bind _returnvalue (Class|AppUtilBPLibrary|IsGamePadConnected))
      (Development|PrintText (Utilities|Text|FormatText "ゲームパッド接続判定：{0}" _returnvalue) true true "(R=1.000000,G=0.000000,B=0.901710,A=1.000000)" 0.0))
    (:then_1
      (switch Utilities|FlowControl|Switch|SwitchonEn_GameState (Variables|Default|Getm_State)
        (:NewEnumerator0
          (CallFunction|ESelectUpdate))
        (:NewEnumerator1
          (CallFunction|EPlayUpdate)
          (bind _enumvalue (|ForEachEn_FightingEnemyState)
            (:LoopBody
              (if (.ReturnValue (Utilities|Map|Find (Variables|Default|GetEnemyTargetMap) _enumvalue))
                (Development|PrintString (Utilities|GetDisplayName (Variables|/Game/Workspace/IoriFUKUNAKA/Blueprints/Characters/Enemy/BP_EnemyTarget.BP_EnemyTarget_C|Getm_TargetPlayer (.Value (Utilities|Map|Find (Variables|Default|GetEnemyTargetMap) _enumvalue)))) true true "(R=0.894237,G=0.000000,B=1.000000,A=1.000000)" 0.0)))))))))

(event EventBeginPlay
  (CallFunction|EInitEnemy))

(event Custom|E_ChangeTarget
  (params (EnemyState :type En_FightingEnemyState%20Enum :default "NewEnumerator0"))
  (bind _enemytargetmap (Variables|Default|GetEnemyTargetMap))
  (bind (_value _returnvalue) (Utilities|Map|Find _enemytargetmap EnemyState))
  (if _returnvalue
    (if (not (Variables|/Game/Workspace/IoriFUKUNAKA/Blueprints/Characters/Enemy/BP_EnemyTarget.BP_EnemyTarget_C|GetisLock? _value))
      (bind _array_element (Utilities|Array|ForEachLoopwithBreak (Variables|Ref|GetEnemiesRef) :!label _label)
        (:LoopBody
          (if (Utilities|Enum|Equal(Enum) (Variables|/Game/Workspace/Yamashita/Blueprint/Base/BP_EnemyBase.BP_EnemyBase_C|GetMyFightingStage _array_element) EnemyState)
            (bind _player (Default|FGetHightestHatePlayer _array_element))
            (Variables|/Game/Workspace/IoriFUKUNAKA/Blueprints/Characters/Enemy/BP_EnemyTarget.BP_EnemyTarget_C|Setm_TargetPlayer _value _player)
            (goto _label Break)))))))

(event Custom|RoS_SpawnEnemyTarget
  (params (enemyState :type En_FightingEnemyState%20Enum :default "NewEnumerator0"))
  (bind _returnvalue (Game|SpawnActorfromClass "/Game/Workspace/IoriFUKUNAKA/Blueprints/Characters/Enemy/BP_EnemyTarget.BP_EnemyTarget_C" (Math|Transform|MakeTransform "0, 0, 0" "0, 0, 0" "1,1,1") "Undefined" 0 0))
  (Utilities|Map|Add (Variables|Default|GetEnemyTargetMap) enemyState _returnvalue))

(fn ConstructionScript)

(fn FAddPlayerRef
  (params (PlayerRef :type BP%20Player%20Object%20Reference))
  (Utilities|Array|AddUnique (Variables|Ref|GetPlayersRef) PlayerRef))

(fn FAddEnemyRef
  (params (EnemyRef :type BP%20Enemy%20Base%20Object%20Reference))
  (Utilities|Array|AddUnique (Variables|Ref|GetEnemiesRef) EnemyRef))

(fn FResetRefArrays
  (Utilities|Array|Clear (Variables|Ref|GetPlayersRef))
  (Utilities|Array|Clear (Variables|Ref|GetEnemiesRef)))

(fn FCheckAllReady
  (params (GMMain :type GM%20Main%20Object%20Reference))
  (for _array_element (Default|FGetPlayerControllerRef GMMain)
    (LocalVariables|SetAlreadyNum (+ (LocalVariables|GetAlreadyNum) (Math|Integer|SelectInt 1 0 (Variables|/Game/Workspace/IoriFUKUNAKA/Blueprints/Characters/Player/BP_PlayerController.BP_PlayerController_C|GetisReady _array_element)))))
  (return (== (Utilities|Array|Length (Default|FGetPlayerControllerRef GMMain)) (LocalVariables|GetAlreadyNum))))

(fn FSetTimeforStartGame
  (params (GMMain :type GM%20Main%20Object%20Reference))
  (bind _isallready (Select|FCheckAllReady GMMain))
  (bind _output_get (Variables|Select|SetIsAllPlayerStunby _isallready))
  (if _output_get
    (Variables|Select|SetTimeForStartGame (Math|Float|Clamp(Float) (- (Variables|Select|GetTimeForStartGame) (Utilities|Time|GetWorldDeltaSeconds)) 0.0 (Variables|Select|GetMaxTimeForStartGame)))
    (else
      (Variables|Select|SetTimeForStartGame (Variables|Select|GetMaxTimeForStartGame)))))

(fn FUpdateSelectUI
  (params (GMMain :type GM%20Main%20Object%20Reference))
  (for _array_element (Default|FGetPlayerControllerRef GMMain)
    (Default|ESelectUpdate _array_element (Variables|Select|GetTimeForStartGame) (Variables|Select|GetIsAllPlayerStunby))))

(fn FonPlayStart
  (params (Controller :type BP%20Player%20Controller%20Object%20Reference))
  (Default|RoCRemoveSelectHUD Controller)
  (Transformation|SetActorLocation (Pawn|GetControlledPawn Controller) (Math|Vector|MakeVector -9e+01 1.56e+03 1.2e+02) false true)
  (Default|EMainInitialize Controller))

(fn FSetEnemyGameState
  (params (CurrentGameState :type En_GameState%20Enum :default "NewEnumerator0"))
  (for _array_element (Variables|Ref|GetEnemiesRef)
    (Variables|/Game/Workspace/Yamashita/Blueprint/Base/BP_EnemyBase.BP_EnemyBase_C|SetCurrentGameState _array_element CurrentGameState)))

(fn FGetNearEnemyfromPlayer
  (params (PlayerPos :type Vector) (CheckDistanceDeadLine :type Float%20%28single-precision%29))
  (for _array_element (Variables|Ref|GetEnemiesRef)
    (Utilities|IsValid _array_element
      (:Is%20Valid
        (bind __nearenemy (LocalVariables|Get_NearEnemy)
          (:then
            (if (< (Class|KismetMathLibrary|VectorDistance2DSquared PlayerPos (Transformation|GetActorLocation _array_element)) (LocalVariables|Get_SqrDistance))
              (LocalVariables|Set_NearEnemy __nearenemy)
              (LocalVariables|Set_SqrDistance (Class|KismetMathLibrary|VectorDistance2DSquared PlayerPos (Transformation|GetActorLocation _array_element)))))
          (:else
            (if (<= (Class|KismetMathLibrary|VectorDistance2DSquared PlayerPos (Transformation|GetActorLocation _array_element)) (Math|Float|Power CheckDistanceDeadLine 2.0))
              (LocalVariables|Set_NearEnemy _array_element)
              (LocalVariables|Set_SqrDistance (Class|KismetMathLibrary|VectorDistance2DSquared PlayerPos (Transformation|GetActorLocation _array_element)))))))))
  (bind __nearenemy_2 (LocalVariables|Get_NearEnemy)
    (:then
      (return __nearenemy_2 true))
    (:else
      (return 0 false))))

(fn FGetEnemyTargetLoc
  (params (EnemyState :type En_FightingEnemyState%20Enum :default "NewEnumerator0"))
  (bind _enemytargetmap (Variables|Default|GetEnemyTargetMap))
  (bind (_value _returnvalue) (Utilities|Map|Find _enemytargetmap EnemyState))
  (if _returnvalue
    (return (Transformation|GetActorLocation _value))
    (else
      (return "0, 0, 0"))))

(fn FGetEnemyRef
  (return (Variables|Ref|GetEnemiesRef)))